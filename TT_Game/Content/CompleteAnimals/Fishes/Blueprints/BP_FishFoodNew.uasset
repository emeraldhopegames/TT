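; BP_FishFoodNew is a fish food actor that holds a set of food types and a finite amount to be eaten.
; CanEat reports whether a requested food type appears in its FoodTypes array.
; Eat subtracts the requested bite from Amount, or destroys the actor when the bite exceeds what remains, returning the amount eaten and whether the food was used up.
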(fn `CanEat`
  (params (FoodType :type "/Game/CompleteAnimals/Fishes/Blueprints/ENum_FoodType Enum" :default "NewEnumerator0"))
  (returns (CanEat :type Boolean))
  (locals (IsEatableFood :type Boolean))
  ;[1 1 1] If there is FoodType in FoodTypes, make IsEatableFood true.
  (for _array_element (`self.FoodTypes`)
    (if (`|EnumEquality` _array_element FoodType)
      (set `local.IsEatableFood` true)))
  (return (`local.IsEatableFood`)))

(fn `Eat`
  (params (EatAmount :type "Float (double-precision)"))
  (returns (EatableAmount :type "Float (double-precision)") (AteUp :type Boolean))
  ;[1 1 1] Amount<EatAmount then destroyActor.
  (if (> EatAmount (`self.Amount`))
    (`self.K2_DestroyActor`)
    (return (`self.Amount`) true)
    (else
      (set `self.Amount` (- (`self.Amount`) EatAmount))
      (return EatAmount false))))

(fn `UserConstructionScript`)
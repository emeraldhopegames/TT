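; BP_FoodSpawn is a timed spawner that drops fish food at its location for the fish animal system.
; Tick accumulates time and calls SpawnFood each interval, which spawns a configured BP_FishFoodNewCharacter only while the count of Interface_Eatable actors is within MaxFoodNum.
; It then notifies every Interface_Predator actor of the new food via FoodSpawnMessage.
; The construction script sets a text label on the spawner.
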(event `self.ReceiveTick`
  (params (DeltaSeconds :type "Float (single-precision)"))
  ;[1 1 1] Increase SpawnTIme
  (bind _output_get (set `self.SpawnTime` (+ DeltaSeconds (`self.SpawnTime`))))
  ;[1 1 1] SpawnInterval>SpawnTime?
  (if (> _output_get (`self.SpawnInterval`))
    ;[1 1 1] SpawnFood
    (set `self.SpawnTime` 0.0)
    (`self.SpawnFood`)))

(fn `SpawnFood`
  (locals (FoodNum :type Integer))
  ;[1 1 1] Number of Eatable Actor<=MaxFoodNum?
  (bind _outactors (`GameplayStatics.GetAllActorsWithInterface` "/Game/CompleteAnimals/Fishes/Blueprints/Interface_Eatable.Interface_Eatable_C"))
  (if (<= (`KismetArrayLibrary.Array_Length` _outactors) (`self.MaxFoodNum`))
    ;[1 1 1] Spawn Food
    (bind _returnvalue (`|SpawnActorFromClass` "/Game/CompleteAnimals/Fishes/Blueprints/BP_FishFoodNewCharacter.BP_FishFoodNewCharacter_C" (`KismetMathLibrary.MakeTransform` (`SceneComponent.K2_GetComponentLocation` (`self.DefaultSceneRoot`))) "Undefined" "OverrideRootScale" null (`self.FoodTypes`) (`self.Amount`) (`self.IsFloat`) null))
    (bind _outactors_2 (`GameplayStatics.GetAllActorsWithInterface` "/Game/CompleteAnimals/Fishes/Blueprints/Interface_Predator.Interface_Predator_C"))
    (for _array_element _outactors_2
      (message `/Game/CompleteAnimals/Fishes/Blueprints/Interface_Predator.FoodSpawn` _array_element _returnvalue))))

(fn `UserConstructionScript`
  ;[1 1 1] Set the text.
  (`TextRenderComponent.K2_SetText` (`self.TextRender`) (`self.Text`)))
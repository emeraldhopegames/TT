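; Koi spawner that fills a 3D grid with BP_ChasingKoiNew actors at BeginPlay, spaced by Interval from its root location.
; Each fish gets random per-axis scale, food-seeking time, satiety, and head and body morph target weights.
; SetTheMaterialParameters then randomizes its dynamic material, picking a white, black, grey, red or gold base.
; The base choice drives pattern colors and weighted random pattern visibility, with patterns off for grey and gold.
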(event `self.ReceiveBeginPlay`
  (bind _returnvalue (`KismetMathLibrary.RandomFloatInRange` 0.6 1.5))
  ;[1 1 1] Set the Spawn position.
  (for _index (range (+ (`self.NumX`) 1))
    (for _index_2 (range (+ (`self.NumY`) 1))
      (for _index_3 (range (+ (`self.NumZ`) 1))
        ;[1 1 1] Spawn actor.
        (bind _returnvalue_2 (`|SpawnActorFromClass` "/Game/CompleteAnimals/Fishes/FreshWaterFishes/Koi/Blueprints/BP_ChasingKoiNew.BP_ChasingKoiNew_C" (`KismetMathLibrary.MakeTransform` (+ (`SceneComponent.K2_GetComponentLocation` (`self.DefaultSceneRoot`)) (`KismetMathLibrary.MakeVector` (* _index (`self.Interval`)) (* _index_2 (`self.Interval`)) (* _index_3 (`self.Interval`)))) (struct) (`KismetMathLibrary.MakeVector` _returnvalue _returnvalue _returnvalue)) "Undefined" "OverrideRootScale" null (struct) (struct) (struct) (struct) (struct) (struct) (struct) (struct) (struct) (struct) (struct) (`KismetMathLibrary.RandomFloatInRange` 0.8 1.2) (`KismetMathLibrary.RandomFloatInRange` 0.0 15.0) "NewEnumerator0" 18.0 "UpperLip" null))
        ;[1 1 1] Get material instance.
        (bind _asmaterial_instance_dynamic (cast `MaterialInstanceDynamic` (`/Game/CompleteAnimals/Fishes/FreshWaterFishes/Koi/Blueprints/BP_ChasingKoiNew.MaterialInstance` _returnvalue_2)))
        (bind _mesh (`Character.Mesh` _returnvalue_2))
        ;[1 1 1] Set the morph target.
        (`SkeletalMeshComponent.SetMorphTarget` _mesh "KoiMiddlePolyHeadMorph" (`KismetMathLibrary.RandomFloatInRange` -1.0 1.0) true)
        (`SkeletalMeshComponent.SetMorphTarget` _mesh "KoiMiddlePoly_BodyMorph" (`KismetMathLibrary.RandomFloatInRange` -1.0 1.0) true)
        ;[1 1 1] Set the material  instanceparameters.
        (`self.SetTheMaterialParameters` _asmaterial_instance_dynamic)))))

(fn `SetTheMaterialParameters`
  (params (InputPin :type "MaterialInstanceDynamic Object Reference"))
  (locals (IsBaseColorWhite :type Boolean :default false) (IsBaseColorBlack :type Boolean) (IsBaseColorGrey :type Boolean) (IsBaseColorRed :type Boolean) (IsBaseColorGold :type Boolean) (MaterialInstance :type "MaterialInstanceDynamic Object Reference"))
  (bind _returnvalue (`KismetMathLibrary.RandomFloatInRange` 0.0 0.1))
  (bind _returnvalue_2 (`KismetMathLibrary.RandomFloatInRange` 0.0 0.1))
  (bind _returnvalue_3 (`KismetMathLibrary.RandomFloatInRange` 0.0 0.1))
  (bind _returnvalue_4 (`KismetMathLibrary.RandomFloatInRange` 0.0 0.05))
  (bind _returnvalue_5 (`KismetMathLibrary.RandomFloatInRange` 0.9 1.0))
  (bind _returnvalue_6 (`KismetMathLibrary.RandomFloatInRange` 0.9 1.0))
  (bind _returnvalue_7 (`KismetMathLibrary.RandomFloatInRange` 0.9 1.0))
  (bind _returnvalue_8 (`KismetMathLibrary.RandomFloatInRange` 0.9 1.0))
  (bind _returnvalue_9 (`KismetMathLibrary.RandomFloatInRange` 0.9 1.0))
  (bind _returnvalue_10 (`KismetMathLibrary.RandomFloatInRange` 0.9 1.0))
  (bind _returnvalue_11 (`KismetMathLibrary.RandomFloatInRange` 0.9 1.0))
  (bind _returnvalue_12 (`KismetMathLibrary.RandomFloatInRange` 0.9 1.0))
  (bind _returnvalue_13 (`KismetMathLibrary.RandomFloatInRange` 0.9 1.0))
  (bind _returnvalue_14 (`KismetMathLibrary.RandomFloatInRange` 0.9 1.0))
  (bind _returnvalue_15 (`KismetMathLibrary.RandomFloatInRange` 0.0 0.05))
  (bind _returnvalue_16 (`KismetMathLibrary.RandomFloatInRange` 0.0 0.05))
  (bind _returnvalue_17 (`KismetMathLibrary.RandomFloatInRange` 0.0 0.05))
  (bind _returnvalue_18 (`KismetMathLibrary.RandomFloatInRange` 0.9 1.0))
  (bind _returnvalue_19 (`KismetMathLibrary.RandomFloatInRange` 0.9 1.0))
  (bind _returnvalue_20 (`KismetMathLibrary.RandomFloatInRange` 0.9 1.0))
  (bind _returnvalue_21 (`KismetMathLibrary.RandomFloatInRange` 0.9 1.0))
  (bind _returnvalue_22 (`KismetMathLibrary.RandomFloatInRange` 0.9 1.0))
  (bind _returnvalue_23 (`KismetMathLibrary.RandomFloatInRange` 0.9 1.0))
  (bind _returnvalue_24 (`KismetMathLibrary.RandomFloatInRange` 0.0 0.1))
  (bind _returnvalue_25 (`KismetMathLibrary.RandomFloatInRange` 0.0 0.1))
  (bind _returnvalue_26 (`KismetMathLibrary.RandomFloatInRange` 0.0 0.1))
  (bind _returnvalue_27 (`KismetMathLibrary.RandomFloatInRange` 0.0 0.1))
  (bind _returnvalue_28 (`KismetMathLibrary.RandomFloatInRange` 0.0 0.1))
  (bind _returnvalue_29 (`KismetMathLibrary.RandomFloatInRange` 0.0 0.1))
  (bind _returnvalue_30 (`KismetMathLibrary.RandomFloatInRange` 0.9 1.0))
  (bind _returnvalue_31 (`KismetMathLibrary.RandomFloatInRange` 0.9 1.0))
  (bind _returnvalue_32 (`KismetMathLibrary.RandomFloatInRange` 0.9 1.0))
  (bind _returnvalue_33 (`KismetMathLibrary.RandomFloatInRange` 0.9 1.0))
  (bind _returnvalue_34 (`KismetMathLibrary.RandomFloatInRange` 0.9 1.0))
  (bind _returnvalue_35 (`KismetMathLibrary.RandomFloatInRange` 0.9 1.0))
  (set `local.MaterialInstance` InputPin)
  ;[1 1 1] Select the base color
  (switch `int` (`KismetMathLibrary.RandomIntegerInRange` 0 4)
    (:`0`
      (set `local.IsBaseColorWhite` true))
    (:`1`
      (set `local.IsBaseColorBlack` true))
    (:`2`
      (set `local.IsBaseColorGrey` true))
    (:`3`
      (set `local.IsBaseColorRed` true))
    (:`4`
      (set `local.IsBaseColorGold` true)))
  ;[1 1 1] Set the base color intensity.
  (if (`local.IsBaseColorBlack`)
    (`MaterialInstanceDynamic.SetVectorParameterValue` (`local.MaterialInstance`) "BlackIntensity" (make `LinearColor` _returnvalue_14 _returnvalue_14 _returnvalue_14))
    (else
      (`MaterialInstanceDynamic.SetVectorParameterValue` (`local.MaterialInstance`) "BlackIntensity" (make `LinearColor` _returnvalue_15 _returnvalue_15 _returnvalue_15))))
  (if (`local.IsBaseColorGrey`)
    (`MaterialInstanceDynamic.SetVectorParameterValue` (`local.MaterialInstance`) "GreyIntensity" (make `LinearColor` _returnvalue_5 _returnvalue_5 _returnvalue_5))
    (else
      (`MaterialInstanceDynamic.SetVectorParameterValue` (`local.MaterialInstance`) "GreyIntensity" (make `LinearColor` _returnvalue_16 _returnvalue_16 _returnvalue_16))))
  (if (`local.IsBaseColorRed`)
    (`MaterialInstanceDynamic.SetVectorParameterValue` (`local.MaterialInstance`) "RedIntensity" (make `LinearColor` _returnvalue_6 _returnvalue_6 _returnvalue_6))
    (else
      (`MaterialInstanceDynamic.SetVectorParameterValue` (`local.MaterialInstance`) "RedIntensity" (make `LinearColor` _returnvalue_17 _returnvalue_17 _returnvalue_17))))
  (if (`local.IsBaseColorGold`)
    (`MaterialInstanceDynamic.SetVectorParameterValue` (`local.MaterialInstance`) "GoldIntensity" (make `LinearColor` _returnvalue_7 _returnvalue_7 _returnvalue_7))
    (else
      (`MaterialInstanceDynamic.SetVectorParameterValue` (`local.MaterialInstance`) "GoldIntensity" (make `LinearColor` _returnvalue_4 _returnvalue_4 _returnvalue_4))))
  (if (`local.IsBaseColorWhite`)
    ;[1 1 1] Set the pattern color.
    (`MaterialInstanceDynamic.SetVectorParameterValue` (`local.MaterialInstance`) "Pttern1BColor" (make `LinearColor` (`KismetMathLibrary.RandomFloatInRange` 0.8 1.0) (`KismetMathLibrary.RandomFloatInRange` 0.0 0.2)))
    (`MaterialInstanceDynamic.SetVectorParameterValue` (`local.MaterialInstance`) "Pttern1GColor" (make `LinearColor` (`KismetMathLibrary.RandomFloatInRange` 0.8 1.0) (`KismetMathLibrary.RandomFloatInRange` 0.0 0.2)))
    (`MaterialInstanceDynamic.SetVectorParameterValue` (`local.MaterialInstance`) "Pttern1RColor" (make `LinearColor` (`KismetMathLibrary.RandomFloatInRange` 0.8 1.0) (`KismetMathLibrary.RandomFloatInRange` 0.0 0.2)))
    (`MaterialInstanceDynamic.SetVectorParameterValue` (`local.MaterialInstance`) "Pttern2BColr" (make `LinearColor` _returnvalue_27 _returnvalue_27 _returnvalue_27))
    (`MaterialInstanceDynamic.SetVectorParameterValue` (`local.MaterialInstance`) "Pttern2GColor" (make `LinearColor` _returnvalue_28 _returnvalue_28 _returnvalue_28))
    (`MaterialInstanceDynamic.SetVectorParameterValue` (`local.MaterialInstance`) "Pttern2RColor" (make `LinearColor` _returnvalue_29 _returnvalue_29 _returnvalue_29))
    ;[1 1 1] Set the pattern intensity.
    (if (`KismetMathLibrary.RandomBoolWithWeight` 0.9)
      (`MaterialInstanceDynamic.SetVectorParameterValue` (`local.MaterialInstance`) "Pattern1BIntensity" (make `LinearColor` _returnvalue_30 _returnvalue_30 _returnvalue_30))
      (else
        (`MaterialInstanceDynamic.SetVectorParameterValue` (`local.MaterialInstance`) "Pattern1BIntensity" (make `LinearColor` 0.0))))
    (if (`KismetMathLibrary.RandomBoolWithWeight` 0.4)
      (`MaterialInstanceDynamic.SetVectorParameterValue` (`local.MaterialInstance`) "Pattern1GIntensity" (make `LinearColor` _returnvalue_31 _returnvalue_31 _returnvalue_31))
      (else
        (`MaterialInstanceDynamic.SetVectorParameterValue` (`local.MaterialInstance`) "Pattern1GIntensity" (make `LinearColor` 0.0))))
    (if (`KismetMathLibrary.RandomBoolWithWeight` 0.4)
      (`MaterialInstanceDynamic.SetVectorParameterValue` (`local.MaterialInstance`) "Pattern1RIntensity" (make `LinearColor` _returnvalue_32 _returnvalue_32 _returnvalue_32))
      (else
        (`MaterialInstanceDynamic.SetVectorParameterValue` (`local.MaterialInstance`) "Pattern1RIntensity" (make `LinearColor` 0.0))))
    (if (`KismetMathLibrary.RandomBoolWithWeight` 0.4)
      (`MaterialInstanceDynamic.SetVectorParameterValue` (`local.MaterialInstance`) "Pattern2BIntensity" (make `LinearColor` _returnvalue_33 _returnvalue_33 _returnvalue_33))
      (else
        (`MaterialInstanceDynamic.SetVectorParameterValue` (`local.MaterialInstance`) "Pattern2BIntensity" (make `LinearColor` 0.0))))
    (if (`KismetMathLibrary.RandomBoolWithWeight` 0.2)
      (`MaterialInstanceDynamic.SetVectorParameterValue` (`local.MaterialInstance`) "Pattern2GIntensity" (make `LinearColor` _returnvalue_34 _returnvalue_34 _returnvalue_34))
      (else
        (`MaterialInstanceDynamic.SetVectorParameterValue` (`local.MaterialInstance`) "Pattern2GIntensity" (make `LinearColor` 0.0))))
    (if (`KismetMathLibrary.RandomBoolWithWeight` 0.2)
      (`MaterialInstanceDynamic.SetVectorParameterValue` (`local.MaterialInstance`) "Pattern2RIntensity" (make `LinearColor` _returnvalue_35 _returnvalue_35 _returnvalue_35))
      (else
        (`MaterialInstanceDynamic.SetVectorParameterValue` (`local.MaterialInstance`) "Pattern2RIntensity" (make `LinearColor` 0.0))))
    (elif (`local.IsBaseColorBlack`)
      ;[1 1 1] Set the pattern color.
      (`MaterialInstanceDynamic.SetVectorParameterValue` (`local.MaterialInstance`) "Pttern1BColor" (make `LinearColor` (`KismetMathLibrary.RandomFloatInRange` 0.8 1.0) (`KismetMathLibrary.RandomFloatInRange` 0.0 0.2)))
      (`MaterialInstanceDynamic.SetVectorParameterValue` (`local.MaterialInstance`) "Pttern1GColor" (make `LinearColor` (`KismetMathLibrary.RandomFloatInRange` 0.8 1.0) (`KismetMathLibrary.RandomFloatInRange` 0.0 0.2)))
      (`MaterialInstanceDynamic.SetVectorParameterValue` (`local.MaterialInstance`) "Pttern1RColor" (make `LinearColor` (`KismetMathLibrary.RandomFloatInRange` 0.8 1.0) (`KismetMathLibrary.RandomFloatInRange` 0.0 0.2)))
      (`MaterialInstanceDynamic.SetVectorParameterValue` (`local.MaterialInstance`) "Pttern2BColr" (make `LinearColor` (`KismetMathLibrary.RandomFloatInRange` 0.8 1.0) (`KismetMathLibrary.RandomFloatInRange` 0.0 0.2)))
      (`MaterialInstanceDynamic.SetVectorParameterValue` (`local.MaterialInstance`) "Pttern2GColor" (make `LinearColor` (`KismetMathLibrary.RandomFloatInRange` 0.8 1.0) (`KismetMathLibrary.RandomFloatInRange` 0.0 0.2)))
      (`MaterialInstanceDynamic.SetVectorParameterValue` (`local.MaterialInstance`) "Pttern2RColor" (make `LinearColor` (`KismetMathLibrary.RandomFloatInRange` 0.8 1.0) (`KismetMathLibrary.RandomFloatInRange` 0.0 0.2)))
      ;[1 1 1] Set the pattern intensity.
      (if (`KismetMathLibrary.RandomBoolWithWeight` 0.9)
        (`MaterialInstanceDynamic.SetVectorParameterValue` (`local.MaterialInstance`) "Pattern1BIntensity" (make `LinearColor` _returnvalue_18 _returnvalue_18 _returnvalue_18))
        (else
          (`MaterialInstanceDynamic.SetVectorParameterValue` (`local.MaterialInstance`) "Pattern1BIntensity" (make `LinearColor` 0.0))))
      (if (`KismetMathLibrary.RandomBoolWithWeight` 0.4)
        (`MaterialInstanceDynamic.SetVectorParameterValue` (`local.MaterialInstance`) "Pattern1GIntensity" (make `LinearColor` _returnvalue_19 _returnvalue_19 _returnvalue_19))
        (else
          (`MaterialInstanceDynamic.SetVectorParameterValue` (`local.MaterialInstance`) "Pattern1GIntensity" (make `LinearColor` 0.0))))
      (if (`KismetMathLibrary.RandomBoolWithWeight` 0.4)
        (`MaterialInstanceDynamic.SetVectorParameterValue` (`local.MaterialInstance`) "Pattern1RIntensity" (make `LinearColor` _returnvalue_20 _returnvalue_20 _returnvalue_20))
        (else
          (`MaterialInstanceDynamic.SetVectorParameterValue` (`local.MaterialInstance`) "Pattern1RIntensity" (make `LinearColor` 0.0))))
      (if (`KismetMathLibrary.RandomBoolWithWeight` 0.4)
        (`MaterialInstanceDynamic.SetVectorParameterValue` (`local.MaterialInstance`) "Pattern2BIntensity" (make `LinearColor` _returnvalue_21 _returnvalue_21 _returnvalue_21))
        (else
          (`MaterialInstanceDynamic.SetVectorParameterValue` (`local.MaterialInstance`) "Pattern2BIntensity" (make `LinearColor` 0.0))))
      (if (`KismetMathLibrary.RandomBoolWithWeight` 0.2)
        (`MaterialInstanceDynamic.SetVectorParameterValue` (`local.MaterialInstance`) "Pattern2GIntensity" (make `LinearColor` _returnvalue_22 _returnvalue_22 _returnvalue_22))
        (else
          (`MaterialInstanceDynamic.SetVectorParameterValue` (`local.MaterialInstance`) "Pattern2GIntensity" (make `LinearColor` 0.0))))
      (if (`KismetMathLibrary.RandomBoolWithWeight` 0.2)
        (`MaterialInstanceDynamic.SetVectorParameterValue` (`local.MaterialInstance`) "Pattern2RIntensity" (make `LinearColor` _returnvalue_23 _returnvalue_23 _returnvalue_23))
        (else
          (`MaterialInstanceDynamic.SetVectorParameterValue` (`local.MaterialInstance`) "Pattern2RIntensity" (make `LinearColor` 0.0))))
      (elif (or (`local.IsBaseColorGrey`) (`local.IsBaseColorGold`))
        ;[1 1 1] Pattern off.
        (`MaterialInstanceDynamic.SetVectorParameterValue` :`self` (`local.MaterialInstance`) :`ParameterName` "Pattern1BIntensity")
        (`MaterialInstanceDynamic.SetVectorParameterValue` :`self` (`local.MaterialInstance`) :`ParameterName` "Pattern1GIntensity")
        (`MaterialInstanceDynamic.SetVectorParameterValue` :`self` (`local.MaterialInstance`) :`ParameterName` "Pattern1RIntensity")
        (`MaterialInstanceDynamic.SetVectorParameterValue` :`self` (`local.MaterialInstance`) :`ParameterName` "Pattern2BIntensity")
        (`MaterialInstanceDynamic.SetVectorParameterValue` :`self` (`local.MaterialInstance`) :`ParameterName` "Pattern2GIntensity")
        (`MaterialInstanceDynamic.SetVectorParameterValue` :`self` (`local.MaterialInstance`) :`ParameterName` "Pattern2RIntensity")
        (elif (`local.IsBaseColorRed`)
          ;[1 1 1] Set the pattern color.
          (`MaterialInstanceDynamic.SetVectorParameterValue` (`local.MaterialInstance`) "Pttern1BColor" (make `LinearColor` _returnvalue _returnvalue _returnvalue))
          (`MaterialInstanceDynamic.SetVectorParameterValue` (`local.MaterialInstance`) "Pttern1GColor" (make `LinearColor` _returnvalue_26 _returnvalue_26 _returnvalue_26))
          (`MaterialInstanceDynamic.SetVectorParameterValue` (`local.MaterialInstance`) "Pttern1RColor" (make `LinearColor` _returnvalue_25 _returnvalue_25 _returnvalue_25))
          (`MaterialInstanceDynamic.SetVectorParameterValue` (`local.MaterialInstance`) "Pttern2BColr" (make `LinearColor` _returnvalue_24 _returnvalue_24 _returnvalue_24))
          (`MaterialInstanceDynamic.SetVectorParameterValue` (`local.MaterialInstance`) "Pttern2GColor" (make `LinearColor` _returnvalue_2 _returnvalue_2 _returnvalue_2))
          (`MaterialInstanceDynamic.SetVectorParameterValue` (`local.MaterialInstance`) "Pttern2RColor" (make `LinearColor` _returnvalue_3 _returnvalue_3 _returnvalue_3))
          ;[1 1 1] Set the pattern intensity.
          (if (`KismetMathLibrary.RandomBoolWithWeight` 0.9)
            (`MaterialInstanceDynamic.SetVectorParameterValue` (`local.MaterialInstance`) "Pattern1BIntensity" (make `LinearColor` _returnvalue_9 _returnvalue_9 _returnvalue_9))
            (else
              (`MaterialInstanceDynamic.SetVectorParameterValue` (`local.MaterialInstance`) "Pattern1BIntensity" (make `LinearColor` 0.0))))
          (if (`KismetMathLibrary.RandomBoolWithWeight` 0.4)
            (`MaterialInstanceDynamic.SetVectorParameterValue` (`local.MaterialInstance`) "Pattern1GIntensity" (make `LinearColor` _returnvalue_10 _returnvalue_10 _returnvalue_10))
            (else
              (`MaterialInstanceDynamic.SetVectorParameterValue` (`local.MaterialInstance`) "Pattern1GIntensity" (make `LinearColor` 0.0))))
          (if (`KismetMathLibrary.RandomBoolWithWeight` 0.4)
            (`MaterialInstanceDynamic.SetVectorParameterValue` (`local.MaterialInstance`) "Pattern1RIntensity" (make `LinearColor` _returnvalue_11 _returnvalue_11 _returnvalue_11))
            (else
              (`MaterialInstanceDynamic.SetVectorParameterValue` (`local.MaterialInstance`) "Pattern1RIntensity" (make `LinearColor` 0.0))))
          (if (`KismetMathLibrary.RandomBoolWithWeight` 0.4)
            (`MaterialInstanceDynamic.SetVectorParameterValue` (`local.MaterialInstance`) "Pattern2BIntensity" (make `LinearColor` _returnvalue_12 _returnvalue_12 _returnvalue_12))
            (else
              (`MaterialInstanceDynamic.SetVectorParameterValue` (`local.MaterialInstance`) "Pattern2BIntensity" (make `LinearColor` 0.0))))
          (if (`KismetMathLibrary.RandomBoolWithWeight` 0.2)
            (`MaterialInstanceDynamic.SetVectorParameterValue` (`local.MaterialInstance`) "Pattern2GIntensity" (make `LinearColor` _returnvalue_13 _returnvalue_13 _returnvalue_13))
            (else
              (`MaterialInstanceDynamic.SetVectorParameterValue` (`local.MaterialInstance`) "Pattern2GIntensity" (make `LinearColor` 0.0))))
          (if (`KismetMathLibrary.RandomBoolWithWeight` 0.2)
            (`MaterialInstanceDynamic.SetVectorParameterValue` (`local.MaterialInstance`) "Pattern2RIntensity" (make `LinearColor` _returnvalue_8 _returnvalue_8 _returnvalue_8))
            (else
              (`MaterialInstanceDynamic.SetVectorParameterValue` (`local.MaterialInstance`) "Pattern2RIntensity" (make `LinearColor` 0.0)))))))))

(fn `UserConstructionScript`)
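; Koi fish actor whose colours and patterns are set through exposed variables.
; The construction script runs the parent's, then creates a dynamic Mat_Koi instance on the mesh's first slot and pushes colour, pattern and emissive values into its vector parameters.
; The event graph holds only disabled stubs, so no chasing behaviour is defined here.
; Pattern2RIntensity feeds a differently named parameter, NonPattern2RIntensitye, unlike the other pattern variables.
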(fn `UserConstructionScript`
  (`parent.UserConstructionScript`)
  ;[1 1 1] Create the dynamic material instance.
  (bind _returnvalue (`PrimitiveComponent.CreateDynamicMaterialInstance` (`self.Mesh`) 0 "/Game/CompleteAnimals/Fishes/FreshWaterFishes/Koi/Materials/Mat_Koi.Mat_Koi"))
  ;[1 1 1] Set the vector parameter values of material instance.
  (bind _output_get (set `self.MaterialInstance` _returnvalue))
  (`MaterialInstanceDynamic.SetVectorParameterValue` _output_get "BlackIntensity" (`self.BlackIntensity`))
  (`MaterialInstanceDynamic.SetVectorParameterValue` _output_get "GreyIntensity" (`self.GreyIntensity`))
  (`MaterialInstanceDynamic.SetVectorParameterValue` _output_get "RedIntensity" (`self.RedIntensity`))
  (`MaterialInstanceDynamic.SetVectorParameterValue` _output_get "GoldIntensity" (`self.GoldIntensity`))
  (`MaterialInstanceDynamic.SetVectorParameterValue` _output_get "Pattern1BIntensity" (`self.Pattern1BIntensity`))
  (`MaterialInstanceDynamic.SetVectorParameterValue` _output_get "Pattern1GIntensity" (`self.Pattern1GIntensity`))
  (`MaterialInstanceDynamic.SetVectorParameterValue` _output_get "Pattern1RIntensity" (`self.Pattern1RIntensity`))
  (`MaterialInstanceDynamic.SetVectorParameterValue` _output_get "Pattern2BIntensity" (`self.Pattern2BIntensity`))
  (`MaterialInstanceDynamic.SetVectorParameterValue` _output_get "Pattern2GIntensity" (`self.Pattern2GIntensity`))
  (`MaterialInstanceDynamic.SetVectorParameterValue` _output_get "NonPattern2RIntensitye" (`self.Pattern2RIntensity`))
  (`MaterialInstanceDynamic.SetVectorParameterValue` _output_get "Emissive" (`self.Emissive`)))
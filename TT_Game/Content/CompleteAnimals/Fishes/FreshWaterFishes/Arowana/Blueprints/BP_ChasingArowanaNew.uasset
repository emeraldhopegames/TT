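; Arowana fish Blueprint whose only active logic is picking the fish's color variant in the Construction Script.
; A switch on TextureType creates a dynamic material instance on mesh slot 0 from the white, yellow, blue or red Arowana material, with white as the default.
; The parent construction script runs first, and the event graph holds only disabled stub events, so this Blueprint adds no chasing logic of its own.
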(fn `UserConstructionScript`
  (`parent.UserConstructionScript`)
  ;[1 1 1] Create dynamic material instance.
  (switch `int` (`self.TextureType`)
    (:`Default`
      (`PrimitiveComponent.CreateDynamicMaterialInstance` (`self.Mesh`) 0 "/Game/CompleteAnimals/Fishes/FreshWaterFishes/Arowana/Materials/Mat_ArowanaWhite.Mat_ArowanaWhite" :!label _label))
    (:`0`
      (goto _label))
    (:`1`
      (`PrimitiveComponent.CreateDynamicMaterialInstance` (`self.Mesh`) 0 "/Game/CompleteAnimals/Fishes/FreshWaterFishes/Arowana/Materials/Mat_ArowanaYellow.Mat_ArowanaYellow"))
    (:`2`
      (`PrimitiveComponent.CreateDynamicMaterialInstance` (`self.Mesh`) 0 "/Game/CompleteAnimals/Fishes/FreshWaterFishes/Arowana/Materials/Mat_ArowanaBlue.Mat_ArowanaBlue"))
    (:`3`
      (`PrimitiveComponent.CreateDynamicMaterialInstance` (`self.Mesh`) 0 "/Game/CompleteAnimals/Fishes/FreshWaterFishes/Arowana/Materials/Mat_ArowanaRed.Mat_ArowanaRed"))))
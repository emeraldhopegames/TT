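; BP_ChasingGoldfishNew is a goldfish actor Blueprint that sets up its material appearance per instance.
; The construction script runs the parent's script, then creates a dynamic Mat_Goldfish instance on the mesh's first material slot.
; It feeds three texture intensity variables into that instance as vector parameters.
; The event graph holds only disabled stub events, so this graph adds no chasing logic.
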(fn `UserConstructionScript`
  (`parent.UserConstructionScript`)
  ;[1 1 1] Create dynamic material instance.
  (bind _returnvalue (`PrimitiveComponent.CreateDynamicMaterialInstance` (`self.Mesh`) 0 "/Game/CompleteAnimals/Fishes/FreshWaterFishes/Goldfish/Materials/Mat_Goldfish.Mat_Goldfish"))
  (`MaterialInstanceDynamic.SetVectorParameterValue` _returnvalue "Texture2Intensity" (`self.Texture2Intensity`))
  (`MaterialInstanceDynamic.SetVectorParameterValue` _returnvalue "Texture3Intensity" (`self.Texture3Intensity`))
  (`MaterialInstanceDynamic.SetVectorParameterValue` _returnvalue "Texture4Intensity" (`self.Texture4Intensity`)))
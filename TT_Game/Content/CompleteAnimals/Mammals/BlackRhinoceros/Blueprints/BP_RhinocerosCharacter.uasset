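; Black rhinoceros character that adapts its body to terrain and can ragdoll, die and stand back up.
; Each tick it traces all four feet for smoothed IK targets, derives pelvis transform from them, and averages a grid of traces for head height.
; Two or fewer grounded feet while walking triggers ragdoll; four allow timed recovery by blending out physics.
; Point damage gives a brief partial-physics reaction, with a left-click damage test.
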(event `self.ReceiveTick`
  (params (DeltaSeconds :type "Float (single-precision)"))
  (bind _returnvalue (* (`SceneComponent.GetUpVector` (`self.CapsuleComponent`)) (`self.TraceHeadDistance`)))
  (bind _returnvalue_2 (/ (+ (`SceneComponent.GetSocketLocation` (`self.Mesh`) (`self.Pelvis`)) (`SceneComponent.GetSocketLocation` (`self.Mesh`) "Head")) 2.0))
  (bind (_remainder _returnvalue_3) (`KismetMathLibrary.FMod` (`KismetMathLibrary.Conv_IntToDouble` (`self.CurrentTraceNumber`)) (`KismetMathLibrary.Conv_IntToDouble` (+ (`self.HorizontalDivisionNumber`) 1))))
  (bind _returnvalue_4 (+ (+ (* (`SceneComponent.GetRightVector` (`self.CapsuleComponent`)) (* _remainder (`self.TraceGridWidth`))) (* (`SceneComponent.GetForwardVector` (`self.CapsuleComponent`)) (* _returnvalue_3 (`self.TraceGridHeight`)))) (+ (+ (+ (`SceneComponent.GetSocketLocation` (`self.Mesh`) "Neck_1") (* (`KismetMathLibrary.GetRightVector` (`SceneComponent.GetSocketRotation` (`self.Mesh`) "Neck_1")) (`self.NeckLength`))) (* (* (`SceneComponent.GetForwardVector` (`self.CapsuleComponent`)) (`self.TraceHalfHeight`)) -1.0)) (* (* (`SceneComponent.GetRightVector` (`self.CapsuleComponent`)) (`self.TraceHalfWidth`)) -1.0))))
  (set `self.DeltaSeconds` DeltaSeconds)
  ;[1 1 1] Set the BoneTransAlpha.
  (set `self.BoneTransAlpha` (`KismetMathLibrary.FInterpTo` (`self.BoneTransAlpha`) (`KismetMathLibrary.SelectFloat` 0.0 1.0 (or (or (or (or (or (not (`self.IsNotRagdoll`)) (`self.StandingUp`)) (`self.IsAttacking`)) (`self.IsHitting`)) (`NavMovementComponent.IsSwimming` (`self.CharacterMovement`))) (`NavMovementComponent.IsFalling` (`self.CharacterMovement`)))) (`self.DeltaSeconds`) 5.0))
  ;[1 1 1] Calculate Foot and Pelvis transform.
  (`self.FootPlacement`)
  (`self.CalculatePelvisTransform`)
  ;[1 1 1] Judge in which direction the rhinoceros is lie down.
  (set `self.DownRight` (>= (`KismetMathLibrary.Dot_VectorVector` (`KismetMathLibrary.GetForwardVector` (`SceneComponent.GetSocketRotation` (`self.Mesh`) "Pelvis")) (0.0 0.0 1.0)) 0.0))
  ;[1 1 1] IsNotRagdoll?
  (if (`self.IsNotRagdoll`)
    ;[1 1 1] Calculate the HeadHeight from the average value of the heights of the HorizontalDivisionNumber × VerticalDivisionNumber points.
    ;;[1 1 1] Trace for lattice points.
    (for _index (range (+ (`self.MaxTraceNumber`) 1))
      (set `self.CurrentTraceNumber` _index)
      (bind _outhit (`KismetSystemLibrary.LineTraceSingle` :`Start` (- _returnvalue_4 _returnvalue) :`End` (+ _returnvalue_4 _returnvalue) :`TraceChannel` "TraceTypeQuery1" :`bTraceComplex` true :`TraceColor` (struct :`R` 1.0 :`G` 0.724743 :`A` 1.0) :`TraceHitColor` (struct :`G` 0.08531 :`B` 1.0 :`A` 1.0)))
      (bind (_bblockinghit _binitialoverlap _time _distance _location _impactpoint) (`GameplayStatics.BreakHitResult` _outhit))
      (if _bblockinghit
        (set `self.HeadHeightSum` (+ (`self.HeadHeightSum`) (`KismetMathLibrary.VSize` (- _returnvalue_4 _impactpoint))))
        (`/Engine/EditorBlueprintResources/StandardMacros.IncrementInt` (`self.HeadHeightColisionNum`))))
    ;;[1 1 1] Set the HeadHeight.
    (if (!= (`self.HeadHeightColisionNum`) 0)
      (set `self.HeadHeight` (`KismetMathLibrary.FInterpTo` (`self.HeadHeight`) (/ (`self.HeadHeightSum`) (`KismetMathLibrary.Conv_IntToDouble` (`self.HeadHeightColisionNum`))) (`self.DeltaSeconds`) 1.0)))
    (set `self.HeadHeightSum` 0.0)
    (set `self.HeadHeightColisionNum` 0)
    (else
      ;[1 1 1] Set the RagdollTime.
      (set `self.RagDollTime` (+ (`self.RagDollTime`) (`self.DeltaSeconds`)))
      ;[1 1 1] Recovering?
      (if (`self.Recovering`)
        ;[1 1 1] Set the PhysicsAlpha.
        (set `self.PhysicsAlpha` (`KismetMathLibrary.FInterpTo` (`self.PhysicsAlpha`) 0.0 (`self.DeltaSeconds`) 3.0))
        (`SkeletalMeshComponent.SetAllBodiesBelowPhysicsBlendWeight` (`self.Mesh`) (`self.Pelvis`) (`self.PhysicsAlpha`) false true)
        ;[1 1 1] RecoveringTime less than 1?
        (set `self.RecoveringTIme` (+ (`self.RecoveringTIme`) (`self.DeltaSeconds`)))
        (if (not (< (`self.RecoveringTIme`) 1.0))
          ;[1 1 1] Playing Rebirth animation by turning off physical simulation. The length of the reverse animation is 2.66666 seconds.
          (`SkeletalMeshComponent.SetAllBodiesBelowSimulatePhysics` (`self.Mesh`) (`self.Pelvis`) false true)
          (set `self.Recovering` false)
          (set `self.IsNotRagdoll` true)
          (`CharacterMovementComponent.SetMovementMode` (`self.CharacterMovement`) "MOVE_Walking" 0)
          (set `self.StandingUp` true)
          (`KismetSystemLibrary.Delay` 2.66666)
          (set `self.StandingUp` false)
          ;[1 1 1] Set the PelvisLocation
          (set `self.PelvisLocation` (`SceneComponent.GetSocketLocation` (`self.Mesh`) (`self.Pelvis`))))
        (else
          ;[1 1 1] Calculate Capsule location.
          (bind (_outhit_2 _returnvalue_5) (`KismetSystemLibrary.LineTraceSingle` _returnvalue_2 (`KismetMathLibrary.MakeVector` (.x _returnvalue_2) (.y _returnvalue_2) (- (.z _returnvalue_2) (`self.TraceDistance`))) "TraceTypeQuery1"))
          (bind _output_get (set `self.CapsuleLocation` (`KismetMathLibrary.SelectVector` (`KismetMathLibrary.MakeVector` (.x (`.Location` (`GameplayStatics.BreakHitResult` _outhit_2))) (.y (`.Location` (`GameplayStatics.BreakHitResult` _outhit_2))) (+ (.z (`.Location` (`GameplayStatics.BreakHitResult` _outhit_2))) (* (`self.PelvisHeight`) 1.5))) _returnvalue_2 _returnvalue_5)))
          (`SceneComponent.K2_SetWorldLocation` (`self.CapsuleComponent`) _output_get false false))))))

(event `self.ReceivePointDamage`
  (params (Damage :type "Float (single-precision)") (DamageType :type "DamageType Object Reference") (HitLocation :type "Vector Structure") (HitNormal :type "Vector Structure") (HitComponent :type "PrimitiveComponent Object Reference") (BoneName :type Name) (ShotFromDirection :type "Vector Structure") (InstigatedBy :type "Controller Object Reference") (DamageCauser :type "Actor Object Reference") (HitInfo :type "HitResult Structure (by ref)"))
  ;[1 1 1] Damage using physics simulation.
  (`SkeletalMeshComponent.SetAllBodiesBelowSimulatePhysics` (`self.Mesh`) (`self.Spine_1`) true true)
  (`SkeletalMeshComponent.SetAllBodiesBelowPhysicsBlendWeight` (`self.Mesh`) (`self.Spine_1`) 0.5 false true)
  (`SkeletalMeshComponent.SetAllBodiesBelowSimulatePhysics` (`self.Mesh`) (`self.Thigh_L`) true true)
  (`SkeletalMeshComponent.SetAllBodiesBelowPhysicsBlendWeight` (`self.Mesh`) (`self.Thigh_L`) 0.5 false true)
  (`SkeletalMeshComponent.SetAllBodiesBelowSimulatePhysics` (`self.Mesh`) (`self.Thigh_R`) true true)
  (`SkeletalMeshComponent.SetAllBodiesBelowPhysicsBlendWeight` (`self.Mesh`) (`self.Thigh_R`) 0.5 false true)
  (`PrimitiveComponent.AddImpulseAtLocation` (`self.Mesh`) (* (`KismetMathLibrary.Normal` (- HitLocation ShotFromDirection)) Damage) HitLocation BoneName)
  (`KismetSystemLibrary.Delay` 0.5)
  (`SkeletalMeshComponent.SetAllBodiesBelowSimulatePhysics` (`self.Mesh`) (`self.Pelvis`) false true))

(event `Key|LeftMouseButton`
  (params (Key :type "Key Structure"))
  (bind _returnvalue (`SceneComponent.GetSocketLocation` (`self.Mesh`) "Neck_1"))
  ;[1 1 1] For damage testing.
  (:`Pressed`
    (bind _outhit (`KismetSystemLibrary.LineTraceSingle` :`Start` _returnvalue :`End` (+ _returnvalue (* (`KismetMathLibrary.GetForwardVector` (`self.GetControlRotation`)) 10000.0)) :`TraceChannel` "TraceTypeQuery1" :`DrawDebugType` "ForOneFrame"))
    (`GameplayStatics.ApplyPointDamage` (`.HitActor` (`GameplayStatics.BreakHitResult` _outhit)) 1000.0 _returnvalue _outhit (`self.GetController`) self "/Script/Engine.DamageType")))

(fn `CalculatePelvisTransform`
  (bind _returnvalue (- 90.0 (`KismetMathLibrary.DegAcos` (`KismetMathLibrary.Dot_VectorVector` (`KismetMathLibrary.Normal` (- (+ (`self.L_Hand_EffectorLoc`) (`self.R_Hand_EffectorLoc`)) (+ (`self.L_Foot_EffectorLoc`) (`self.R_Foot_EffectorLoc`)))) (0.0 0.0 1.0)))))
  ;[1 1 1] Calculate Pelvis rotation.
  (set `self.PelvisRotation` (`KismetMathLibrary.RInterpTo` (`self.PelvisRotation`) (`KismetMathLibrary.RotatorFromAxisAndAngle` (1.0 0.0 0.0) _returnvalue) (`self.DeltaSeconds`) 10.0))
  ;[1 1 1] Calculate Pelvis location.
  (set `self.PelvisLocation` (`KismetMathLibrary.VInterpTo` (`self.PelvisLocation`) (+ (- (- (`SceneComponent.K2_GetComponentLocation` (`self.CapsuleComponent`)) (* (* (`SceneComponent.GetForwardVector` (`self.CapsuleComponent`)) (`self.PelvisDistance`)) (`KismetMathLibrary.DegCos` _returnvalue))) (* (`KismetMathLibrary.MakeVector` 0.0 0.0 (`KismetMathLibrary.DegSin` _returnvalue)) (`self.PelvisDistance`))) (`KismetMathLibrary.MakeVector` 0.0 0.0 (`KismetMathLibrary.SelectFloat` (`self.PelvisHeight`) 0.0 (`self.IsNotRagdoll`)))) (`self.DeltaSeconds`) 10.0)))

(fn `CanJumpInternal`
  (returns (ReturnValue :type Boolean))
  (return (and (and (and (and (`CharacterMovementComponent.IsWalking` (`self.CharacterMovement`)) (`self.IsNotRagdoll`)) (not (`self.IsAttacking`))) (not (`self.IsHitting`))) (not (`self.IsEating`)))))

(fn `Death`
  (set `self.IsLived` false)
  (`self.ToRagdoll`))

(fn `FootPlacement`
  (bind _groundreachedfeetnum (`self.GroundReachedFeetNum`))
  (bind _groundreachedfeetnum_2 (`self.GroundReachedFeetNum`))
  (bind _groundreachedfeetnum_3 (`self.GroundReachedFeetNum`))
  (bind _groundreachedfeetnum_4 (`self.GroundReachedFeetNum`))
  (set `self.GroundReachedFeetNum` 0)
  ;[1 1 1] Calculate the L_FootEffectorLoc's Location and L_Foot's rotation.
  (bind (_legikeffectorloc _footrot _reachtheground) (`self.TraceIKEffector` (`self.L_Foot`) (`self.IKTraceDistance`) (`self.IKHeightOffset`)))
  (set `self.GroundReachedFeetNum` (`KismetMathLibrary.SelectInt` (+ _groundreachedfeetnum_2 1) _groundreachedfeetnum_2 _reachtheground))
  ;[1 1 1] Set the left foot rotation.
  (set `self.L_Foot_Rot` (`KismetMathLibrary.RInterpTo` (`self.L_Foot_Rot`) _footrot (`GameplayStatics.GetWorldDeltaSeconds`) (`self.FootRotInterpSpeed`)))
  ;[1 1 1] Set the left foot IK effecter location.
  (set `self.L_Foot_EffectorLoc` (`KismetMathLibrary.VInterpTo` (`self.L_Foot_EffectorLoc`) _legikeffectorloc (`GameplayStatics.GetWorldDeltaSeconds`) (`self.IKInterpSpeed`)))
  ;[1 1 1] Calculate the R_FootEffectorLoc's Location and R_Foot's rotation.
  (bind (_legikeffectorloc_2 _footrot_2 _reachtheground_2) (`self.TraceIKEffector` (`self.R_Foot`) (`self.IKTraceDistance`) (`self.IKHeightOffset`)))
  (set `self.GroundReachedFeetNum` (`KismetMathLibrary.SelectInt` (+ _groundreachedfeetnum 1) _groundreachedfeetnum _reachtheground_2))
  ;[1 1 1] Set the right foot rotation.
  (set `self.R_Foot_Rot` (`KismetMathLibrary.RInterpTo` (`self.R_Foot_Rot`) _footrot_2 (`GameplayStatics.GetWorldDeltaSeconds`) (`self.FootRotInterpSpeed`)))
  ;[1 1 1] Set the right foot effector location.
  (set `self.R_Foot_EffectorLoc` (`KismetMathLibrary.VInterpTo` (`self.R_Foot_EffectorLoc`) _legikeffectorloc_2 (`GameplayStatics.GetWorldDeltaSeconds`) (`self.IKInterpSpeed`)))
  ;[1 1 1] Calculate the L_HandEffectorLoc's Location and L_Hand's rotation.
  (bind (_legikeffectorloc_3 _footrot_3 _reachtheground_3) (`self.TraceIKEffector` (`self.L_Hand`) (`self.IKTraceDistance`) (`self.IKHeightOffset`)))
  (set `self.GroundReachedFeetNum` (`KismetMathLibrary.SelectInt` (+ _groundreachedfeetnum_3 1) _groundreachedfeetnum_3 _reachtheground_3))
  ;[1 1 1] Set the left hand rotation.
  (set `self.L_Hand_Rot` (`KismetMathLibrary.RInterpTo` (`self.L_Hand_Rot`) _footrot_3 (`GameplayStatics.GetWorldDeltaSeconds`) (`self.FootRotInterpSpeed`)))
  ;[1 1 1] Set the left hand effector location.
  (set `self.L_Hand_EffectorLoc` (`KismetMathLibrary.VInterpTo` (`self.L_Hand_EffectorLoc`) _legikeffectorloc_3 (`GameplayStatics.GetWorldDeltaSeconds`) (`self.IKInterpSpeed`)))
  ;[1 1 1] Calculate the R_HandEffectorLoc's Location and R_Hand's rotation.
  (bind (_legikeffectorloc_4 _footrot_4 _reachtheground_4) (`self.TraceIKEffector` (`self.R_Hand`) (`self.IKTraceDistance`) (`self.IKHeightOffset`)))
  (set `self.GroundReachedFeetNum` (`KismetMathLibrary.SelectInt` (+ _groundreachedfeetnum_4 1) _groundreachedfeetnum_4 _reachtheground_4))
  ;[1 1 1] Set the right hand rotation.
  (set `self.R_Hand_Rot` (`KismetMathLibrary.RInterpTo` (`self.R_Hand_Rot`) _footrot_4 (`GameplayStatics.GetWorldDeltaSeconds`) (`self.FootRotInterpSpeed`)))
  ;[1 1 1] Set the right hand effector location.
  (set `self.R_Hand_EffectorLoc` (`KismetMathLibrary.VInterpTo` (`self.R_Hand_EffectorLoc`) _legikeffectorloc_4 (`GameplayStatics.GetWorldDeltaSeconds`) (`self.IKInterpSpeed`)))
  ;[1 1 1] If there are two or less feet on the ground, ToRagdoll.
  (if (`self.IsNotRagdoll`)
    (if (`CharacterMovementComponent.IsWalking` (`self.CharacterMovement`))
      (if (`self.Recovering`)
        _
        (elif (`self.StandingUp`)
          _
          (elif (<= (`self.GroundReachedFeetNum`) 2)
            (`self.ToRagdoll`)))))
    (else
      ;[1 1 1] It stands up when the four feet are grounded.
      (if (== (`self.GroundReachedFeetNum`) 4)
        (if (`self.Recovering`)
          _
          (elif (not (`self.StandingUp`))
            (`self.StandUp`)))))))

(fn `Rebirth`
  (set `self.IsLived` true)
  (`self.StandUp`))

(fn `StandUp`
  ;[1 1 1] If IsNotRagdoll is false, Set Recovering, RicoveriingTime and PhysicsAlpha.
  (if (`self.IsLived`)
    (if (`self.IsNotRagdoll`)
      _
      (elif (> (`self.RagDollTime`) 2.0)
        (set `self.Recovering` true)
        (set `self.RecoveringTIme` 0.0)
        (set `self.PhysicsAlpha` 1.0)))))

(fn `ToRagdoll`
  ;[1 1 1] Set the physics simulation.
  (set `self.IsNotRagdoll` false)
  (`SkeletalMeshComponent.SetAllBodiesBelowSimulatePhysics` (`self.Mesh`) (`self.Pelvis`) true true)
  (`SkeletalMeshComponent.SetAllBodiesBelowPhysicsBlendWeight` (`self.Mesh`) (`self.Pelvis`) 1.0 false true)
  (`CharacterMovementComponent.SetMovementMode` (`self.CharacterMovement`) "MOVE_None" 0)
  ;[1 1 1] Set the Cupsule location.
  (set `self.CapsuleLocation` (`SceneComponent.K2_GetComponentLocation` (`self.CapsuleComponent`)))
  ;[1 1 1] Set the RagdollTime Zero.
  (set `self.RagDollTime` 0.0))

(fn `TraceIKEffector`
  (params (FootName :type Name) (TraceDistance :type "Float (double-precision)" :default 50.0) (HeightOffset :type "Float (double-precision)" :default 10.0))
  (returns (LegIKEffectorLoc :type "Vector Structure") (FootRot :type "Rotator Structure") (ReachTheGround :type Boolean))
  (locals (GroundNormal :type "Vector Structure") (InitialFootLocation :type "Vector Structure") (InitialFootRotation :type "Rotator Structure") (DoesReachThaGround :type Boolean))
  (bind _x (.x (`local.InitialFootLocation`)))
  (bind _y (.y (`local.InitialFootLocation`)))
  (bind _z (.z (`local.InitialFootLocation`)))
  (bind (_x_2 _y_2 _z_2) (`KismetMathLibrary.BreakRotIntoAxes` (`local.InitialFootRotation`)))
  (bind _returnvalue (`KismetMathLibrary.Cross_VectorVector` _y_2 (`local.GroundNormal`)))
  (bind _returnvalue_2 (`KismetMathLibrary.DegAsin` (`KismetMathLibrary.VSize` _returnvalue)))
  ;[1 1 1] Set the InitialFootLocation and InitialFootRotation  for use later.
  (set `local.InitialFootLocation` (`SceneComponent.GetSocketLocation` (`self.Mesh`) FootName))
  (set `local.InitialFootRotation` (`SceneComponent.GetSocketRotation` (`self.Mesh`) FootName))
  ;[1 1 1] Calculate the location of foot.
  ;;[1 1 1] Trace from foot location to the location lowered by the TraceDistance from the location of the foot
  (bind _outactors (`GameplayStatics.GetAllActorsOfClass` "BP_RhinocerosCharacter_C"))
  (bind (_outhit _returnvalue_3) (`KismetSystemLibrary.LineTraceSingle` (`KismetMathLibrary.MakeVector` _x _y (+ _z TraceDistance)) (`KismetMathLibrary.MakeVector` _x _y (- _z TraceDistance)) "TraceTypeQuery1" true _outactors))
  ;;[1 1 1] Set the DoesReachTheGround and GroundNormal  for use later.
  (set `local.DoesReachThaGround` _returnvalue_3)
  (bind (_bblockinghit _binitialoverlap _time _distance _location _impactpoint _normal) (`GameplayStatics.BreakHitResult` _outhit))
  (set `local.GroundNormal` _normal)
  (return (`KismetMathLibrary.SelectVector` (`KismetMathLibrary.MakeVector` (.x _location) (.y _location) (+ (.z _location) HeightOffset)) (`local.InitialFootLocation`) (`local.DoesReachThaGround`)) (`KismetMathLibrary.SelectRotator` (`KismetMathLibrary.MakeRotationFromAxes` (`KismetMathLibrary.RotateAngleAxis` _x_2 _returnvalue_2 _returnvalue) (`local.GroundNormal`) (`KismetMathLibrary.RotateAngleAxis` _z_2 _returnvalue_2 _returnvalue)) (`local.InitialFootRotation`) (`local.DoesReachThaGround`)) (`local.DoesReachThaGround`)))

(fn `UserConstructionScript`
  (bind _scale (`self.Scale`))
  ;[1 1 1] Set the Scale.
  (set `self.Scale` (.z (.scale (`self.GetTransform`))))
  ;[1 1 1] Set the scale dependent variables.
  (set `self.IKTraceDistance` (* (* (`CapsuleComponent.CapsuleHalfHeight` (`self.CapsuleComponent`)) 2.0) _scale))
  (set `self.IKHeightOffset` (* (`self.IKHeightOffset`) _scale))
  (set `self.PelvisDistance` (* (`self.PelvisDistance`) _scale))
  (set `self.PelvisHeight` (* (`self.PelvisHeight`) _scale))
  (set `self.NeckLength` (* (`self.NeckLength`) _scale))
  (set `self.TraceDistance` (* (`self.TraceDistance`) _scale))
  (set `self.TraceHeadDistance` (* (`self.TraceHeadDistance`) _scale))
  (set `self.TraceHalfHeight` (* (`self.TraceHalfHeight`) _scale))
  (set `self.TraceHalfWidth` (* (`self.TraceHalfWidth`) _scale))
  ;[1 1 1] Set the MaxTraceNumber
  (set `self.MaxTraceNumber` (- (* (+ (`self.VerticalDivisionNumber`) 1) (+ (`self.HorizontalDivisionNumber`) 1)) 1))
  ;[1 1 1] Set the TraceGridHeight
  (set `self.TraceGridHeight` (/ (* (`self.TraceHalfHeight`) 2.0) (`KismetMathLibrary.Conv_IntToDouble` (`self.VerticalDivisionNumber`))))
  ;[1 1 1] Set the TraceGridWidth
  (set `self.TraceGridWidth` (/ (* (`self.TraceHalfWidth`) 2.0) (`KismetMathLibrary.Conv_IntToDouble` (`self.HorizontalDivisionNumber`)))))
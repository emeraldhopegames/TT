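; Playable wolf character that can shapeshift into a penguin or BeastBoy and switch between running gaits.
; Keys 1 and 2 spawn the new form in place, possess it, set its spring arm to the control rotation and destroy the wolf.
; Left Shift, C and T set IsRunning and MaxRunForwardSpeed for gallop, canter and trot.
; Releasing C or T clears IsRunning, while Left Shift has no release handler here.
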(event `Key|One`
  (params (Key :type "Key Structure"))
  (bind _returnvalue (`GameplayStatics.GetPlayerController` 0))
  (bind _returnvalue_2 (`self.GetTransform`))
  (:`Pressed`
    (bind _returnvalue_3 (`|SpawnActorFromClass` "/Game/CompleteAnimals/Birds/Penguin/Blueprints/BP_PenguinThirdPersonCharacter.BP_PenguinThirdPersonCharacter_C" (`KismetMathLibrary.MakeTransform` (`KismetMathLibrary.MakeVector` (.x (.location _returnvalue_2)) (.y (.location _returnvalue_2)) (.z (.location _returnvalue_2))) (.rotation _returnvalue_2)) "Undefined" "MultiplyWithRoot" null null))
    (`Controller.Possess` _returnvalue _returnvalue_3)
    (`SceneComponent.K2_SetRelativeRotation` (`/Game/CompleteAnimals/Birds/Penguin/Blueprints/BP_PenguinThirdPersonCharacter.SpringArm` _returnvalue_3) (`Controller.GetControlRotation` _returnvalue) false false)
    (`self.K2_DestroyActor`)))

(event `Key|Two`
  (params (Key :type "Key Structure"))
  (bind _returnvalue (`self.GetTransform`))
  (bind _returnvalue_2 (`GameplayStatics.GetPlayerController` 0))
  (:`Pressed`
    (bind _returnvalue_3 (`|SpawnActorFromClass` "/Game/Blueprints/BP_BeastBoy.BP_BeastBoy_C" (`KismetMathLibrary.MakeTransform` (`KismetMathLibrary.MakeVector` (.x (.location _returnvalue)) (.y (.location _returnvalue)) (.z (.location _returnvalue))) (.rotation _returnvalue)) "Undefined" "MultiplyWithRoot" null null))
    (`Controller.Possess` _returnvalue_2 _returnvalue_3)
    (`SceneComponent.K2_SetRelativeRotation` (`/Game/Blueprints/SandboxCharacter_CMC.SpringArm` _returnvalue_3) (`Controller.GetControlRotation` _returnvalue_2) false false)
    (`self.K2_DestroyActor`)))

(event `Key|LeftShift`
  (params (Key :type "Key Structure"))
  ;[1 1 1] G, C, T:Gallop, Canter, Trot
  (:`Pressed`
    (set `self.IsRunning` true)
    (set `self.MaxRunForwardSpeed` 4.0)))

(event `Key|C`
  (params (Key :type "Key Structure"))
  ;[1 1 1] G, C, T:Gallop, Canter, Trot
  (:`Pressed`
    (set `self.IsRunning` true)
    (set `self.MaxRunForwardSpeed` 3.0))
  (:`Released`
    (set `self.IsRunning` false :!label _label)))

(event `Key|T`
  (params (Key :type "Key Structure"))
  ;[1 1 1] G, C, T:Gallop, Canter, Trot
  (:`Pressed`
    (set `self.IsRunning` true)
    (set `self.MaxRunForwardSpeed` 2.0))
  (:`Released`
    (goto _label)))

(fn `UserConstructionScript`
  (`parent.UserConstructionScript`)
  (set `self.MaxRunForwardSpeed` 4.0))
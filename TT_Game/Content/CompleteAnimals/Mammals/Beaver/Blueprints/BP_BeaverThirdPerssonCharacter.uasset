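; Beaver third-person character that adds swimming movement on top of its parent class's behavior.
; W and S set a target vertical speed, which Tick smooths with FInterpTo.
; While the movement component reports swimming, Tick moves the capsule with swept local offsets from forward and vertical speed and yaws it by turn speed.
; The construction script overrides the maximum forward run speed.
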(event `Key|W`
  (params (Key :type "Key Structure"))
  ;[1 1 1] W, S:upDownSpeed Change
  (:`Pressed`
    (set `self.AimUpDownSpeed` 1.0))
  (:`Released`
    (set `self.AimUpDownSpeed` 0.0 :!label _label)))

(event `self.ReceiveTick`
  (params (DeltaSeconds :type "Float (single-precision)"))
  (`parent.ReceiveTick` DeltaSeconds)
  ;[1 1 1] IsSwimming?
  (if (`NavMovementComponent.IsSwimming` (`self.CharacterMovement`))
    ;[1 1 1] Swimming
    (`SceneComponent.K2_AddLocalOffset` (`self.CapsuleComponent`) (`KismetMathLibrary.MakeVector` 0.0 (* (* (`self.ForwardSpeed`) (`GameplayStatics.GetWorldDeltaSeconds`)) (`self.SwimSpeedMultiplier`)) (* (* (`self.UpDownSpeed`) (`GameplayStatics.GetWorldDeltaSeconds`)) (`self.SwimSpeedMultiplier`))) true false)
    (`SceneComponent.K2_AddLocalRotation` (`self.CapsuleComponent`) (`KismetMathLibrary.MakeRotator` 0.0 0.0 (* (`self.TurnSpeed`) (`GameplayStatics.GetWorldDeltaSeconds`))) false false)
    ;[1 1 1] Set UpDownSpeed
    (set `self.UpDownSpeed` (`KismetMathLibrary.FInterpTo` (`self.UpDownSpeed`) (`self.AimUpDownSpeed`) (`GameplayStatics.GetWorldDeltaSeconds`) 2.0))))

(event `Key|S`
  (params (Key :type "Key Structure"))
  ;[1 1 1] W, S:upDownSpeed Change
  (:`Pressed`
    (set `self.AimUpDownSpeed` -1.0))
  (:`Released`
    (goto _label)))

(fn `UserConstructionScript`
  (`parent.UserConstructionScript`)
  (set `self.MaxRunForwardSpeed` 4.0))
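; Bear character Blueprint that drives procedural body animation, swimming, melee attacks, hit reactions and ragdoll death and revival.
; Tick computes pelvis transforms from hand and foot sockets and averages a grid of downward traces for head height.
; Timed attack flags enable hand-swept traces that apply point damage; incoming damage blends in physics below the pelvis.
; While ragdolled the capsule follows the body, and recovery blends physics out before standing up.
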(event `self.ReceiveTick`
  (params (DeltaSeconds :type "Float (single-precision)"))
  (bind _scale (`self.Scale`))
  (bind _returnvalue (* (`SceneComponent.GetUpVector` (`self.CapsuleComponent`)) (`self.TraceHeadDistance`)))
  (bind (_remainder _returnvalue_2) (`KismetMathLibrary.FMod` (`KismetMathLibrary.Conv_IntToDouble` (`self.CurrentTraceNumber`)) (`KismetMathLibrary.Conv_IntToDouble` (+ (`self.HorizontalDivisionNumber`) 1))))
  (bind _returnvalue_3 (+ (+ (* (`SceneComponent.GetRightVector` (`self.CapsuleComponent`)) (* _remainder (`self.TraceGridWidth`))) (* (`SceneComponent.GetForwardVector` (`self.CapsuleComponent`)) (* _returnvalue_2 (`self.TraceGridHeight`)))) (+ (+ (+ (`SceneComponent.GetSocketLocation` (`self.Mesh`) "Spine_3") (* (`KismetMathLibrary.GetRightVector` (`SceneComponent.GetSocketRotation` (`self.Mesh`) "Spine_3")) (`self.NeckLength`))) (* (* (`SceneComponent.GetForwardVector` (`self.CapsuleComponent`)) (`self.TraceHalfHeight`)) -1.0)) (* (* (`SceneComponent.GetRightVector` (`self.CapsuleComponent`)) (`self.TraceHalfWidth`)) -1.0))))
  (set `self.DeltaSeconds` DeltaSeconds)
  ;[1 1 1] Set the BoneTransAlpha.
  (set `self.BoneTransAlpha` (`KismetMathLibrary.FInterpTo` (`self.BoneTransAlpha`) (`KismetMathLibrary.SelectFloat` 0.0 1.0 (or (or (or (or (or (`self.IsStanding`) (not (`self.IsNotRagdoll`))) (`self.IsAttacking`)) (`self.IsHitting`)) (`NavMovementComponent.IsSwimming` (`self.CharacterMovement`))) (`NavMovementComponent.IsFalling` (`self.CharacterMovement`)))) (`self.DeltaSeconds`) 5.0))
  ;[1 1 1] Calculate Foot and Pelvis transform.
  (set `self.PelvisDistance` (`KismetMathLibrary.FClamp` (* (+ (* (`self.ForwardSpeed`) -22.5) 97.5) _scale) 0.0 (* _scale 75.0)))
  (`self.CalculatePelvisTransform`)
  ;[1 1 1] Judge in which direction the bear is lie down.
  (set `self.DownRight` (>= (`KismetMathLibrary.Dot_VectorVector` (`KismetMathLibrary.GetForwardVector` (`SceneComponent.GetSocketRotation` (`self.Mesh`) "Pelvis")) (0.0 0.0 1.0)) 0.0))
  ;[1 1 1] IsNotRagdoll?
  (if (`self.IsNotRagdoll`)
    (if (not (`self.StandingUp`))
      ;[1 1 1] Calculate the HeadHeight from the average value of the heights of the HorizontalDivisionNumber × VerticalDivisionNumber points.
      ;;[1 1 1] Trace for lattice points.
      (for _index (range (+ (`self.MaxTraceNumber`) 1))
        (set `self.CurrentTraceNumber` _index)
        (bind _outhit (`KismetSystemLibrary.LineTraceSingle` :`Start` (- _returnvalue_3 _returnvalue) :`End` (+ _returnvalue_3 _returnvalue) :`TraceChannel` "TraceTypeQuery1" :`bTraceComplex` true :`TraceColor` (struct :`R` 1.0 :`G` 0.724743 :`A` 1.0) :`TraceHitColor` (struct :`G` 0.08531 :`B` 1.0 :`A` 1.0)))
        (bind (_bblockinghit _binitialoverlap _time _distance _location _impactpoint) (`GameplayStatics.BreakHitResult` _outhit))
        (if _bblockinghit
          (set `self.HeadHeightSum` (+ (`self.HeadHeightSum`) (`KismetMathLibrary.VSize` (- _returnvalue_3 _impactpoint))))
          (`/Engine/EditorBlueprintResources/StandardMacros.IncrementInt` (`self.HeadHeightColisionNum`))))
      ;;[1 1 1] Set the HeadHeight.
      (if (!= (`self.HeadHeightColisionNum`) 0)
        (set `self.HeadHeight` (+ (`KismetMathLibrary.FInterpTo` (`self.HeadHeight`) (/ (`self.HeadHeightSum`) (`KismetMathLibrary.Conv_IntToDouble` (`self.HeadHeightColisionNum`))) (`self.DeltaSeconds`) 1.0) (`self.HeadHeightOffset`))))
      (set `self.HeadHeightSum` 0.0)
      (set `self.HeadHeightColisionNum` 0)
      ;[1 1 1] IsSwimming?
      (if (`NavMovementComponent.IsSwimming` (`self.CharacterMovement`))
        ;[1 1 1] Swimming
        (`SceneComponent.K2_AddLocalOffset` (`self.CapsuleComponent`) (`KismetMathLibrary.MakeVector` (* (* (`self.ForwardSpeed`) (`self.DeltaSeconds`)) (`self.SwimSpeedMultiplier`))) false false)
        (`SceneComponent.K2_AddLocalRotation` (`self.CapsuleComponent`) (`KismetMathLibrary.MakeRotator` 0.0 0.0 (* (* (`self.TurnSpeed`) (`self.DeltaSeconds`)) 45.0)) false false))
      ;[1 1 1] Attack by right arm.
      (bind _output_get (set `self.ArmROldLocation` (`self.ArmRLocation`)))
      (bind _output_get_2 (set `self.ArmRLocation` (`SceneComponent.GetSocketLocation` (`self.Mesh`) (`self.R_Hand`))))
      (if (`self.IsAttacking`)
        (bind _outhit_2 (`KismetSystemLibrary.LineTraceSingle` :`Start` _output_get_2 :`End` (+ _output_get_2 (`KismetMathLibrary.Normal` (- _output_get_2 _output_get))) :`TraceChannel` "TraceTypeQuery1" :`DrawDebugType` "ForOneFrame"))
        (`GameplayStatics.ApplyPointDamage` (`.HitActor` (`GameplayStatics.BreakHitResult` _outhit_2)) 1.0 _output_get_2 _outhit_2 (`self.GetController`) self "/Script/Engine.DamageType"))
      ;[1 1 1] Attack by Left arm.
      (bind _output_get_3 (set `self.ArmLOldLocation` (`self.ArmLLocation`)))
      (bind _output_get_4 (set `self.ArmLLocation` (`SceneComponent.GetSocketLocation` (`self.Mesh`) (`self.L_Hand`))))
      (if (`self.IsAttackingLeft`)
        (bind _outhit_3 (`KismetSystemLibrary.LineTraceSingle` :`Start` _output_get_4 :`End` (+ _output_get_4 (`KismetMathLibrary.Normal` (- _output_get_4 _output_get_3))) :`TraceChannel` "TraceTypeQuery1" :`DrawDebugType` "ForOneFrame"))
        (`GameplayStatics.ApplyPointDamage` (`.HitActor` (`GameplayStatics.BreakHitResult` _outhit_3)) 1.0 _output_get_4 _outhit_3 (`self.GetController`) self "/Script/Engine.DamageType"))
      ;[1 1 1] Set the AttackedPhysicsAlpha.
      (if (`self.IsHitting`)
        (bind _output_get_5 (set `self.AttackedTime` (+ (`self.AttackedTime`) (`self.DeltaSeconds`))))
        (if (> _output_get_5 2.0)
          (`SkeletalMeshComponent.SetAllBodiesBelowSimulatePhysics` (`self.Mesh`) (`self.Pelvis`) false true)
          (set `self.IsHitting` false)
          (else
            (bind _output_get_6 (set `self.AttackedPhysicsAlpha` (`KismetMathLibrary.FInterpTo` (`self.AttackedPhysicsAlpha`) 0.0 (`self.DeltaSeconds`) 0.5)))
            (`SkeletalMeshComponent.SetAllBodiesBelowPhysicsBlendWeight` (`self.Mesh`) (`self.Pelvis`) _output_get_6 false true)
            (`self.CalculateCapsuleLocation`)))))
    (else
      ;[1 1 1] Set the RagdollTime.
      (set `self.RagDollTime` (+ (`self.RagDollTime`) (`self.DeltaSeconds`)))
      ;[1 1 1] Recovering?
      (if (`self.Recovering`)
        ;[1 1 1] Set the PhysicsAlpha.
        (set `self.PhysicsAlpha` (`KismetMathLibrary.FInterpTo` (`self.PhysicsAlpha`) 0.0 (`self.DeltaSeconds`) 3.0))
        (`SkeletalMeshComponent.SetAllBodiesBelowPhysicsBlendWeight` (`self.Mesh`) (`self.Pelvis`) (`self.PhysicsAlpha`) false true)
        ;[1 1 1] RecoveringTime less than 1?
        (set `self.RecoveringTIme` (+ (`self.RecoveringTIme`) (`self.DeltaSeconds`)))
        (if (not (< (`self.RecoveringTIme`) 2.0))
          ;[1 1 1] Playing Rebirth animation by turning off physical simulation. The length of the reverse animation is 2 seconds.
          (`SkeletalMeshComponent.SetAllBodiesBelowSimulatePhysics` (`self.Mesh`) (`self.Pelvis`) false true)
          (`SceneComponent.K2_AttachToComponent` (`self.Mesh`) (`self.CapsuleComponent`) "None" "KeepRelative" "KeepRelative" "KeepRelative" true)
          (`SceneComponent.K2_SetRelativeLocationAndRotation` (`self.Mesh`) (0.0 0.0 -46.0) (struct :`Yaw` -90.0) false false)
          (set `self.Recovering` false)
          (set `self.IsNotRagdoll` true)
          (`CharacterMovementComponent.SetMovementMode` (`self.CharacterMovement`) "MOVE_Walking" 0)
          (set `self.StandingUp` true)
          (`KismetSystemLibrary.Delay` 2.0)
          (set `self.StandingUp` false))
        (else
          (`self.CalculateCapsuleLocation`))))))

(event `self.ReceivePointDamage`
  (params (Damage :type "Float (single-precision)") (DamageType :type "DamageType Object Reference") (HitLocation :type "Vector Structure") (HitNormal :type "Vector Structure") (HitComponent :type "PrimitiveComponent Object Reference") (BoneName :type Name) (ShotFromDirection :type "Vector Structure") (InstigatedBy :type "Controller Object Reference") (DamageCauser :type "Actor Object Reference") (HitInfo :type "HitResult Structure (by ref)"))
  ;[1 1 1] Damage using physics simulation.
  (set `self.AttackedPhysicsAlpha` 0.5)
  (`SkeletalMeshComponent.SetAllBodiesBelowSimulatePhysics` (`self.Mesh`) (`self.Pelvis`) true true)
  (`SkeletalMeshComponent.SetAllBodiesBelowPhysicsBlendWeight` (`self.Mesh`) (`self.Pelvis`) 1.0 false true)
  (`PrimitiveComponent.AddImpulseAtLocation` (`self.Mesh`) (* (`KismetMathLibrary.Normal` (- HitLocation ShotFromDirection)) Damage) HitLocation BoneName)
  (set `self.IsHitting` true)
  (set `self.AttackedTime` 0.0))

(event `Key|LeftMouseButton`
  (params (Key :type "Key Structure"))
  (bind _returnvalue (`SceneComponent.GetSocketLocation` (`self.Mesh`) "Neck_1"))
  ;[1 1 1] For damage testing.
  (:`Pressed`
    (bind _outhit (`KismetSystemLibrary.LineTraceSingle` _returnvalue (+ _returnvalue (* (`KismetMathLibrary.GetForwardVector` (`self.GetControlRotation`)) 10000.0)) "TraceTypeQuery1"))
    (`GameplayStatics.ApplyPointDamage` (`.HitActor` (`GameplayStatics.BreakHitResult` _outhit)) 1000.0 _returnvalue _outhit (`self.GetController`) self "/Script/Engine.DamageType")))

(event `ToBipedal`
  ;[1 1 1] Bipdal
  (set `self.IsStanding` true)
  (set `self.IsHandIKOn` false))

(event `ToQuadruped`
  ;[1 1 1] Quadruped
  (set `self.IsStanding` false)
  (`KismetSystemLibrary.Delay` 3.0)
  (if (not (`self.IsStanding`))
    (set `self.IsHandIKOn` true)))

(event `Attack`
  ;[1 1 1] Attack
  (set `self.IsAttacking` true)
  (`KismetSystemLibrary.Delay` 1.0)
  (set `self.IsAttacking` false))

(event `AttackLeft`
  ;[1 1 1] AttackLeft
  (set `self.IsAttackingLeft` true)
  (`KismetSystemLibrary.Delay` 1.0)
  (set `self.IsAttackingLeft` false))

(fn `CalculateCapsuleLocation`
  (bind _returnvalue (/ (+ (`SceneComponent.GetSocketLocation` (`self.Mesh`) (`self.Pelvis`)) (`SceneComponent.GetSocketLocation` (`self.Mesh`) "Head")) 2.0))
  ;[1 1 1] Calculate Capsule location.
  (bind (_outhit _returnvalue_2) (`KismetSystemLibrary.LineTraceSingle` _returnvalue (`KismetMathLibrary.MakeVector` (.x _returnvalue) (.y _returnvalue) (- (.z _returnvalue) (`self.TraceDistance`))) "TraceTypeQuery1"))
  (bind _output_get (set `self.CapsuleLocation` (`KismetMathLibrary.SelectVector` (`KismetMathLibrary.MakeVector` (.x (`.Location` (`GameplayStatics.BreakHitResult` _outhit))) (.y (`.Location` (`GameplayStatics.BreakHitResult` _outhit))) (+ (.z (`.Location` (`GameplayStatics.BreakHitResult` _outhit))) (* (`self.PelvisHeight`) 2.25))) _returnvalue _returnvalue_2)))
  (`SceneComponent.K2_SetWorldLocation` (`self.CapsuleComponent`) _output_get false false))

(fn `CalculatePelvisTransform`
  (bind _standpelvisheight (`self.StandPelvisHeight`))
  (bind _returnvalue (- 90.0 (`KismetMathLibrary.DegAcos` (`KismetMathLibrary.Dot_VectorVector` (`KismetMathLibrary.Normal` (- (+ (`SceneComponent.GetSocketLocation` (`self.Mesh`) (`self.L_Hand`)) (`SceneComponent.GetSocketLocation` (`self.Mesh`) (`self.R_Hand`))) (+ (`SceneComponent.GetSocketLocation` (`self.Mesh`) (`self.L_Foot`)) (`SceneComponent.GetSocketLocation` (`self.Mesh`) (`self.R_Foot`))))) (0.0 0.0 1.0)))))
  ;[1 1 1] Calculate Pelvis rotation.
  (set `self.PelvisRotation` (`KismetMathLibrary.SelectRotator` (struct) (`KismetMathLibrary.RInterpTo` (`self.PelvisRotation`) (`KismetMathLibrary.RotatorFromAxisAndAngle` (1.0 0.0 0.0) _returnvalue) (`self.DeltaSeconds`) 2.0) (`self.IsStanding`)))
  ;[1 1 1] Calculate Pelvis location.
  (set `self.PelvisLocation` (`KismetMathLibrary.VInterpTo` (`self.PelvisLocation`) (+ (- (- (`SceneComponent.K2_GetComponentLocation` (`self.CapsuleComponent`)) (* (* (`SceneComponent.GetForwardVector` (`self.CapsuleComponent`)) (`self.PelvisDistance`)) (`KismetMathLibrary.DegCos` _returnvalue))) (* (`KismetMathLibrary.MakeVector` 0.0 0.0 (`KismetMathLibrary.DegSin` _returnvalue)) (`self.PelvisDistance`))) (`KismetMathLibrary.MakeVector` 0.0 0.0 (`KismetMathLibrary.SelectFloat` (`KismetMathLibrary.SelectFloat` (`KismetMathLibrary.SelectFloat` (* _standpelvisheight 0.5) _standpelvisheight (`self.StandingUp`)) (`self.PelvisHeight`) (`self.IsStanding`)) 0.0 (`self.IsNotRagdoll`)))) (`self.DeltaSeconds`) 10.0)))

(fn `CanJumpInternal`
  (returns (ReturnValue :type Boolean))
  (return (and (and (and (and (`CharacterMovementComponent.IsWalking` (`self.CharacterMovement`)) (`self.IsNotRagdoll`)) (not (`self.IsAttacking`))) (not (`self.IsHitting`))) (not (`self.IsEating`)))))

(fn `Death`
  (set `self.IsLived` false)
  (`self.ToRagdoll`))

(fn `Rebirth`
  (set `self.IsLived` true)
  (`self.StandUp`))

(fn `StandUp`
  ;[1 1 1] If IsNotRagdoll is false, Set Recovering, RicoveriingTime and PhysicsAlpha.
  (if (`self.IsLived`)
    (if (`self.IsNotRagdoll`)
      _
      (elif (> (`self.RagDollTime`) 2.0)
        (set `self.Recovering` true)
        (set `self.RecoveringTIme` 0.0)
        (set `self.PhysicsAlpha` 1.0)))))

(fn `ToRagdoll`
  ;[1 1 1] Set the physics simulation.
  (set `self.IsNotRagdoll` false)
  (`SkeletalMeshComponent.SetAllBodiesBelowSimulatePhysics` (`self.Mesh`) (`self.Pelvis`) true true)
  (`SkeletalMeshComponent.SetAllBodiesBelowPhysicsBlendWeight` (`self.Mesh`) (`self.Pelvis`) 1.0 false true)
  (`CharacterMovementComponent.SetMovementMode` (`self.CharacterMovement`) "MOVE_None" 0)
  ;[1 1 1] Set the Cupsule location.
  (set `self.CapsuleLocation` (`SceneComponent.K2_GetComponentLocation` (`self.CapsuleComponent`)))
  ;[1 1 1] Set the RagdollTime Zero.
  (set `self.RagDollTime` 0.0))

(fn `UserConstructionScript`
  (bind _scale (`self.Scale`))
  ;[1 1 1] Set the Scale.
  (set `self.Scale` (.z (.scale (`self.GetTransform`))))
  ;[1 1 1] Set the scale dependent variables.
  (set `self.HeadHeightOffset` (* (`self.HeadHeightOffset`) _scale))
  (set `self.IKHeightOffset` (* (`self.IKHeightOffset`) _scale))
  (set `self.PelvisDistance` (* (`self.PelvisDistance`) _scale))
  (set `self.PelvisHeight` (* (`self.PelvisHeight`) _scale))
  (set `self.NeckLength` (* (`self.NeckLength`) _scale))
  (set `self.TraceDistance` (* (`self.TraceDistance`) _scale))
  (set `self.TraceHeadDistance` (* (`self.TraceHeadDistance`) _scale))
  (set `self.TraceHalfHeight` (* (`self.TraceHalfHeight`) _scale))
  (set `self.TraceHalfWidth` (* (`self.TraceHalfWidth`) _scale))
  (set `self.SwimSpeedMultiplier` (* (`self.SwimSpeedMultiplier`) _scale))
  (set `self.StandPelvisHeight` (* (`self.StandPelvisHeight`) _scale))
  ;[1 1 1] Set the MaxTraceNumber
  (set `self.MaxTraceNumber` (- (* (+ (`self.VerticalDivisionNumber`) 1) (+ (`self.HorizontalDivisionNumber`) 1)) 1))
  ;[1 1 1] Set the TraceGridHeight
  (set `self.TraceGridHeight` (/ (* (`self.TraceHalfHeight`) 2.0) (`KismetMathLibrary.Conv_IntToDouble` (`self.VerticalDivisionNumber`))))
  ;[1 1 1] Set the TraceGridWidth
  (set `self.TraceGridWidth` (/ (* (`self.TraceHalfWidth`) 2.0) (`KismetMathLibrary.Conv_IntToDouble` (`self.HorizontalDivisionNumber`)))))
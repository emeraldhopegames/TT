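; Player character Blueprint for a third-person goat that adds keyboard gait selection for gallop, canter and trot.
; Holding G, C or T sets IsRunning and a matching MaxRunForwardSpeed, from fastest to slowest, and releasing any of them clears IsRunning.
; The construction script runs the parent's logic, then defaults the maximum speed to the gallop value.
; Movement itself is not handled in these graphs.
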(event `Key|G`
  (params (Key :type "Key Structure"))
  ;[1 1 1] G, C, T:Gallop, Canter, Trot
  (:`Pressed`
    (set `self.IsRunning` true)
    (set `self.MaxRunForwardSpeed` 4.0))
  (:`Released`
    (set `self.IsRunning` false :!label _label)))

(event `Key|C`
  (params (Key :type "Key Structure"))
  ;[1 1 1] G, C, T:Gallop, Canter, Trot
  (:`Pressed`
    (set `self.IsRunning` true)
    (set `self.MaxRunForwardSpeed` 3.0))
  (:`Released`
    (goto _label)))

(event `Key|T`
  (params (Key :type "Key Structure"))
  ;[1 1 1] G, C, T:Gallop, Canter, Trot
  (:`Pressed`
    (set `self.IsRunning` true)
    (set `self.MaxRunForwardSpeed` 2.0))
  (:`Released`
    (goto _label)))

(fn `UserConstructionScript`
  (`parent.UserConstructionScript`)
  (set `self.MaxRunForwardSpeed` 4.0))
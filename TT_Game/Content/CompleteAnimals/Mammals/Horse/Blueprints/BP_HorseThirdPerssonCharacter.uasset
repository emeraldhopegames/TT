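; Third-person horse character Blueprint that maps held keys to trot, canter and gallop gaits.
; Pressing T, C or G sets AimForward to a progressively higher value, and releasing any of them resets it to zero.
; The graph only writes this variable and contains no movement logic; BeginPlay, overlap and Tick are disabled stubs, and the construction script just calls its parent.
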(event `Key|T`
  (params (Key :type "Key Structure"))
  ;[1 1 1] T:Trot
  (:`Pressed`
    (set `self.AimForward` 2.0))
  (:`Released`
    (set `self.AimForward` 0.0)))

(event `Key|C`
  (params (Key :type "Key Structure"))
  ;[1 1 1] C:Canter
  (:`Pressed`
    (set `self.AimForward` 3.0))
  (:`Released`
    (set `self.AimForward` 0.0)))

(event `Key|G`
  (params (Key :type "Key Structure"))
  ;[1 1 1] G:Gallop
  (:`Pressed`
    (set `self.AimForward` 4.0))
  (:`Released`
    (set `self.AimForward` 0.0)))

(fn `UserConstructionScript`
  (`parent.UserConstructionScript`))
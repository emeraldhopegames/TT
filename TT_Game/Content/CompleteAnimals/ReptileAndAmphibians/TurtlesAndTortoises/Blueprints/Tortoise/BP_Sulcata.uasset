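; BP_Sulcata is the Sulcata tortoise animal Blueprint, providing a random behavior picker for the creature.
; RandomBihavior clears the attacking, eating and defensing flags, then a random integer switch sets one of them or leaves all off.
; It returns true only for eating or defensing; attacking and idle rolls return false.
; The event graph is unused and the construction script only calls its parent.
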(fn `RandomBihavior`
  (returns (IsInitialSpeedZero :type Boolean))
  (set `self.IsAttacking` false)
  (set `self.IsEating` false)
  (set `self.IsDefensing` false)
  (switch `int` (`KismetMathLibrary.RandomIntegerInRange` 0 5)
    (:`Default`
      _)
    (:`0`
      (set `self.IsAttacking` true))
    (:`1`
      (set `self.IsEating` true)
      (return true))
    (:`2`
      (set `self.IsDefensing` true)
      (return true)))
  (return false))

(fn `UserConstructionScript`
  (`parent.UserConstructionScript`))
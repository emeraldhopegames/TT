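; Giant tortoise animal Blueprint that supplies a swimming movement event and a random behavior picker.
; Swimming yaws the capsule by TurnSpeed and frame time and feeds forward movement input, unless the tortoise is defending or drinking.
; RandomBihavior clears the state flags, then randomly sets attack, eat, defend, drink or none, returning true only for eat, defend and drink.
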(event `self.Swimming`
  ;[1 1 1] Swimming behavior
  (if (not (or (`self.IsDefensing`) (`self.IsDrinking`)))
    (`SceneComponent.K2_AddLocalRotation` (`self.CapsuleComponent`) (`KismetMathLibrary.MakeRotator` 0.0 0.0 (* (* (`GameplayStatics.GetWorldDeltaSeconds`) (`self.TurnSpeed`)) 45.0)) false false)
    (`PawnMovementComponent.AddInputVector` (`self.CharacterMovement`) (* (* (`SceneComponent.GetForwardVector` (`self.CapsuleComponent`)) (`self.ForwardSpeed`)) 0.3) false)))

(fn `RandomBihavior`
  (returns (IsInitialSpeedZero :type Boolean))
  ;[1 1 1] Initialize behavior
  (set `self.IsAttacking` false)
  (set `self.IsEating` false)
  (set `self.IsDefensing` false)
  (set `self.IsDrinking` false)
  (switch `int` (`KismetMathLibrary.RandomIntegerInRange` 0 10)
    (:`Default`
      _)
    (:`0`
      ;[1 1 1] Set new behavior
      (set `self.IsAttacking` true))
    (:`1`
      (set `self.IsEating` true)
      (return true))
    (:`2`
      (set `self.IsDefensing` true)
      (return true))
    (:`3`
      (set `self.IsDrinking` true)
      (return true)))
  (return false))

(fn `UserConstructionScript`
  (`parent.UserConstructionScript`))
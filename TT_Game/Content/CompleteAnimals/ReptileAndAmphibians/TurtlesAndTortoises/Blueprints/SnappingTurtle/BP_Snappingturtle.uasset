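; Snapping turtle animal Blueprint that swims and picks random eating, biting or ambushing behaviors.
; The Swimming event, skipped while ambushing, yaws the capsule by TurnSpeed and delta time and adds forward movement input scaled by ForwardSpeed.
; RandomBihavior clears action flags, rolls a random state and returns true only for eating or ambushing.
; Biting and default rolls end ambushing, while eating leaves that flag unchanged.
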(event `self.Swimming`
  (if (not (`self.IsAmbushing`))
    ;[1 1 1] Swimming behavior
    (`SceneComponent.K2_AddLocalRotation` (`self.CapsuleComponent`) (`KismetMathLibrary.MakeRotator` 0.0 0.0 (* (* (`GameplayStatics.GetWorldDeltaSeconds`) (`self.TurnSpeed`)) 45.0)) false false)
    (`PawnMovementComponent.AddInputVector` (`self.CharacterMovement`) (* (* (`SceneComponent.GetForwardVector` (`self.CapsuleComponent`)) (`self.ForwardSpeed`)) 0.5) false)))

(fn `RandomBihavior`
  (returns (IsInitialSpeedZero :type Boolean))
  ;[1 1 1] Initialize behavior
  (set `self.IsAttacking` false)
  (set `self.IsEating` false)
  (set `self.IsBiting` false)
  (switch `int` (`KismetMathLibrary.RandomIntegerInRange` 0 6)
    (:`Default`
      ;[1 1 1] Set new behavior
      (set `self.IsAmbushing` false :!label _label))
    (:`0`
      (set `self.IsEating` true)
      (return true))
    (:`1`
      (set `self.IsBiting` true))
    (:`2`
      (set `self.IsAmbushing` true)
      (return true))
    (:`3`
      (goto _label)))
  (return false))

(fn `UserConstructionScript`
  (`parent.UserConstructionScript`))
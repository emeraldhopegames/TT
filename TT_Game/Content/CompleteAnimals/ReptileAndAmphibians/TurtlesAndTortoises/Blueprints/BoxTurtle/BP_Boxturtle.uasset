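; Box turtle character Blueprint that defines the animal's swimming movement and random behavior selection.
; The Swimming event yaws the capsule by TurnSpeed and adds forward movement input, unless the turtle is boxed or defending.
; RandomBihavior clears the action flags, then randomly picks attack, eat, box, crouch, uncrouch or nothing, returning true only for the first three.
; BeginPlay, overlap and Tick hold no active logic, and construction only calls the parent.
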(event `self.Swimming`
  (if (not (or (`self.IsBox`) (`self.IsDefense`)))
    ;[1 1 1] コメント
    (`SceneComponent.K2_AddLocalRotation` (`self.CapsuleComponent`) (`KismetMathLibrary.MakeRotator` 0.0 0.0 (* (* (`GameplayStatics.GetWorldDeltaSeconds`) (`self.TurnSpeed`)) 45.0)) false false)
    (`PawnMovementComponent.AddInputVector` (`self.CharacterMovement`) (* (* (`SceneComponent.GetForwardVector` (`self.CapsuleComponent`)) (`self.ForwardSpeed`)) 0.1) false)))

(fn `RandomBihavior`
  (returns (IsInitialSpeedZero :type Boolean))
  ;[1 1 1] Initialize behavior
  (set `self.IsAttacking` false)
  (set `self.IsEating` false)
  (set `self.IsBox` false)
  (switch `int` (`KismetMathLibrary.RandomIntegerInRange` 0 5)
    (:`Default`
      _)
    (:`0`
      ;[1 1 1] Set new behavior
      (set `self.IsAttacking` true)
      (return true))
    (:`1`
      (set `self.IsEating` true)
      (return true))
    (:`2`
      (set `self.IsBox` true)
      (return true))
    (:`3`
      (`self.Crouch`))
    (:`4`
      (`self.UnCrouch`)))
  (return false))

(fn `UserConstructionScript`
  (`parent.UserConstructionScript`))
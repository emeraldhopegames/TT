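; Pond turtle animal Blueprint that supplies a random behavior picker, with its event graph left as disabled stubs.
; RandomBihavior clears the attack, eat and defense flags, then rolls an integer to set one flag, crouch, uncrouch or do nothing.
; It returns true only for eating and defense; attacking and all other outcomes return false.
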(fn `RandomBihavior`
  (returns (IsInitialSpeedZero :type Boolean))
  ;[1 1 1] Initialize behavior
  (set `self.IsAttacking` false)
  (set `self.IsEating` false)
  (set `self.IsDefense` false)
  (switch `int` (`KismetMathLibrary.RandomIntegerInRange` 0 5)
    (:`Default`
      _)
    (:`0`
      ;[1 1 1] Set new behavior
      (set `self.IsAttacking` true))
    (:`1`
      (set `self.IsEating` true)
      (return true))
    (:`2`
      (set `self.IsDefense` true)
      (return true))
    (:`3`
      (`self.Crouch`))
    (:`4`
      (`self.UnCrouch`)))
  (return false))

(fn `UserConstructionScript`
  (`parent.UserConstructionScript`))
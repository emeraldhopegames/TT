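; Tarantula character that crawls over uneven surfaces with custom capsule movement and applies one of five species material sets.
; Each tick it eases speed and body offsets, then averages a head trace grid to adjust capsule height and blends that normal with a foot-derived plane for orientation.
; Per-leg traces set IK offsets; lost ground contact or death switches to gravity-driven Falling, and landing restores crawling if alive.
; Construction scales trace and movement values by actor scale.
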(event `self.ReceiveBeginPlay`
  ;[1 1 1] Set dynamic material instance.
  (switch `/Game/CompleteAnimals/Invertebrates/Tarantula/Blueprints/Enum_Tarantula` (`self.TarantulaEnum`)
    (:`NewEnumerator0`
      (`PrimitiveComponent.CreateDynamicMaterialInstance` (`self.Mesh`) 0 "/Game/CompleteAnimals/Invertebrates/Tarantula/Materials/Mat_TarantulaBlueFang.Mat_TarantulaBlueFang")
      (`PrimitiveComponent.CreateDynamicMaterialInstance` (`self.Mesh`) 1 "/Game/CompleteAnimals/Invertebrates/Tarantula/Materials/Mat_TarantulaBlueFangLegFur.Mat_TarantulaBlueFangLegFur")
      (`PrimitiveComponent.CreateDynamicMaterialInstance` (`self.Mesh`) 2 "/Game/CompleteAnimals/Invertebrates/Tarantula/Materials/Mat_TarantulaBlueFangBodyFur.Mat_TarantulaBlueFangBodyFur"))
    (:`NewEnumerator1`
      (`PrimitiveComponent.CreateDynamicMaterialInstance` (`self.Mesh`) 0 "/Game/CompleteAnimals/Invertebrates/Tarantula/Materials/Mat_TarantulaKingBaboon.Mat_TarantulaKingBaboon")
      (`PrimitiveComponent.CreateDynamicMaterialInstance` (`self.Mesh`) 1 "/Game/CompleteAnimals/Invertebrates/Tarantula/Materials/Mat_TarantulaKingBaboonLegFur.Mat_TarantulaKingBaboonLegFur")
      (`PrimitiveComponent.CreateDynamicMaterialInstance` (`self.Mesh`) 2 "/Game/CompleteAnimals/Invertebrates/Tarantula/Materials/Mat_TarantulaKingBaboonBodyFur.Mat_TarantulaKingBaboonBodyFur"))
    (:`NewEnumerator2`
      (`PrimitiveComponent.CreateDynamicMaterialInstance` (`self.Mesh`) 0 "/Game/CompleteAnimals/Invertebrates/Tarantula/Materials/Mat_TarantulaOrangeBaboon.Mat_TarantulaOrangeBaboon")
      (`PrimitiveComponent.CreateDynamicMaterialInstance` (`self.Mesh`) 1 "/Game/CompleteAnimals/Invertebrates/Tarantula/Materials/Mat_TarantulaKingBaboonLegFur.Mat_TarantulaKingBaboonLegFur")
      (`PrimitiveComponent.CreateDynamicMaterialInstance` (`self.Mesh`) 2 "/Game/CompleteAnimals/Invertebrates/Tarantula/Materials/Mat_TarantulaOrangeBaboonBodyFur.Mat_TarantulaOrangeBaboonBodyFur"))
    (:`NewEnumerator3`
      (`PrimitiveComponent.CreateDynamicMaterialInstance` (`self.Mesh`) 0 "/Game/CompleteAnimals/Invertebrates/Tarantula/Materials/Mat_TarantulaRedKnee.Mat_TarantulaRedKnee")
      (`PrimitiveComponent.CreateDynamicMaterialInstance` (`self.Mesh`) 1 "/Game/CompleteAnimals/Invertebrates/Tarantula/Materials/Mat_TarantulaRedKneeLegFur.Mat_TarantulaRedKneeLegFur")
      (`PrimitiveComponent.CreateDynamicMaterialInstance` (`self.Mesh`) 2 "/Game/CompleteAnimals/Invertebrates/Tarantula/Materials/Mat_TarantulaRedKneeBodyFur.Mat_TarantulaRedKneeBodyFur"))
    (:`NewEnumerator4`
      (`PrimitiveComponent.CreateDynamicMaterialInstance` (`self.Mesh`) 0 "/Game/CompleteAnimals/Invertebrates/Tarantula/Materials/Mat_TarantulaRose.Mat_TarantulaRose")
      (`PrimitiveComponent.CreateDynamicMaterialInstance` (`self.Mesh`) 1 "/Game/CompleteAnimals/Invertebrates/Tarantula/Materials/Mat_TarantulaRoseLegFur.Mat_TarantulaRoseLegFur")
      (`PrimitiveComponent.CreateDynamicMaterialInstance` (`self.Mesh`) 2 "/Game/CompleteAnimals/Invertebrates/Tarantula/Materials/Mat_TarantulaRoseBodyFur.Mat_TarantulaRoseBodyFur"))))

(event `self.ReceiveTick`
  (params (DeltaSeconds :type "Float (single-precision)"))
  (bind _returnvalue (`KismetMathLibrary.GetUpVector` (struct)))
  (bind _meanheadheight (`self.MeanHeadHeight`))
  (bind _returnvalue_2 (`SceneComponent.K2_GetComponentLocation` (`self.CapsuleComponent`)))
  (bind _returnvalue_3 (`SceneComponent.K2_GetComponentRotation` (`self.CapsuleComponent`)))
  (bind _returnvalue_4 (`SceneComponent.GetUpVector` (`self.CapsuleComponent`)))
  (bind _returnvalue_5 (`SceneComponent.GetSocketLocation` (`self.Mesh`) (`self.Leg45_R`)))
  (bind _returnvalue_6 (`SceneComponent.K2_GetComponentRotation` (`self.CapsuleComponent`)))
  (bind _returnvalue_7 (`SceneComponent.GetSocketLocation` (`self.Mesh`) "Belly2_L"))
  (bind _returnvalue_8 (`SceneComponent.GetSocketLocation` (`self.Mesh`) (`self.Leg15_L`)))
  (bind _returnvalue_9 (`SceneComponent.GetSocketLocation` (`self.Mesh`) (`self.Leg45_L`)))
  (bind _returnvalue_10 (`SceneComponent.GetSocketLocation` (`self.Mesh`) (`self.Leg15_R`)))
  (bind _returnvalue_11 (* _returnvalue_4 (`self.TraceHeadDistance`)))
  (bind (_x _y _z) (`KismetMathLibrary.BreakRotIntoAxes` _returnvalue_3))
  (bind (_x_2 _y_2 _z_2) (`KismetMathLibrary.BreakRotIntoAxes` _returnvalue_6))
  (bind _returnvalue_12 (`KismetMathLibrary.Cross_VectorVector` _z_2 _returnvalue))
  (bind (_remainder _returnvalue_13) (`KismetMathLibrary.FMod` (`KismetMathLibrary.Conv_IntToDouble` (`self.CurrentTraceNumber`)) (`KismetMathLibrary.Conv_IntToDouble` (+ (`self.HorizontalDivisionNumber`) 1))))
  (bind _returnvalue_14 (* (/ (`KismetMathLibrary.Conv_IntToDouble` (`self.GroundHitNum`)) (`KismetMathLibrary.Conv_IntToDouble` (`self.MaxTraceNumber`))) 0.3))
  (bind _returnvalue_15 (`KismetMathLibrary.DegAsin` (`KismetMathLibrary.VSize` _returnvalue_12)))
  (bind _returnvalue_16 (+ (* (`KismetMathLibrary.Normal` (`KismetMathLibrary.Cross_VectorVector` (- (+ _returnvalue_8 _returnvalue_9) (+ _returnvalue_10 _returnvalue_5)) (- (+ _returnvalue_8 _returnvalue_10) (+ _returnvalue_9 _returnvalue_5)))) (- 1.0 _returnvalue_14)) (* (`self.MeanGroundNormal`) _returnvalue_14)))
  (bind _returnvalue_17 (+ (+ (* (`SceneComponent.GetRightVector` (`self.CapsuleComponent`)) (* _remainder (`self.TraceGridWidth`))) (* (`SceneComponent.GetForwardVector` (`self.CapsuleComponent`)) (* _returnvalue_13 (`self.TraceGridHeight`)))) (+ (+ (`SceneComponent.GetSocketLocation` (`self.Mesh`) (`self.Head`)) (* (* (`SceneComponent.GetForwardVector` (`self.CapsuleComponent`)) (`self.TraceHalfHeight`)) -1.0)) (* (* (`SceneComponent.GetRightVector` (`self.CapsuleComponent`)) (`self.TraceHalfWidth`)) -1.0))))
  (bind _returnvalue_18 (`KismetMathLibrary.Cross_VectorVector` _z _returnvalue_16))
  (bind _returnvalue_19 (`KismetMathLibrary.DegAsin` (`KismetMathLibrary.VSize` _returnvalue_18)))
  (set `self.DeltaSeconds` DeltaSeconds)
  (if (`self.IsLived`)
    ;[1 1 1] Set the Forward Speed.
    (set `self.ForwardSpeed` (`KismetMathLibrary.FInterpTo` (`self.ForwardSpeed`) (`self.AimForwardSpeed`) (`self.DeltaSeconds`) 5.0))
    ;[1 1 1] Set the TurnSpeed.
    (set `self.TurnSpeed` (`KismetMathLibrary.FInterpTo` (`self.TurnSpeed`) (`self.AimTurnSpeed`) (`self.DeltaSeconds`) 5.0))
    ;[1 1 1] Set the SideStepSpeed.
    (set `self.SideStepSpeed` (`KismetMathLibrary.FInterpTo` (`self.SideStepSpeed`) (`self.AimSideStepSpeed`) (`self.DeltaSeconds`) 5.0))
    ;[1 1 1] Set th BodyTransform.
    (set `self.BodyTransformOffset` (`KismetMathLibrary.TInterpTo` (`self.BodyTransformOffset`) (`KismetMathLibrary.MakeTransform` (`KismetMathLibrary.MakeVector` (`self.AimBodyLocX`) (`self.AimBodyLocY`) (`self.AimBodyLocZ`)) (`KismetMathLibrary.MakeRotator` (`self.AimBodyRotX`) (`self.AimBodyRotY`) (`self.AimBodyRotZ`))) (`self.DeltaSeconds`) (`self.BodyTransInterpSpeed`)))
    ;[1 1 1] Is MovementMode Castom?
    (if (`|EnumEquality` (`CharacterMovementComponent.MovementMode` (`self.CharacterMovement`)) "MOVE_Custom")
      ;[1 1 1] IsThreating or IsEating?
      (if (not (or (`self.IsEating`) (`self.IsThreating`)))
        ;[1 1 1] Move Forward.
        (`SceneComponent.K2_AddLocalOffset` (`self.CapsuleComponent`) (`KismetMathLibrary.MakeVector` (* (* (`self.ForwardSpeed`) (`self.ForwardSpeedMultiplier`)) (`self.DeltaSeconds`))) false false)
        ;[1 1 1] IsAttacking or IsHitting?
        (if (not (or (`self.IsAttacking`) (`self.IsHitting`)))
          ;[1 1 1] IsSIdeStepping?
          (if (`self.IsSideStepping`)
            ;[1 1 1] Move Horizontally.
            (`SceneComponent.K2_AddLocalOffset` (`self.CapsuleComponent`) (`KismetMathLibrary.MakeVector` 0.0 (* (* (`self.SideStepSpeed`) (`self.SideStepSpeedMultiplier`)) (`self.DeltaSeconds`))) false false)
            (else
              ;[1 1 1] Turn.
              (`SceneComponent.K2_AddLocalRotation` (`self.CapsuleComponent`) (`KismetMathLibrary.MakeRotator` 0.0 0.0 (* (* (`self.TurnSpeed`) (`self.TurnSpeedMultiplier`)) (`self.DeltaSeconds`))) false false)))))
      ;[1 1 1] Calculate the HeadHeight from the average value of the heights of the HorizontalDivisionNumber × VerticalDivisionNumber points.
      (set `self.HeadHeightSum` 0.0)
      (set `self.NormalSum` (0.0 0.0 0.0))
      (set `self.GroundHitNum` 0)
      ;;[1 1 1] Trace for lattice points.
      (for _index (range (+ (`self.MaxTraceNumber`) 1))
        (set `self.CurrentTraceNumber` _index)
        (bind _outhit (`KismetSystemLibrary.LineTraceSingle` :`Start` _returnvalue_17 :`End` (+ (+ _returnvalue_17 (* (`SceneComponent.GetUpVector` (`self.CapsuleComponent`)) (`self.TraceHeadDistance`))) (* (`SceneComponent.GetForwardVector` (`self.CapsuleComponent`)) (`self.ForwardSpeed`))) :`TraceChannel` "TraceTypeQuery1" :`bTraceComplex` true :`TraceColor` (struct :`R` 1.0 :`G` 0.724743 :`A` 1.0) :`TraceHitColor` (struct :`G` 0.08531 :`B` 1.0 :`A` 1.0) :`DrawTime` 0.2))
        (bind (_bblockinghit _binitialoverlap _time _distance _location _impactpoint _normal) (`GameplayStatics.BreakHitResult` _outhit))
        (if _bblockinghit
          (set `self.HeadHeightSum` (+ (`self.HeadHeightSum`) (`KismetMathLibrary.Dot_VectorVector` (`SceneComponent.GetUpVector` (`self.CapsuleComponent`)) (- _returnvalue_17 _impactpoint))))
          (`/Engine/EditorBlueprintResources/StandardMacros.IncrementInt` (`self.GroundHitNum`)
            (:`  `
              (set `self.NormalSum` (+ (`self.NormalSum`) _normal))))))
      ;;[1 1 1] Set the MeanHeadHeight and MeanGroundNormal
      (if (!= (`self.GroundHitNum`) 0)
        (set `self.MeanHeadHeight` (`KismetMathLibrary.FInterpTo` (`self.MeanHeadHeight`) (/ (`self.HeadHeightSum`) (`KismetMathLibrary.Conv_IntToDouble` (`self.GroundHitNum`))) (`self.DeltaSeconds`) 10.0))
        (set `self.MeanGroundNormal` (`KismetMathLibrary.VInterpTo` (`self.MeanGroundNormal`) (/ (`self.NormalSum`) (`self.GroundHitNum`)) (`self.DeltaSeconds`) 10.0))
        (else
          (set `self.MeanHeadHeight` (`self.MaxHeadHeight`))
          (set `self.MeanGroundNormal` (* (`SceneComponent.GetUpVector` (`self.CapsuleComponent`)) -1.0))))
      ;[1 1 1] When the number of traces hit from the head and the number of hits from the leg are 0, change the Movement Mode to Falling.
      (if (not (or (>= (`self.GroundedFootNum`) 2) (>= (`self.GroundHitNum`) 1)))
        (`CharacterMovementComponent.SetMovementMode` (`self.CharacterMovement`) "MOVE_Falling" 0)
        (`PrimitiveComponent.SetEnableGravity` (`self.CapsuleComponent`) true))
      ;[1 1 1] Change the height of the capsule according to the mean head height.
      (if (>= _meanheadheight (`self.MaxHeadHeight`))
        (set `self.ChangingHeadDistance` true)
        (elif (< _meanheadheight (`self.StandardHeadHeight`))
          (set `self.ChangingHeadDistance` false)))
      (if (`self.ChangingHeadDistance`)
        (`SceneComponent.K2_AddWorldOffset` (`self.CapsuleComponent`) (* (`SceneComponent.GetUpVector` (`self.CapsuleComponent`)) (* (- (`self.CapsuleHeightOffset`) _meanheadheight) (* (`self.DeltaSeconds`) (`KismetMathLibrary.Abs` (`self.ForwardSpeed`))))) false false))
      ;[1 1 1] Rotate the capsule.
      (if (and (and (not (`self.IsEating`)) (not (`self.IsThreating`))) (> (`KismetMathLibrary.Abs` _returnvalue_19) 1.0))
        (`SceneComponent.K2_SetWorldRotation` (`self.CapsuleComponent`) (`KismetMathLibrary.RInterpTo` _returnvalue_3 (`KismetMathLibrary.MakeRotationFromAxes` (`KismetMathLibrary.RotateAngleAxis` _x _returnvalue_19 _returnvalue_18) (`KismetMathLibrary.RotateAngleAxis` _y _returnvalue_19 _returnvalue_18) _returnvalue_16) (`self.DeltaSeconds`) 2.0) false false))
      ;[1 1 1] Measurement of abdominal height.
      (bind (_outhit_2 _returnvalue_20) (`KismetSystemLibrary.LineTraceSingle` (- _returnvalue_7 _returnvalue_11) (+ _returnvalue_7 _returnvalue_11) "TraceTypeQuery1"))
      (if _returnvalue_20
        (set `self.InverseAbdomenHeightRatio` (`KismetMathLibrary.FClamp` (`KismetMathLibrary.FInterpTo` (`self.InverseAbdomenHeightRatio`) (+ (* (`KismetMathLibrary.Dot_VectorVector` (- (`.Location` (`GameplayStatics.BreakHitResult` _outhit_2)) _returnvalue_7) _returnvalue_4) (`self.InverseScaleFactor`)) 60.0) (`self.DeltaSeconds`) 3.0) -80.0 80.0))
        (else
          (set `self.InverseAbdomenHeightRatio` 0.0)))
      (`self.FeetPlacement`)
      (else
        ;[1 1 1] Is Movement Mode Falling?
        (if (`|EnumEquality` (`CharacterMovementComponent.MovementMode` (`self.CharacterMovement`)) "MOVE_Falling")
          ;[1 1 1] Have capsule landed?
          (bind (_outhit_3 _returnvalue_21) (`KismetSystemLibrary.LineTraceSingle` _returnvalue_2 (+ _returnvalue_2 (* (`SceneComponent.GetUpVector` (`self.CapsuleComponent`)) (`self.TraceHeadDistance`))) "TraceTypeQuery1"))
          (if (and (and (> (`KismetMathLibrary.Dot_VectorVector` (`SceneComponent.GetUpVector` (`self.CapsuleComponent`)) (`.Normal` (`GameplayStatics.BreakHitResult` _outhit_3))) 0.0) _returnvalue_21) (`self.IsLived`))
            ;[1 1 1] Change the Movement Mode.
            (`CharacterMovementComponent.SetMovementMode` (`self.CharacterMovement`) "MOVE_Custom" 0)
            (`PrimitiveComponent.SetEnableGravity` (`self.CapsuleComponent`) false)
            (else
              ;[1 1 1] While falling, rotate so that the capsule stands.
              (`SceneComponent.K2_SetWorldRotation` (`self.CapsuleComponent`) (`KismetMathLibrary.RInterpTo` _returnvalue_6 (`KismetMathLibrary.MakeRotationFromAxes` (`KismetMathLibrary.RotateAngleAxis` _x_2 _returnvalue_15 _returnvalue_12) (`KismetMathLibrary.RotateAngleAxis` _y_2 _returnvalue_15 _returnvalue_12) _returnvalue) (`self.DeltaSeconds`) 2.0) false false))))))))

(fn `Death`
  (set `self.IsLived` false)
  (`CharacterMovementComponent.SetMovementMode` (`self.CharacterMovement`) "MOVE_Falling" 0)
  (`PrimitiveComponent.SetEnableGravity` (`self.CapsuleComponent`) true))

(fn `FeetPlacement`
  (set `self.GroundedFootNum` 0)
  ;[1 1 1] Calculate the LegLIKOffset.
  (`self.FootPlacement` (`self.Leg15_L`) (`self.Leg15_LIKOffset`))
  ;[1 1 1] Calculate the LegR IKOffset.
  (`self.FootPlacement` (`self.Leg15_R`) (`self.Leg15_RIKOffset`))
  (`self.FootPlacement` (`self.Leg25_L`) (`self.Leg25_LIKOffset`))
  (`self.FootPlacement` (`self.Leg25_R`) (`self.Leg25_RIKOffset`))
  (`self.FootPlacement` (`self.Leg35_L`) (`self.Leg35_LIKOffset`))
  (`self.FootPlacement` (`self.Leg35_R`) (`self.Leg35_RIKOffset`))
  (`self.FootPlacement` (`self.Leg45_L`) (`self.Leg45_LIKOffset`))
  (`self.FootPlacement` (`self.Leg45_R`) (`self.Leg45_RIKOffset`)))

(fn `FootPlacement`
  (params (FootName :type Name) (HeightOffset :type "Float (double-precision) (by ref)"))
  ;[1 1 1] Set the IKHeightOffset and GroundedFootNum
  (bind (_ikheightoffsett _footisgrounded) (`self.TraceIKEffector` FootName (`self.IKTraceDistance`) (`self.IKHeightOffset`)))
  (set `self.GroundedFootNum` (+ (`KismetMathLibrary.SelectInt` 1 0 _footisgrounded) (`self.GroundedFootNum`)))
  (`|VariableSetRef` HeightOffset (`KismetMathLibrary.FInterpTo` HeightOffset _ikheightoffsett (`self.DeltaSeconds`) (`KismetMathLibrary.SelectFloat` (`self.IKInterpSpeedFast`) (`self.IKInterpSpeedSlow`) (> _ikheightoffsett 0.0)))))

(fn `Rebirth`
  (set `self.IsLived` true))

(fn `SetWalkingAnimRate`
  (params (AnimRate :type "Float (double-precision)"))
  (bind _output_get (set `self.WalkingAnimRate` AnimRate))
  (bind _output_get_2 (set `self.TurnSpeedMultiplier` _output_get))
  (bind _returnvalue (* (* _output_get_2 (`self.Scale`)) 6.0))
  (set `self.ForwardSpeedMultiplier` _returnvalue)
  (set `self.SideStepSpeedMultiplier` _returnvalue))

(fn `TraceIKEffector`
  (params (FootName :type Name) (TraceDistance :type "Float (double-precision)") (HeightOffset :type "Float (double-precision)"))
  (returns (IKHeightOffsett :type "Float (double-precision)") (FootIsGrounded :type Boolean) (IKPos :type "Vector Structure"))
  (bind _returnvalue (`SceneComponent.GetSocketLocation` (`self.Mesh`) FootName))
  (bind _returnvalue_2 (+ (* (`SceneComponent.GetUpVector` (`self.CapsuleComponent`)) TraceDistance) (* (`SceneComponent.GetForwardVector` (`self.CapsuleComponent`)) (* (`self.ForwardSpeed`) -1.0))))
  ;[1 1 1] Trace from foot.
  (bind (_outhit _returnvalue_3) (`KismetSystemLibrary.LineTraceSingle` (+ _returnvalue _returnvalue_2) (- _returnvalue _returnvalue_2) "TraceTypeQuery1" true))
  (if _returnvalue_3
    (bind _returnvalue_4 (`KismetMathLibrary.InverseTransformLocation` (`SceneComponent.K2_GetComponentToWorld` (`self.Mesh`)) (`.Location` (`GameplayStatics.BreakHitResult` _outhit))))
    ;[1 1 1] Calculate IKHeightOffset in Meshe's coordinate.
    (return (- (.z _returnvalue_4) HeightOffset) _returnvalue_3 _returnvalue_4)
    (else
      (return (`self.MaxLegIKOffset`) false (0.0 0.0 0.0)))))

(fn `UserConstructionScript`
  (bind _scale (`self.Scale`))
  ;[1 1 1] Set the Scale
  (set `self.Scale` (.z (.scale (`self.GetTransform`))))
  ;[1 1 1] Set the Scale dependent variables.
  (set `self.InverseScaleFactor` (/ 45.0 (`self.Scale`)))
  (set `self.TraceHeadDistance` (* (`self.TraceHeadDistance`) _scale))
  (set `self.TraceHalfHeight` (* (`self.TraceHalfHeight`) _scale))
  (set `self.TraceHalfWidth` (* (`self.TraceHalfWidth`) _scale))
  (set `self.IKTraceDistance` (* (`self.IKTraceDistance`) _scale))
  (set `self.CapsuleHeightOffset` (* (`self.CapsuleHeightOffset`) _scale))
  (set `self.MaxLegIKOffset` (* (`self.MaxLegIKOffset`) _scale))
  (set `self.ForwardSpeedMultiplier` (* (`self.ForwardSpeedMultiplier`) _scale))
  (set `self.SideStepSpeedMultiplier` (* (`self.SideStepSpeedMultiplier`) _scale))
  (set `self.StandardHeadHeight` (* (`self.StandardHeadHeight`) _scale))
  (set `self.MaxHeadHeight` (* (`self.MaxHeadHeight`) _scale))
  ;[1 1 1] Set the MaxTraceNumber
  (set `self.MaxTraceNumber` (- (* (+ (`self.VerticalDivisionNumber`) 1) (+ (`self.HorizontalDivisionNumber`) 1)) 1))
  ;[1 1 1] Set the TraceGridHeight
  (set `self.TraceGridHeight` (/ (* (`self.TraceHalfHeight`) 2.0) (`KismetMathLibrary.Conv_IntToDouble` (`self.VerticalDivisionNumber`))))
  ;[1 1 1] Set the TraceGridWidth
  (set `self.TraceGridWidth` (/ (* (`self.TraceHalfWidth`) 2.0) (`KismetMathLibrary.Conv_IntToDouble` (`self.HorizontalDivisionNumber`)))))
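; Old tarantula random-walk character that wanders and switches behaviors at random, with no player or target input in its graph.
; Tick accumulates time and, at random intervals of up to three seconds, rerolls target forward, turn and sidestep speeds plus walking animation rate.
; Each reroll clears the action flags, then raises one of attack, hit, eat, threat or sidestep, or leaves all off.
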(event `self.ReceiveTick`
  (params (DeltaSeconds :type "Float (single-precision)"))
  (`parent.ReceiveTick` DeltaSeconds)
  ;[1 1 1] Increase SpeedChangeTime.
  (set `self.SpeedChangeTime` (+ (`self.SpeedChangeTime`) (`self.DeltaSeconds`)))
  ;[1 1 1] SpeedChangeTime>=NextSpeedChangeTime?
  (if (>= (`self.SpeedChangeTime`) (`self.NextSpeedChangeTime`))
    ;[1 1 1] Set the random behavior.
    (set `self.AimForwardSpeed` (`KismetMathLibrary.RandomFloatInRange` -1.0 2.0))
    (set `self.AimTurnSpeed` (`KismetMathLibrary.RandomFloatInRange` -45.0 45.0))
    (set `self.AimSideStepSpeed` (`KismetMathLibrary.RandomFloatInRange` -1.0 1.0))
    (`self.SetWalkingAnimRate` (`KismetMathLibrary.RandomFloatInRange` 0.5 2.0))
    (set `self.NextSpeedChangeTime` (`KismetMathLibrary.RandomFloatInRange` 0.0 3.0))
    (set `self.SpeedChangeTime` 0.0)
    (set `self.IsAttacking` false)
    (set `self.IsHitting` false)
    (set `self.IsEating` false)
    (set `self.IsThreating` false)
    (set `self.IsSideStepping` false)
    (switch `int` (`KismetMathLibrary.RandomIntegerInRange` 0 5)
      (:`0`
        (set `self.IsAttacking` true))
      (:`1`
        (set `self.IsHitting` true))
      (:`2`
        (set `self.IsEating` true))
      (:`3`
        (set `self.IsThreating` true))
      (:`4`
        (set `self.IsSideStepping` true)))))

(fn `UserConstructionScript`
  (`parent.UserConstructionScript`))
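; Snow crab Character Blueprint with smoothed movement, attacks, physical hit reactions, death and rebirth.
; Tick interpolates speeds and body pose toward aim values, and traces along the right arm socket's motion to apply point damage during attacks.
; Hits briefly blend in ragdoll physics with an impulse; Death fully ragdolls with the capsule following the body, and Rebirth blends back before standing up.
; Construction scales body limits and trace distance by actor scale.
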(event `self.ReceiveTick`
  (params (DeltaSeconds :type "Float (single-precision)"))
  (bind _returnvalue (`SceneComponent.GetSocketLocation` (`self.Mesh`) (`self.body`)))
  (set `self.DeltaSeconds` DeltaSeconds)
  ;[1 1 1] IsLived?
  (if (`self.IsLived`)
    ;[1 1 1] Set the Forward Speed.
    (set `self.ForwardSpeed` (`KismetMathLibrary.FInterpTo` (`self.ForwardSpeed`) (`self.AimForwardSpeed`) (`self.DeltaSeconds`) 5.0))
    ;[1 1 1] Set the TurnSpeed.
    (set `self.TurnSpeed` (`KismetMathLibrary.FInterpTo` (`self.TurnSpeed`) (`self.AimTurnSpeed`) (`self.DeltaSeconds`) 5.0))
    ;[1 1 1] Set the SideStepSpeed.
    (set `self.SideStepSpeed` (`KismetMathLibrary.FInterpTo` (`self.SideStepSpeed`) (`self.AimSideStepSpeed`) (`self.DeltaSeconds`) 5.0))
    ;[1 1 1] Set th BodyTransform.
    (set `self.BodyTransform` (`KismetMathLibrary.TInterpTo` (`self.BodyTransform`) (`KismetMathLibrary.MakeTransform` (`KismetMathLibrary.MakeVector` (`self.AimBodyLocX`) (`self.AimBodyLocY`) (`self.AimBodyLocZ`)) (`KismetMathLibrary.MakeRotator` (`self.AimBodyRotX`) (`self.AimBodyRotY`) (`self.AimBodyRotZ`))) (`self.DeltaSeconds`) (`self.BodyTransInterpSpeed`)))
    ;[1 1 1] Attack by right arm.
    (bind _output_get (set `self.ArmROldLocation` (`self.ArmRLocation`)))
    (bind _output_get_2 (set `self.ArmRLocation` (`SceneComponent.GetSocketLocation` (`self.Mesh`) "ArmPropodus_R")))
    (if (or (or (`self.IsAttacking1`) (`self.IsAttacking2`)) (`self.IsAttacking3`))
      (bind _outhit (`KismetSystemLibrary.LineTraceSingle` :`Start` _output_get_2 :`End` (+ _output_get_2 (`KismetMathLibrary.Normal` (- _output_get_2 _output_get))) :`TraceChannel` "TraceTypeQuery1" :`DrawDebugType` "ForOneFrame"))
      (`GameplayStatics.ApplyPointDamage` (`.HitActor` (`GameplayStatics.BreakHitResult` _outhit)) 1.0 _output_get_2 _outhit (`self.GetController`) self "/Script/Engine.DamageType"))
    ;[1 1 1] Set the AttackedPhysicsAlpha.
    (if (`self.IsAttacked`)
      (bind _output_get_3 (set `self.AttackedTime` (+ (`self.AttackedTime`) (`self.DeltaSeconds`))))
      (if (> _output_get_3 2.0)
        (`SkeletalMeshComponent.SetAllBodiesBelowSimulatePhysics` (`self.Mesh`) (`self.body`) false true)
        (set `self.IsAttacked` false)
        (else
          (bind _output_get_4 (set `self.AttackedPhysicsAlpha` (`KismetMathLibrary.FInterpTo` (`self.AttackedPhysicsAlpha`) 0.0 (`self.DeltaSeconds`) 0.5)))
          (`SkeletalMeshComponent.SetAllBodiesBelowPhysicsBlendWeight` (`self.Mesh`) (`self.body`) _output_get_4 false true)
          ;[1 1 1] Calculate Capsule location.
          (bind (_outhit_2 _returnvalue_2) (`KismetSystemLibrary.LineTraceSingle` _returnvalue (`KismetMathLibrary.MakeVector` (.x _returnvalue) (.y _returnvalue) (- (.z _returnvalue) (`self.TraceDistance`))) "TraceTypeQuery1" :!label _label))
          (`SceneComponent.K2_SetWorldLocation` (`self.CapsuleComponent`) (`KismetMathLibrary.SelectVector` (`.Location` (`GameplayStatics.BreakHitResult` _outhit_2)) _returnvalue _returnvalue_2) false false))))
    (else
      ;[1 1 1] Recovering?
      (if (`self.Recovering`)
        ;[1 1 1] Set the PhysicsAlpha.
        (set `self.PhysicsAlpha` (`KismetMathLibrary.FInterpTo` (`self.PhysicsAlpha`) 0.0 (`self.DeltaSeconds`) 3.0))
        (`SkeletalMeshComponent.SetAllBodiesBelowPhysicsBlendWeight` (`self.Mesh`) (`self.body`) (`self.PhysicsAlpha`) false true)
        ;[1 1 1] RecoveringTime less than 1?
        (set `self.RecoveringTIme` (+ (`self.RecoveringTIme`) (`self.DeltaSeconds`)))
        (if (not (< (`self.RecoveringTIme`) 1.0))
          ;[1 1 1] Playing Rebirth animation by turning off physical simulation. The length of the reverse animation is 1 seconds.
          (`SkeletalMeshComponent.SetAllBodiesBelowSimulatePhysics` (`self.Mesh`) (`self.body`) false true)
          (set `self.Recovering` false)
          (set `self.IsLived` true)
          (`CharacterMovementComponent.SetMovementMode` (`self.CharacterMovement`) "MOVE_Walking" 0)
          (set `self.StandingUp` true)
          (`KismetSystemLibrary.Delay` 1.0)
          (set `self.StandingUp` false))
        (else
          (goto _label))))))

(event `self.ReceivePointDamage`
  (params (Damage :type "Float (single-precision)") (DamageType :type "DamageType Object Reference") (HitLocation :type "Vector Structure") (HitNormal :type "Vector Structure") (HitComponent :type "PrimitiveComponent Object Reference") (BoneName :type Name) (ShotFromDirection :type "Vector Structure") (InstigatedBy :type "Controller Object Reference") (DamageCauser :type "Actor Object Reference") (HitInfo :type "HitResult Structure (by ref)"))
  ;[1 1 1] Damage using physics simulation.
  (if (`self.IsAttacked`)
    _
    (elif (`KismetMathLibrary.BooleanNOR` (== BoneName "ArmPropodus_R") (== BoneName "Leg1Propodus_L"))
      (`SkeletalMeshComponent.SetAllBodiesBelowSimulatePhysics` (`self.Mesh`) (`self.body`) true true)
      (bind _output_get (set `self.AttackedPhysicsAlpha` 0.5))
      (`SkeletalMeshComponent.SetAllBodiesBelowPhysicsBlendWeight` (`self.Mesh`) (`self.body`) _output_get false true)
      (`PrimitiveComponent.AddImpulseAtLocation` (`self.Mesh`) (* (`KismetMathLibrary.Normal` (- HitLocation ShotFromDirection)) Damage) HitLocation BoneName)
      (set `self.IsAttacked` true)
      (set `self.AttackedTime` 0.0))))

(fn `CanJumpInternal`
  (returns (ReturnValue :type Boolean))
  (return false))

(fn `Death`
  (set `self.IsLived` false)
  ;[1 1 1] Set the physics simulation.
  (`SkeletalMeshComponent.SetAllBodiesBelowSimulatePhysics` (`self.Mesh`) (`self.body`) true true)
  (`SkeletalMeshComponent.SetAllBodiesBelowPhysicsBlendWeight` (`self.Mesh`) (`self.body`) 1.0 false true)
  (`CharacterMovementComponent.SetMovementMode` (`self.CharacterMovement`) "MOVE_None" 0))

(fn `Rebirth`
  ;[1 1 1] If rhinoceros is dead, Set Recovering, RicoveriingTime and PhysicsAlpha.
  (if (not (`self.IsLived`))
    (set `self.Recovering` true)
    (set `self.RecoveringTIme` 0.0)
    (set `self.PhysicsAlpha` 1.0)))

(fn `UserConstructionScript`
  ;[1 1 1] Set the scale.
  (set `self.Scale` (.z (.scale (`self.GetTransform`))))
  ;[1 1 1] Set the scale dependent variables.
  (set `self.MinBodyLocX` (* (`self.MinBodyLocX`) (`self.Scale`)))
  (set `self.MaxBodyLocX` (* (`self.MaxBodyLocX`) (`self.Scale`)))
  (set `self.MinBodyLocY` (* (`self.MinBodyLocY`) (`self.Scale`)))
  (set `self.MaxBodyLocY` (* (`self.MaxBodyLocY`) (`self.Scale`)))
  (set `self.MinBodyLocZ` (* (`self.MinBodyLocZ`) (`self.Scale`)))
  (set `self.MaxBodyLocZ` (* (`self.MaxBodyLocZ`) (`self.Scale`)))
  (set `self.MinBodyRotX` (* (`self.MinBodyRotX`) (`self.Scale`)))
  (set `self.MaxBodyRotX` (* (`self.MaxBodyRotX`) (`self.Scale`)))
  (set `self.MinBodyRotY` (* (`self.MinBodyRotY`) (`self.Scale`)))
  (set `self.MaxBodyRotY` (* (`self.MaxBodyRotY`) (`self.Scale`)))
  (set `self.MinBodyRotZ` (* (`self.MinBodyRotZ`) (`self.Scale`)))
  (set `self.MaxBodyRotZ` (* (`self.MaxBodyRotZ`) (`self.Scale`)))
  (set `self.TraceDistance` (* (`self.TraceDistance`) (`self.Scale`))))
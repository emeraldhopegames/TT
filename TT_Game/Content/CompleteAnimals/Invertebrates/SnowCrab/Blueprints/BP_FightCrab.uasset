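; AI-driven fighting snow crab that chases the player's snow crab character and attacks it at close range.
; Each tick it finds a navmesh path and uses dot products to the next point to set turn and forward speed.
; A forward trace that hits a Character overrides forward speed to full, despite a comment saying stop.
; Within range, a timer drives two-second attack bursts separated by a short cooldown.
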(event `self.ReceiveBeginPlay`
  (`parent.ReceiveBeginPlay`)
  ;[1 1 1] Set the AttackTarget.
  (bind _asbp_snow_crab_character (cast `/Game/CompleteAnimals/Invertebrates/SnowCrab/Blueprints/BP_SnowCrabCharacter` (`GameplayStatics.GetPlayerPawn` 0))
    (:`then`
      (set `self.AttackTarget` _asbp_snow_crab_character))
    (:`CastFailed`
      (set `self.CastFailed` true))))

(event `self.ReceiveTick`
  (params (DeltaSeconds :type "Float (single-precision)"))
  (bind _returnvalue (`SceneComponent.K2_GetComponentLocation` (`self.CapsuleComponent`)))
  (`parent.ReceiveTick` DeltaSeconds)
  ;[1 1 1] Set the GoalCloc.
  (if (not (`self.CastFailed`))
    (set `self.GoalLoc` (`self.K2_GetActorLocation` (`self.AttackTarget`)))
    ;[1 1 1] Is eating?
    (if (`self.IsAttacking1`)
      ;[1 1 1] When 2 seconds passed since started attacking, stop attacking.
      (set `self.FightStartTime` (+ (`self.FightStartTime`) (`self.DeltaSeconds`)))
      (if (> (`self.FightStartTime`) 2.0)
        (set `self.IsAttacking1` false)
        (set `self.FightStartTime` -1.0))
      (else
        ;[1 1 1] Set IsEating true, if the goal is close.
        (if (<= (`KismetMathLibrary.VSizeSquared` (- (`self.GoalLoc`) (`self.K2_GetActorLocation`))) 900.0)
          (if (> (`self.FightStartTime`) 0.0)
            (set `self.IsAttacking1` true)
            (set `self.FightStartTime` 0.0)
            (else
              (set `self.FightStartTime` (+ (`self.FightStartTime`) (`self.DeltaSeconds`)))))
          (else
            ;[1 1 1] Set the next moving point.
            (bind _returnvalue_2 (`NavigationSystem.FindPathToLocationSynchronously` (`self.K2_GetActorLocation`) (`self.GoalLoc`) null "/Script/AIModule.NavFilter_AIControllerDefault"))
            (bind _returnvalue_3 (`KismetMathLibrary.Normal` (- (`|GetArrayItem` (`NavigationPath.PathPoints` _returnvalue_2) 1) (`SceneComponent.K2_GetComponentLocation` (`self.CapsuleComponent`)))))
            (bind _returnvalue_4 (`KismetMathLibrary.Dot_VectorVector` (`SceneComponent.GetForwardVector` (`self.CapsuleComponent`)) _returnvalue_3))
            (bind _returnvalue_5 (>= _returnvalue_4 0.0))
            ;[1 1 1] Set AimTurnSpeed according to the positional relationship between the character and the next movement point.
            (if _returnvalue_5
              (set `self.AimTurnSpeed` (* (`KismetMathLibrary.Dot_VectorVector` _returnvalue_3 (`SceneComponent.GetRightVector` (`self.CapsuleComponent`))) 1.0))
              (else
                (set `self.AimTurnSpeed` -1.0)))
            ;[1 1 1] If a character is in front, stop.
            (bind (_outhit _returnvalue_6) (`KismetSystemLibrary.LineTraceSingle` _returnvalue (+ _returnvalue (* (`KismetMathLibrary.GetForwardVector` (`SceneComponent.K2_GetComponentRotation` (`self.CapsuleComponent`))) 500.0)) "TraceTypeQuery1"))
            (if _returnvalue_6
              (cast `Character` (`.HitActor` (`GameplayStatics.BreakHitResult` _outhit))
                (:`then`
                  (set `self.AimForwardSpeed` 1.0))
                (:`CastFailed`
                  (bind _returnvalue_7 (`KismetMathLibrary.VSizeSquared` _returnvalue_3))
                  ;[1 1 1] Set the AimForwardSpeed.
                  (set `self.AimForwardSpeed` (* (`KismetMathLibrary.SelectFloat` (`KismetMathLibrary.Abs` _returnvalue_4) 0.0 _returnvalue_5) (`KismetMathLibrary.SelectFloat` 1.0 (+ (* _returnvalue_7 0.08) 0.2) (>= _returnvalue_7 10.0))) :!label _label)))
              (else
                (goto _label)))))))))

(fn `UserConstructionScript`
  (`parent.UserConstructionScript`))
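; Raven character Blueprint that drives morph targets on the bird's high-poly mesh when IsMorphModel is set.
; BeginPlay applies initial head, throat, back and random morph weights.
; Each Tick eases head, throat and back weights toward high or low targets chosen by their morphing flags, using Lerp with DeltaSeconds as alpha.
; The random morph weight is reapplied without change, and nothing here sets the flags.
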(event `self.ReceiveBeginPlay`
  (`parent.ReceiveBeginPlay`)
  ;[1 1 1] Set the initial morph weights.
  (if (`self.IsMorphModel`)
    (`SkeletalMeshComponent.SetMorphTarget` (`self.Mesh`) "RavenHighPolyHeadMorph" (`self.HeadMorphIntensity`) true)
    (`SkeletalMeshComponent.SetMorphTarget` (`self.Mesh`) "RavenHighPolyThroatMorph" (`self.ThroatMorphIntensity`) true)
    (`SkeletalMeshComponent.SetMorphTarget` (`self.Mesh`) "RavenHighPolyBackMorph" (`self.BackMorphIntensity`) true)
    (`SkeletalMeshComponent.SetMorphTarget` (`self.Mesh`) "RavenHighPolyRundomMorph" (`self.Randomorphintensity`) true)))

(event `self.ReceiveTick`
  (params (DeltaSeconds :type "Float (single-precision)"))
  (`parent.ReceiveTick` DeltaSeconds)
  ;[1 1 1] Set the morph target intensity.
  (if (`self.IsMorphModel`)
    (set `self.HeadMorphIntensity` (`KismetMathLibrary.Lerp` (`self.HeadMorphIntensity`) (`KismetMathLibrary.SelectFloat` 1.0 0.1 (`self.IsHeadMorphing`)) (`self.DeltaSeconds`)))
    (set `self.ThroatMorphIntensity` (`KismetMathLibrary.Lerp` (`self.ThroatMorphIntensity`) (`KismetMathLibrary.SelectFloat` 1.0 0.1 (`self.IsThroatMorphing`)) (`self.DeltaSeconds`)))
    (set `self.BackMorphIntensity` (`KismetMathLibrary.Lerp` (`self.BackMorphIntensity`) (`KismetMathLibrary.SelectFloat` 1.0 0.1 (`self.IsBackMorphing`)) (`self.DeltaSeconds`)))
    ;[1 1 1] Set the morph target.
    (`SkeletalMeshComponent.SetMorphTarget` (`self.Mesh`) "RavenHighPolyHeadMorph" (`self.HeadMorphIntensity`) true)
    (`SkeletalMeshComponent.SetMorphTarget` (`self.Mesh`) "RavenHighPolyThroatMorph" (`self.ThroatMorphIntensity`) true)
    (`SkeletalMeshComponent.SetMorphTarget` (`self.Mesh`) "RavenHighPolyBackMorph" (`self.BackMorphIntensity`) true)
    (`SkeletalMeshComponent.SetMorphTarget` (`self.Mesh`) "RavenHighPolyRundomMorph" (`self.Randomorphintensity`) true)))

(fn `UserConstructionScript`
  (`parent.UserConstructionScript`))
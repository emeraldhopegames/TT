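; Cassowary character Blueprint that wanders between randomly chosen BP_CassowaryFood actors and pauses to eat at each.
; SelectFood picks a goal at BeginPlay and after each roughly five-second meal; without food, the bird stops.
; While seeking, Tick recomputes a synchronous navigation path, using dot products toward the next point to set turn and forward targets.
; Interpolated TurnSpeed and ForwardSpeed smooth the motion, with no direct movement calls here.
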(event `self.ReceiveBeginPlay`
  (`parent.ReceiveBeginPlay`)
  (`self.SelectFood`))

(event `self.ReceiveTick`
  (params (DeltaSeconds :type "Float (single-precision)"))
  (`parent.ReceiveTick` DeltaSeconds)
  ;[1 1 1] Is ther food?
  (if (`self.IsThereFood`)
    ;[1 1 1] Is eating?
    (if (`self.IsEating`)
      ;[1 1 1] Set the TurnSpeed.
      (set `self.TurnSpeed` (`KismetMathLibrary.FInterpTo` (`self.TurnSpeed`) (`self.AimTurnSpeed`) (`self.DeltaSeconds`) 1.0))
      ;[1 1 1] Set the ForwardSpeed
      (set `self.ForwardSpeed` (`KismetMathLibrary.FInterpTo` (`self.ForwardSpeed`) (`self.AimForwardSpeed`) (`self.DeltaSeconds`) 15.0))
      ;[1 1 1] When five seconds passed since started eating, look for the next food.
      (set `self.EatStartTime` (+ (`self.EatStartTime`) (`self.DeltaSeconds`)))
      (if (> (`self.EatStartTime`) 5.0)
        (set `self.IsEating` false)
        (set `self.EatStartTime` 0.0)
        (`self.SelectFood`))
      (else
        ;[1 1 1] Set IsEating true, if the goal is close.
        (if (<= (`KismetMathLibrary.VSizeSquared` (- (`self.GoalLoc`) (`self.K2_GetActorLocation`))) 10000.0)
          (set `self.IsEating` true)
          (set `self.EatStartTime` 0.0)
          ;[1 1 1] Stop the character.
          (set `self.AimTurnSpeed` 0.0)
          (set `self.AimForwardSpeed` 0.0)
          (else
            ;[1 1 1] Set the next moving point.
            (bind _returnvalue (`NavigationSystem.FindPathToLocationSynchronously` (`self.K2_GetActorLocation`) (`self.GoalLoc`)))
            (bind _returnvalue_2 (- (`|GetArrayItem` (`NavigationPath.PathPoints` _returnvalue) 1) (`SceneComponent.K2_GetComponentLocation` (`self.CapsuleComponent`))))
            (bind _returnvalue_3 (`KismetMathLibrary.Normal` _returnvalue_2))
            (bind _returnvalue_4 (`KismetMathLibrary.Dot_VectorVector` _returnvalue_3 (`SceneComponent.GetForwardVector` (`self.CapsuleComponent`))))
            (bind _returnvalue_5 (>= _returnvalue_4 0.0))
            ;[1 1 1] Set AimTurnSpeed according to the positional relationship between the character and the next movement point.
            (if _returnvalue_5
              (set `self.AimTurnSpeed` (* (`KismetMathLibrary.Dot_VectorVector` _returnvalue_3 (`SceneComponent.GetRightVector` (`self.CapsuleComponent`))) 180.0))
              (else
                (set `self.AimTurnSpeed` -180.0)))
            (bind _returnvalue_6 (`KismetMathLibrary.VSizeSquared` _returnvalue_2))
            ;[1 1 1] Set the AimForwardSpeed.
            (set `self.AimForwardSpeed` (* (`KismetMathLibrary.SelectFloat` (`KismetMathLibrary.Abs` _returnvalue_4) 0.0 _returnvalue_5) (`KismetMathLibrary.SelectFloat` 1.0 (+ (* _returnvalue_6 8e-09) 0.2) (>= _returnvalue_6 100000000.0))))
            ;[1 1 1] Set the TurnSpeed.
            (set `self.TurnSpeed` (`KismetMathLibrary.FInterpTo` (`self.TurnSpeed`) (`self.AimTurnSpeed`) (`self.DeltaSeconds`) 1.0))
            ;[1 1 1] Set the ForwardSpeed
            (set `self.ForwardSpeed` (`KismetMathLibrary.FInterpTo` (`self.ForwardSpeed`) (`self.AimForwardSpeed`) (`self.DeltaSeconds`) 15.0))))))
    (else
      ;[1 1 1] Stop the character.
      (set `self.AimTurnSpeed` 0.0)
      (set `self.AimForwardSpeed` 0.0)
      ;[1 1 1] Set the TurnSpeed.
      (set `self.TurnSpeed` (`KismetMathLibrary.FInterpTo` (`self.TurnSpeed`) (`self.AimTurnSpeed`) (`self.DeltaSeconds`) 1.0))
      ;[1 1 1] Set the ForwardSpeed
      (set `self.ForwardSpeed` (`KismetMathLibrary.FInterpTo` (`self.ForwardSpeed`) (`self.AimForwardSpeed`) (`self.DeltaSeconds`) 15.0)))))

(fn `SelectFood`
  ;[1 1 1] When there is a BP_Food, set IsThereFood true.
  (bind _outactors (`GameplayStatics.GetAllActorsOfClass` "/Game/CompleteAnimals/Birds/Cassowary/Blueprints/BP_CassowaryFood.BP_CassowaryFood_C"))
  (bind _returnvalue (`KismetArrayLibrary.Array_Length` _outactors))
  (if (> _returnvalue 0)
    (set `self.IsThereFood` true)
    ;[1 1 1] Select one BP_Food and make that position GoalLoc.
    (set `self.GoalLoc` (`self.K2_GetActorLocation` (`|GetArrayItem` _outactors (`KismetMathLibrary.RandomInteger` _returnvalue))))
    (else
      (set `self.IsThereFood` false))))

(fn `UserConstructionScript`
  (`parent.UserConstructionScript`))
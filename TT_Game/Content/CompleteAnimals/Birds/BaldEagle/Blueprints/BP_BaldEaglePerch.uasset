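; Perch actor that lands a BP_BaldEagleCharacter on a branch when it overlaps the trigger box.
; On overlap it scales the foot arrow offsets, cached at construction, by the eagle's scale and repositions the body arrows using world-up height to allow for tilted branches.
; A dot product with the eagle's forward vector picks one of two opposite-side arrow sets, which is passed to StartLandToPerch.
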(event `self.Box.OnComponentBeginOverlap`
  (params (OverlappedComponent :type "PrimitiveComponent Object Reference") (OtherActor :type "Actor Object Reference") (OtherComp :type "PrimitiveComponent Object Reference") (OtherBodyIndex :type Integer) (bFromSweep :type Boolean) (SweepResult :type "HitResult Structure (by ref)"))
  (bind _arrow1 (`self.Arrow1`))
  ;[1 1 1] When the eagle overlaps in the box.
  (bind _asbp_bald_eagle_character (cast `/Game/CompleteAnimals/Birds/BaldEagle/Blueprints/BP_BaldEagleCharacter` OtherActor))
  ;[1 1 1] Set the arrow scale according to eagle scale.
  (`self.ArrowsScaling` (`/Game/CompleteAnimals/Birds/BaldEagle/Blueprints/BP_BaldEagleCharacter.Scale` _asbp_bald_eagle_character))
  (bind _returnvalue (> (`KismetMathLibrary.Dot_VectorVector` (`self.GetActorForwardVector` _asbp_bald_eagle_character) (`SceneComponent.GetForwardVector` _arrow1)) 0.0))
  ;[1 1 1] Select the arrow to be set according to the positional relationship between the branch and the Bald eagle.
  (bind _asarrow_component (cast `ArrowComponent` (`KismetMathLibrary.SelectObject` _arrow1 (`self.Arrow2`) _returnvalue)))
  (bind _asarrow_component_2 (cast `ArrowComponent` (`KismetMathLibrary.SelectObject` (`self.LeftFootArrow1`) (`self.LeftFootArrow2`) _returnvalue)))
  (bind _asarrow_component_3 (cast `ArrowComponent` (`KismetMathLibrary.SelectObject` (`self.RightFootArrow1`) (`self.RightFootArrow2`) _returnvalue)))
  (`/Game/CompleteAnimals/Birds/BaldEagle/Blueprints/BP_BaldEagleCharacter.StartLandToPerch` _asbp_bald_eagle_character _asarrow_component _asarrow_component_2 _asarrow_component_3))

(fn `ArrowsScaling`
  (params (EagleScale :type "Float (double-precision)" :default 1.0))
  (bind _returnvalue (* EagleScale 5.013489))
  (bind _returnvalue_2 (* EagleScale 48.902954))
  (bind _defaultsceneroot (`self.DefaultSceneRoot`))
  (bind _defaultsceneroot_2 (`self.DefaultSceneRoot`))
  ;[1 1 1] Set the position of RightFootArrow1 according to EagleScale.
  (`SceneComponent.K2_SetRelativeLocationAndRotation` (`self.RightFootArrow1`) (* (`self.RightFootArrow1DefaultPos`) EagleScale) (`SceneComponent.RelativeRotation` (`self.RightFootArrow1`)) false false)
  ;[1 1 1] Set the position of LeftFootArrow1 according to EagleScale.
  (`SceneComponent.K2_SetRelativeLocationAndRotation` (`self.LeftFootArrow1`) (* (`self.LeftFoorArrow1DefaultPos`) EagleScale) (`SceneComponent.RelativeRotation` (`self.LeftFootArrow1`)) false false)
  ;[1 1 1] Set the position of RightFootArrow2 according to EagleScale.
  (`SceneComponent.K2_SetRelativeLocationAndRotation` (`self.RightFootArrow2`) (* (`self.RightFootArrow2DefaultPos`) EagleScale) (`SceneComponent.RelativeRotation` (`self.RightFootArrow2`)) false false)
  ;[1 1 1] Set the position of LeftFootArrow2 according to EagleScale.
  (`SceneComponent.K2_SetRelativeLocationAndRotation` (`self.LeftFootArrow2`) (* (`self.LeftFoorArrow2DefaultPos`) EagleScale) (`SceneComponent.RelativeRotation` (`self.LeftFootArrow2`)) false false)
  ;[1 1 1] Adjustment of the position of the arrow when the branch is tilted.
  (`SceneComponent.K2_SetWorldLocation` (`self.Arrow1`) (+ (`SceneComponent.K2_GetComponentLocation` _defaultsceneroot_2) (+ (* (`SceneComponent.GetRightVector` _defaultsceneroot_2) _returnvalue) (`KismetMathLibrary.MakeVector` 0.0 0.0 _returnvalue_2))) false false)
  (`SceneComponent.K2_SetWorldLocation` (`self.Arrow2`) (+ (`SceneComponent.K2_GetComponentLocation` _defaultsceneroot) (+ (* (`SceneComponent.GetRightVector` _defaultsceneroot) (* -1 _returnvalue)) (`KismetMathLibrary.MakeVector` 0.0 0.0 _returnvalue_2))) false false))

(fn `UserConstructionScript`
  ;[1 1 1] Set the default position of arrows.
  (set `self.LeftFoorArrow1DefaultPos` (`SceneComponent.RelativeLocation` (`self.LeftFootArrow1`)))
  (set `self.RightFootArrow1DefaultPos` (`SceneComponent.RelativeLocation` (`self.RightFootArrow1`)))
  (set `self.LeftFoorArrow2DefaultPos` (`SceneComponent.RelativeLocation` (`self.LeftFootArrow2`)))
  (set `self.RightFootArrow2DefaultPos` (`SceneComponent.RelativeLocation` (`self.RightFootArrow2`))))
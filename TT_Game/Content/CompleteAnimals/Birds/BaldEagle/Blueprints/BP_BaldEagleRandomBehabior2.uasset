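; Bald eagle character Blueprint that autonomously switches between random ground behaviors, perching and flight.
; Tick branches on movement mode: walking picks random actions or takes off on a timer or player proximity, while flying steers toward random perch or landing-point actors.
; Obstacle avoidance spreads a sphere-trace grid over successive frames, one trace per tick.
; Hit and overlap events handle eagle collisions, landing and climbing away from water.
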(event `self.ReceiveTick`
  (params (DeltaSeconds :type "Float (single-precision)"))
  (bind _returnvalue (`SceneComponent.K2_GetComponentToWorld` (`self.CapsuleComponent`)))
  (bind _returnvalue_2 (< (`self.FlyForwardSpeed`) (`self.MeanForwardSpeed`)))
  (bind _returnvalue_3 (`KismetMathLibrary.InverseTransformLocation` _returnvalue (`self.ObjectivePoint`)))
  (bind _returnvalue_4 (- (.z (`self.ObjectivePoint`)) (.z (.location _returnvalue))))
  (bind (_remainder _returnvalue_5) (`KismetMathLibrary.FMod` (`KismetMathLibrary.Conv_IntToDouble` (`self.CurrentTraceNumber`)) (`KismetMathLibrary.Conv_IntToDouble` (+ (`self.HorizontalDivisionNumber`) 1))))
  (bind _y (.y (`KismetMathLibrary.Normal` _returnvalue_3)))
  (bind _returnvalue_6 (/ (* (`self.TraceSightDistance`) -3.0) (.x (`KismetMathLibrary.InverseTransformLocation` (`SceneComponent.K2_GetComponentToWorld` (`self.CapsuleComponent`)) (`self.LastHitLocation`)))))
  (bind _returnvalue_7 (> (`KismetMathLibrary.VSizeSquared` _returnvalue_3) 20000.0))
  (`parent.ReceiveTick` DeltaSeconds)
  ;[1 1 1] IsWalking?
  (if (`CharacterMovementComponent.IsWalking` (`self.CharacterMovement`))
    ;[1 1 1] Is LandingPerch true?
    (if (`self.IsLandingPerch`)
      ;[1 1 1] When IsLandingPerch is true
      (set `self.ChangeTime` (+ (`self.ChangeTime`) (`GameplayStatics.GetWorldDeltaSeconds`)))
      (if (> (`self.ChangeTime`) 10.0)
        (set `self.IsSoaring` true)
        (set `self.FlyForwardSpeed` 10.0)
        (set `self.UpSpeed` 2.0)
        (set `self.FlyForwardAcceleration` 5.0)
        (set `self.FlyUpAcceleration` 2.0)
        (`KismetSystemLibrary.Delay` 0.5)
        (`self.Soar`)
        (`self.SetObjectivePoint` true)
        (set `self.IsObjectivePointLand` true)
        (set `self.IsTryLandingToLand` false)
        (set `self.IsLandingPerch` false))
      (else
        ;[1 1 1] If player is near then soar.
        (if (and (< (`KismetMathLibrary.VSizeSquared` (- (`self.K2_GetActorLocation` (`self.Player`)) (`self.K2_GetActorLocation`))) (`self.PlayerFindDistanceSquared`)) (not (`self.SoaringStart`)))
          (set `self.SoaringStart` true)
          (set `self.IdleTransitionTime` 0.0)
          (`self.BehaviorOff`))
        ;[1 1 1] Random behabior at the ground.
        ;;[1 1 1] Turn the Bald eagle
        (`self.IsDoingSomething`)
        (if (and (not false) (`self.IsLived`))
          (`SceneComponent.K2_AddLocalRotation` (`self.CapsuleComponent`) (`KismetMathLibrary.MakeRotator` 0.0 0.0 (* (* (`self.DeltaSeconds`) (`self.TurnSpeed`)) 45.0)) false false))
        (if (> (`self.ChangeTime`) (`self.NextChangeTime`))
          (if (`self.IsSoaring`)
            _
            (elif (`self.SoaringStart`)
              (if (>= (`self.IdleTransitionTime`) 3.0)
                ;;[1 1 1] Soar
                (if (and (!= (`KismetArrayLibrary.Array_Length` (`self.LandingPoints`)) 0) (!= (`KismetArrayLibrary.Array_Length` (`self.Perches`)) 0))
                  (set `self.SoaringStart` false)
                  (set `self.IsSoaring` true)
                  (set `self.FlyForwardSpeed` 10.0)
                  (set `self.UpSpeed` 2.0)
                  (set `self.FlyForwardAcceleration` 5.0)
                  (set `self.FlyUpAcceleration` 2.0)
                  (if (< (`KismetMathLibrary.Abs` (`self.ForwardSpeed`)) 0.1)
                    (`KismetSystemLibrary.Delay` 0.35))
                  (`self.Soar`)
                  (`self.SetObjectivePoint` (== (`KismetArrayLibrary.Array_Length` (`self.Perches`)) 0))
                  (set `self.IsTryLandingToLand` false)
                  (set `self.IsObjectivePointLand` false)
                  (set `self.ChangeTime` 0.0)
                  (set `self.NextChangeTime` 0.0)
                  (else
                    (set `self.ChangeTime` 0.0 :!label _label)
                    (set `self.NextChangeTime` (`KismetMathLibrary.RandomFloatInRange` 1.0 3.0))
                    (set `self.InitialForwardSpeed` (`self.ForwardSpeed`))
                    (set `self.AimForwardSpeed` (`KismetMathLibrary.RandomFloatInRange` -0.5 1.0))
                    (set `self.InitialTurnSpeed` (`self.TurnSpeed`))
                    (set `self.AimTurnSpeed` (`KismetMathLibrary.RandomFloatInRange` -1.0 1.0)))))
              (else
                (`self.BehaviorOff`)
                (switch `int` (`KismetMathLibrary.RandomIntegerInRange` 0 10)
                  (:`Default`
                    (set `self.SoaringStart` true)
                    (set `self.IdleTransitionTime` 0.0)
                    (`self.BehaviorOff`))
                  (:`0`
                    (set `self.IsGrooming` true)
                    (set `self.ChangeTime` 0.0 :!label _label_2)
                    (set `self.NextChangeTime` (`KismetMathLibrary.RandomFloatInRange` 1.0 3.0))
                    (set `self.InitialForwardSpeed` (`self.ForwardSpeed`))
                    (set `self.AimForwardSpeed` 0.0)
                    (set `self.InitialTurnSpeed` (`self.TurnSpeed`))
                    (set `self.AimTurnSpeed` 0.0))
                  (:`1`
                    (set `self.IsEating` true)
                    (goto _label_2))
                  (:`2`
                    (set `self.IsCrying` true)
                    (goto _label_2))
                  (:`3`
                    (set `self.IsAttacking` true)
                    (goto _label))
                  (:`4`
                    (set `self.IsAttacking2` true)
                    (goto _label))
                  (:`5`
                    (goto _label))
                  (:`6`
                    (set `self.IsHopping` false)
                    (goto _label))
                  (:`7`
                    (set `self.IsHopping` true)
                    (goto _label))))))
          (else
            (bind _output_get (set `self.ChangeTime` (+ (`self.ChangeTime`) (`GameplayStatics.GetWorldDeltaSeconds`))))
            ;;[1 1 1] Change the Forward Speed.
            (set `self.ForwardSpeed` (`KismetMathLibrary.Lerp` (`self.InitialForwardSpeed`) (`self.AimForwardSpeed`) (`KismetMathLibrary.FClamp` _output_get)))
            ;;[1 1 1] Change the TurnSpeed.
            (set `self.TurnSpeed` (`KismetMathLibrary.Lerp` (`self.InitialTurnSpeed`) (`self.AimForwardSpeed`) (`KismetMathLibrary.FClamp` _output_get)))))))
    (else
      ;[1 1 1] IsFlying?
      (if (`NavMovementComponent.IsFlying` (`self.CharacterMovement`))
        ;[1 1 1] Turn the Bald eagle.
        (`SceneComponent.K2_AddLocalRotation` (`self.CapsuleComponent`) (`KismetMathLibrary.MakeRotator` 0.0 0.0 (* (* (`self.DeltaSeconds`) (`self.TurnSpeed`)) 45.0)) false false)
        ;[1 1 1] Is TryLandPerch true?
        (if (`self.IsTryLandPerch`)
          ;[1 1 1] When IsTryLandPerch is true
          (set `self.ChangeTime` (+ (`self.ChangeTime`) (`GameplayStatics.GetWorldDeltaSeconds`)))
          (if (> (`self.ChangeTime`) 5.0)
            ;;[1 1 1] If Bald eagle can not landing to perch, when 5 seconds after.
            (set `self.IsTryLandPerch` false)
            (`self.SetObjectivePoint` true)
            (set `self.IsObjectivePointLand` true))
          (else
            ;[1 1 1] Is TryLandingToLand true?
            (if (`self.IsTryLandingToLand`)
              (if (not (`self.IsFlyOnWater`))
                ;[1 1 1] Decelerate when IsTryLandingToLand is true.
                (set `self.AimFlyUpAcceleration` -5.0)
                (set `self.AimFlyForwardAcceleration` -5.0))
              (else
                ;[1 1 1] Is there obstacle?
                (if (not (`self.IsThereObstacle`))
                  ;[1 1 1] Movement mode is Flying and IsTryLandPerch is false and IsTryingToLand is false.
                  (if (> (`KismetMathLibrary.Abs` _returnvalue_4) 1.0)
                    (set `self.UpAccelerationChange` true)
                    (set `self.AimFlyUpAcceleration` (`KismetMathLibrary.FClamp` _returnvalue_4 -5.0 5.0))
                    (else
                      (set `self.UpAccelerationChange` false)
                      (set `self.AimFlyUpAcceleration` 0.0)))
                  ;;[1 1 1] Calculate the AimTurnSpeed from relative position of Bald eagle and ObjectivePoint.
                  (if (> (.x (`KismetMathLibrary.Normal` _returnvalue_3)) 0.0)
                    (set `self.AimTurnSpeed` (* _y 2.5))
                    (elif (> _y 0.0)
                      (set `self.AimTurnSpeed` 1.0)
                      (else
                        (set `self.AimTurnSpeed` -1.0))))
                  ;;[1 1 1] (far away and slow) or (near and fast) then forward accelerate.
                  (if (or (and (not _returnvalue_7) (not _returnvalue_2)) (and _returnvalue_7 _returnvalue_2))
                    (set `self.ForwardAccelerationChange` true)
                    (set `self.AimFlyForwardAcceleration` (`KismetMathLibrary.FClamp` (.x _returnvalue_3) -5.0 5.0))
                    (else
                      (set `self.ForwardAccelerationChange` false)
                      (set `self.AimFlyForwardAcceleration` 0.0)
                      (set `self.AimForwardSpeed` 0.0))))
                ;[1 1 1] If IsThereObstacle is True, then object avoidance.
                ;;[1 1 1] Trace for lattice point.
                (bind (_outhit _returnvalue_8) (`KismetSystemLibrary.SphereTraceSingle` (`SceneComponent.K2_GetComponentLocation` (`self.CapsuleComponent`)) (+ (+ (+ (* (`SceneComponent.GetRightVector` (`self.CapsuleComponent`)) (* (+ _remainder 1.0) (`self.TraceGridWidth`))) (* (`SceneComponent.GetUpVector` (`self.CapsuleComponent`)) (* _returnvalue_5 (`self.TraceGridHeight`)))) (+ (+ (`SceneComponent.K2_GetComponentLocation` (`self.CapsuleComponent`)) (* (* (`SceneComponent.GetUpVector` (`self.CapsuleComponent`)) (`self.TraceHalfHeight`)) -1.0)) (* (* (`SceneComponent.GetRightVector` (`self.CapsuleComponent`)) (`self.TraceHalfWidth`)) -1.0))) (* (`SceneComponent.GetForwardVector` (`self.CapsuleComponent`)) (`self.TraceSightDistance`))) (`CapsuleComponent.GetScaledCapsuleRadius` (`self.CapsuleComponent`)) "TraceTypeQuery1" false (`self.Perches`)))
                (set `self.DoesHitAtLeastOnce` (or _returnvalue_8 (`self.DoesHitAtLeastOnce`)))
                (set `self.LastHitLocation` (`.Location` (`GameplayStatics.BreakHitResult` _outhit)))
                ;;[1 1 1] All latice points were traced?
                (if (<= (`self.CurrentTraceNumber`) (`self.MaxTraceNumber`))
                  ;;[1 1 1] Increment the CurrentTraceNumber.
                  (`/Engine/EditorBlueprintResources/StandardMacros.IncrementInt` (`self.CurrentTraceNumber`)
                    (:`  `
                      _))
                  (else
                    ;;[1 1 1] Initialize the variables.
                    (set `self.CurrentTraceNumber` 0)
                    (set `self.WasThereObstacle` (`self.IsThereObstacle`))
                    (bind _output_get_2 (set `self.IsThereObstacle` (`self.DoesHitAtLeastOnce`)))
                    (set `self.DoesHitAtLeastOnce` false)
                    (if _output_get_2
                      ;;[1 1 1] Was there Obstacle?
                      (if (not (`self.WasThereObstacle`))
                        ;;[1 1 1] Set the AimTurnSpeed according to the relative location of LasHitLocation from capsule component.
                        (if (> (.y (`KismetMathLibrary.InverseTransformLocation` (`SceneComponent.K2_GetComponentToWorld` (`self.CapsuleComponent`)) (`self.LastHitLocation`))) 0.0)
                          (set `self.AimTurnSpeed` -2.5)
                          (else
                            (set `self.AimTurnSpeed` 2.5))))
                      ;;[1 1 1] If not IsTryLandingToLand then AimFlyUpAcceleration set 5.
                      (if (not (`self.IsTryLandingToLand`))
                        (set `self.AimFlyUpAcceleration` 5.0))
                      ;;[1 1 1] Set the FlyForwardAcceleration and AimFlyForwardAcceleration according to LastHitLocation.
                      (set `self.AimFlyForwardAcceleration` _returnvalue_6)
                      (set `self.FlyForwardAcceleration` _returnvalue_6)
                      (set `self.ForwardAccelerationChange` true))))
                (if (`self.IsObjectivePointLand`)
                  (if (< (`KismetMathLibrary.VSizeSquared` (- (`SceneComponent.K2_GetComponentLocation` (`self.CapsuleComponent`)) (`self.ObjectivePoint`))) 20000.0)
                    (set `self.IsTryLandingToLand` true)
                    (set `self.ChangeTime` 0.0)
                    (set `self.NextChangeTime` 5.0)
                    (set `self.ForwardAccelerationChange` false)
                    (set `self.UpAccelerationChange` false)))))))
        (else
          ;[1 1 1] IsSwimming
          (if (`NavMovementComponent.IsSwimming` (`self.CharacterMovement`))
            ;[1 1 1] Turn the Bald eagle.
            (`SceneComponent.K2_AddLocalRotation` (`self.CapsuleComponent`) (`KismetMathLibrary.MakeRotator` 0.0 0.0 (* (* (`self.DeltaSeconds`) (`self.TurnSpeed`)) 45.0)) false false)
            (set `self.ForwardSpeed` 1.0)
            (set `self.TurnSpeed` 0.0)))))))

(event `self.ReceiveBeginPlay`
  (set `self.Player` (`GameplayStatics.GetPlayerPawn` 0))
  ;[1 1 1] Set the Perches
  (bind _outactors (`GameplayStatics.GetAllActorsOfClass` "/Game/CompleteAnimals/Birds/BaldEagle/Blueprints/BP_BaldEaglePerch.BP_BaldEaglePerch_C"))
  (set `self.Perches` _outactors)
  (set `self.APerch` (`|GetArrayItem` _outactors (`KismetMathLibrary.RandomIntegerInRange` 0 (- (`KismetArrayLibrary.Array_Length` _outactors) 1))))
  ;[1 1 1] Set the LandingPoints
  (bind _outactors_2 (`GameplayStatics.GetAllActorsOfClass` "/Game/CompleteAnimals/Birds/BaldEagle/Blueprints/BP_LandingPoint.BP_LandingPoint_C"))
  (bind _output_get (set `self.LandingPoints` _outactors_2))
  (set `self.LandingPoint` (`|GetArrayItem` _output_get (`KismetMathLibrary.RandomIntegerInRange` 0 (- (`KismetArrayLibrary.Array_Length` _output_get) 1))))
  ;[1 1 1] Set the MaxTraceNumber
  (set `self.MaxTraceNumber` (* (+ (`self.VerticalDivisionNumber`) 1) (+ (`self.HorizontalDivisionNumber`) 1)))
  ;[1 1 1] Set the TraceHalfHeight
  (set `self.TraceHalfHeight` (* (`CapsuleComponent.GetScaledCapsuleHalfHeight` (`self.CapsuleComponent`)) 3.0))
  ;[1 1 1] Set the TraceHalfWidth
  (set `self.TraceHalfWidth` (* (`CapsuleComponent.GetScaledCapsuleRadius` (`self.CapsuleComponent`)) 3.0))
  ;[1 1 1] Set the TraceGridHeight
  (set `self.TraceGridHeight` (/ (* (`self.TraceHalfHeight`) 2.0) (`KismetMathLibrary.Conv_IntToDouble` (`self.VerticalDivisionNumber`))))
  ;[1 1 1] Set the TraceGridWidth
  (set `self.TraceGridWidth` (/ (* (`self.TraceHalfWidth`) 2.0) (`KismetMathLibrary.Conv_IntToDouble` (`self.HorizontalDivisionNumber`))))
  ;[1 1 1] Set the TraceSightDistance
  (set `self.TraceSightDistance` (* (`self.TraceSightDistance`) (`self.Scale`))))

(event `self.PushedOutFromPerch`
  ;[1 1 1] Soaring when pushed out from perch.
  (set `self.IsSoaring` true)
  (set `self.FlyForwardSpeed` 10.0)
  (set `self.UpSpeed` 2.0)
  (set `self.FlyForwardAcceleration` 5.0)
  ;[1 1 1] Movement mode is Flying and IsTryLandPerch is false and IsTryingToLand is false.
  (set `self.FlyUpAcceleration` 2.0)
  (`self.Soar`)
  (set `self.IsObjectivePointLand` true)
  (set `self.IsLandingPerch` false)
  (set `self.IsTryLandingToLand` false)
  (set `self.IsObjectivePointLand` true)
  (`self.SetObjectivePoint` true))

(event `self.CapsuleComponent.OnComponentHit`
  (params (HitComponent :type "PrimitiveComponent Object Reference") (OtherActor :type "Actor Object Reference") (OtherComp :type "PrimitiveComponent Object Reference") (NormalImpulse :type "Vector Structure") (Hit :type "HitResult Structure (by ref)"))
  ;[1 1 1] Collided the other eagle?
  (cast `/Game/CompleteAnimals/Birds/BaldEagle/Blueprints/BP_BaldEagleCharacter` OtherActor
    (:`then`
      ;[1 1 1] IsLandingPerch?
      (if (`self.IsLandingPerch`)
        ;[1 1 1] When Hit other Bald eagle on the perch.
        (set `self.IsLandingPerch` false)
        (`self.SetObjectivePoint` true)
        (set `self.IsSoaring` true)
        (set `self.FlyForwardSpeed` 10.0)
        (set `self.UpSpeed` 2.0)
        (set `self.FlyForwardAcceleration` 5.0)
        (set `self.FlyUpAcceleration` 2.0)
        (if (< (`KismetMathLibrary.Abs` (`self.ForwardSpeed`)) 0.1)
          (`KismetSystemLibrary.Delay` 0.35))
        (`self.Soar`)
        (set `self.IsObjectivePointLand` true)
        (else
          ;[1 1 1] IsWalking?
          (if (`CharacterMovementComponent.IsWalking` (`self.CharacterMovement`))
            ;[1 1 1] When Hit other Bald eagle at the ground.
            (switch `int` (`KismetMathLibrary.RandomIntegerInRange` 0 5)
              (:`Default`
                (set `self.JumpStart` true)
                (`KismetSystemLibrary.Delay` 0.3)
                (`self.Jump`)
                (set `self.JumpStart` false))
              (:`0`
                (set `self.IsAttacking` true))
              (:`1`
                (set `self.IsAttacking2` true))
              (:`2`
                (set `self.IsHitting` true)))
            (else
              ;[1 1 1] IsFlying?
              (if (`NavMovementComponent.IsFlying` (`self.CharacterMovement`)) :!label _label_3
                ;[1 1 1] IsTryLandPerch?
                (if (not (`self.IsTryLandPerch`))
                  ;[1 1 1] Change to the setting to be landing.
                  (set `self.IsSoaring` false)
                  (set `self.ChangeTime` 0.0)
                  (set `self.NextChangeTime` 5.0)
                  (set `self.ForwardAccelerationChange` false)
                  (set `self.UpAccelerationChange` false)
                  (`PrimitiveComponent.SetEnableGravity` (`self.CapsuleComponent`) true)
                  (`CharacterMovementComponent.SetMovementMode` (`self.CharacterMovement`) "MOVE_Walking" 0)
                  (`PrimitiveComponent.SetSimulatePhysics` (`self.CapsuleComponent`) false)
                  (set `self.IKInterpSpeed` 10.0))))))))
    (:`CastFailed`
      (goto _label_3))))

(event `self.Box_0.OnComponentBeginOverlap`
  (params (OverlappedComponent :type "PrimitiveComponent Object Reference") (OtherActor :type "Actor Object Reference") (OtherComp :type "PrimitiveComponent Object Reference") (OtherBodyIndex :type Integer) (bFromSweep :type Boolean) (SweepResult :type "HitResult Structure (by ref)"))
  (bind `_asフィジックス_ボリューム` (cast `PhysicsVolume` OtherActor))
  (if (`PhysicsVolume.bWaterVolume` `_asフィジックス_ボリューム`)
    (set `self.AimFlyUpAcceleration` 5.0)
    (set `self.AimFlyForwardAcceleration` 5.0)
    (set `self.UpSpeed` 5.0)
    (set `self.IsFlyOnWater` true)))

(event `self.Box_0.OnComponentEndOverlap`
  (params (OverlappedComponent :type "PrimitiveComponent Object Reference") (OtherActor :type "Actor Object Reference") (OtherComp :type "PrimitiveComponent Object Reference") (OtherBodyIndex :type Integer))
  (bind `_asフィジックス_ボリューム` (cast `PhysicsVolume` OtherActor))
  (if (`PhysicsVolume.bWaterVolume` `_asフィジックス_ボリューム`)
    (set `self.IsFlyOnWater` false)
    (if (`self.IsTryLandingToLand`)
      (set `self.AimFlyUpAcceleration` -5.0)
      (set `self.AimFlyForwardAcceleration` -5.0))))

(fn `SetObjectivePoint`
  (params (IsLand :type Boolean))
  (bind _perches (`self.Perches`))
  (bind _landingpoints (`self.LandingPoints`))
  ;[1 1 1] Case where the ObjectivePoint is on the ground or not.
  (if IsLand
    ;[1 1 1] Random select LandingPoint from LandingPoints.
    (bind _output_get (set `self.LandingPoint` (`|GetArrayItem` _landingpoints (`KismetMathLibrary.RandomIntegerInRange` 0 (- (`KismetArrayLibrary.Array_Length` _landingpoints) 1)))))
    (set `self.ObjectivePoint` (`SceneComponent.K2_GetComponentLocation` (`/Game/CompleteAnimals/Birds/BaldEagle/Blueprints/BP_LandingPoint.DefaultSceneRoot` _output_get)))
    (else
      ;[1 1 1] Random Select APerch from Perches.
      (bind _output_get_2 (set `self.APerch` (`|GetArrayItem` _perches (`KismetMathLibrary.RandomIntegerInRange` 0 (- (`KismetArrayLibrary.Array_Length` _perches) 1)))))
      (set `self.ObjectivePoint` (`SceneComponent.K2_GetComponentLocation` (`/Game/CompleteAnimals/Birds/BaldEagle/Blueprints/BP_BaldEaglePerch.DefaultSceneRoot` _output_get_2))))))

(fn `UserConstructionScript`
  (`parent.UserConstructionScript`))
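; Bald eagle character that walks, swims, flies, lands on the ground and perches on supplied arrow points.
; Tick branches on movement mode, easing speeds, integrating flight acceleration and tracing downward to land while descending.
; Perch landing interpolates body and feet onto the arrows, and displacement from the perch triggers Soar.
; Otherwise, ground traces drive smoothed foot IK locations and slope-aligned rotations, with distances and speed factors scaled by actor size.
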(event `self.ReceiveTick`
  (params (DeltaSeconds :type "Float (single-precision)"))
  (bind _aimpercharrow (`self.AimPerchArrow`))
  (bind _scale (`self.Scale`))
  (bind _returnvalue (`SceneComponent.K2_GetComponentLocation` (`self.CapsuleComponent`)))
  (bind _returnvalue_2 (`SceneComponent.K2_GetComponentLocation` _aimpercharrow))
  (bind _returnvalue_3 (`SceneComponent.K2_GetComponentLocation` (`self.CapsuleComponent`)))
  (bind _y (.y (`KismetMathLibrary.InverseTransformLocation` (`SceneComponent.K2_GetComponentToWorld` (`self.CapsuleComponent`)) (+ _returnvalue_3 (`SceneComponent.GetForwardVector` (`self.AimPerchArrow`))))))
  (bind _y_2 (.y (`KismetMathLibrary.InverseTransformLocation` (`SceneComponent.K2_GetComponentToWorld` (`self.CapsuleComponent`)) (+ _returnvalue (* (`SceneComponent.GetForwardVector` _aimpercharrow) (`self.Scale`))))))
  (bind _output_get (set `self.DeltaSeconds` DeltaSeconds))
  ;[1 1 1] Set the elapsed time since starting transition to idle animation.
  (set `self.IdleTransitionTime` (+ _output_get (`self.IdleTransitionTime`)))
  ;[1 1 1] Set the elapsed time since landing started.
  (set `self.LandingStartTime` (+ (`self.DeltaSeconds`) (`self.LandingStartTime`)))
  ;[1 1 1] Set Forward Speed
  (set `self.ForwardSpeed` (`KismetMathLibrary.FInterpTo` (`self.ForwardSpeed`) (`self.AimForwardSpeed`) (`self.DeltaSeconds`) 5.0))
  ;[1 1 1] Set TurnSpeed
  (set `self.TurnSpeed` (`KismetMathLibrary.FInterpTo` (`self.TurnSpeed`) (`self.AimTurnSpeed`) (`self.DeltaSeconds`) 5.0))
  ;[1 1 1] IsWalking?
  (if (`CharacterMovementComponent.IsWalking` (`self.CharacterMovement`))
    ;[1 1 1] Is IsLandingPerch true?
    (if (`self.IsLandingPerch`)
      ;[1 1 1] IsLandingPerch is true.
      (if (> (`KismetMathLibrary.VSizeSquared` (- (`SceneComponent.K2_GetComponentLocation` (`self.CapsuleComponent`)) (`SceneComponent.K2_GetComponentLocation` (`self.AimPerchArrow`)))) (* (* _scale _scale) 625.0))
        (`self.PushedOutFromPerch`)
        (else
          ;;[1 1 1] Move the Bald eagle to AimPerchArrow.
          (`SceneComponent.K2_SetWorldLocation` (`self.CapsuleComponent`) (`KismetMathLibrary.VInterpTo` _returnvalue_3 (`SceneComponent.K2_GetComponentLocation` (`self.AimPerchArrow`)) (`self.DeltaSeconds`) 10.0) false false)
          ;;[1 1 1] Change the AimTurnSpeed according to positional relationship between Bald eagle and AimPerchArrow.
          (if (> _y 0.05)
            (set `self.AimTurnSpeed` 0.5)
            (elif (< _y -0.05)
              (set `self.AimTurnSpeed` -0.5)
              (else
                (set `self.AimTurnSpeed` 0.0))))
          ;;[1 1 1] Set feet location and rotation to PerchLeftFootArrow and PerchRightFootArrow's location and rotation.
          (set `self.L_Tarsus_2EffectorLoc` (`SceneComponent.K2_GetComponentLocation` (`self.PerchLeftFootArrow`)) :!label _label)
          (set `self.R_Tarsus_2EffectorLoc` (`SceneComponent.K2_GetComponentLocation` (`self.PerchRightFootArrow`)))
          (set `self.R_Tarsus_2Rot` (`KismetMathLibrary.RInterpTo` (`self.R_Tarsus_2Rot`) (`SceneComponent.K2_GetComponentRotation` (`self.PerchRightFootArrow`)) (`GameplayStatics.GetWorldDeltaSeconds`) (`self.FootRotInterpSpeed`)))
          (set `self.L_Tarsus_2Rot` (`KismetMathLibrary.RInterpTo` (`self.L_Tarsus_2Rot`) (`SceneComponent.K2_GetComponentRotation` (`self.PerchLeftFootArrow`)) (`GameplayStatics.GetWorldDeltaSeconds`) (`self.FootRotInterpSpeed`)))
          ;[1 1 1] Change IdleParameter
          (if (> (`self.IdleParameterChangeTime`) 1.0) :!label _label_2
            (set `self.IdleParameterChangeTime` 0.0)
            (set `self.AimIdleParameter` (`KismetMathLibrary.Conv_IntToDouble` (`KismetMathLibrary.RandomIntegerInRange` -2 2)))
            (else
              (set `self.IdleParameter` (`KismetMathLibrary.FInterpTo` (`self.IdleParameter`) (`self.AimIdleParameter`) (`self.DeltaSeconds`) 1.0))
              (set `self.IdleParameterChangeTime` (+ (`self.IdleParameterChangeTime`) (`self.DeltaSeconds`)))))))
      (else
        ;[1 1 1] Movement mode is Walking and IsLandingPerch is false.
        (`self.FootPlacement`)
        (bind _issomething (`self.IsDoingSomething`))
        (if (and (and (not _issomething) (`self.IsLived`)) (>= (`self.LandingStartTime`) 2.0))
          (`PawnMovementComponent.AddInputVector` (`self.CharacterMovement`) (* (* (`SceneComponent.GetForwardVector` (`self.CapsuleComponent`)) (`self.ForwardSpeed`)) (`self.InputScaleFactor`)) false)
          (goto _label_2))))
    (else
      ;[1 1 1] IsFalling?
      (if (`NavMovementComponent.IsFalling` (`self.CharacterMovement`))
        (`self.FootPlacement`)
        (else
          ;[1 1 1] IsFlying?
          (if (`NavMovementComponent.IsFlying` (`self.CharacterMovement`))
            ;[1 1 1] Is TryLandPerch true?
            (if (`self.IsTryLandPerch`)
              ;[1 1 1] Movement mode is Flying and IsTryLandPerch is true.
              ;;[1 1 1] Move the Bald eagle to AimPerchArrow.
              (`SceneComponent.K2_SetWorldLocation` (`self.CapsuleComponent`) (`KismetMathLibrary.VInterpTo` _returnvalue _returnvalue_2 (`self.DeltaSeconds`) (* (`self.Scale`) 3.0)) false false)
              ;;[1 1 1] Change the AimTurnSpeed according to positional relationship between Bald eagle and AimPerchArrow.
              (if (> _y_2 0.01)
                (set `self.AimTurnSpeed` 0.5)
                (elif (< _y_2 -0.01)
                  (set `self.AimTurnSpeed` -0.5)))
              ;;[1 1 1] True when the position and orientation of Bald ragle is close to AimPerchArrow.
              (if (and (< (`KismetMathLibrary.VSize` (- _returnvalue _returnvalue_2)) (* (`self.Scale`) 15.0)) (< (`KismetMathLibrary.Abs` _y_2) 0.05))
                ;;[1 1 1] When Bald Eagle's position and rotation is near the AimPerchArrow's  position and rotation.
                (set `self.IsLandingPerch` true)
                (set `self.IsTryLandPerch` false)
                (`CharacterMovementComponent.SetMovementMode` (`self.CharacterMovement`) "MOVE_Walking" 0)
                (set `self.IsSoaring` false)
                (`PrimitiveComponent.SetSimulatePhysics` (`self.CapsuleComponent`) false)
                (else
                  (goto _label)))
              (else
                ;[1 1 1] Movement mode is Flying and IsTryLandPerch is false.
                ;;[1 1 1] Change UpSpeed by FlyUpAccelaration.
                (set `self.UpSpeed` (`KismetMathLibrary.FClamp` (+ (`self.UpSpeed`) (* (`self.FlyUpAcceleration`) (`self.DeltaSeconds`))) (`self.MaxDownSpeed`) (`self.MaxUpSpeed`)))
                ;;[1 1 1] Change FlyForwardSpeed by FlyForwardAcceleration.
                (set `self.FlyForwardSpeed` (`KismetMathLibrary.FClamp` (+ (`self.FlyForwardSpeed`) (* (`self.FlyForwardAcceleration`) (`self.DeltaSeconds`))) 0.0 (`self.MaxFlySpeed`)))
                ;;[1 1 1] Change FlyUpAcceleration by AimFlyUpAcceleration.
                (set `self.FlyUpAcceleration` (`KismetMathLibrary.FInterpTo` (`self.FlyUpAcceleration`) (`self.AimFlyUpAcceleration`) (`self.DeltaSeconds`) 5.0))
                ;;[1 1 1] Change FlyForwardAcceleration by AimFlyForwardAcceleration.
                (set `self.FlyForwardAcceleration` (`KismetMathLibrary.FInterpTo` (`self.FlyForwardAcceleration`) (`self.AimFlyForwardAcceleration`) (`self.DeltaSeconds`) 5.0))
                (if (not (or (`self.ForwardAccelerationChange`) (`self.UpAccelerationChange`)))
                  ;;[1 1 1] Calculate AimFlyUpAccleration and AimFlyForwardAcceleration from FlyForwardSpeed.
                  (set `self.AimFlyUpAcceleration` (* (- (`self.MeanForwardSpeed`) (`self.FlyForwardSpeed`)) -0.1))
                  (set `self.AimFlyForwardAcceleration` (* (`self.FlyForwardSpeed`) -0.1)))
                ;;[1 1 1] Move the Bald Eagle by FlyForwardSpeed and FlyUpSpeed.
                (`self.K2_AddActorLocalOffset` (* (`KismetMathLibrary.MakeVector` (* (`self.FlyForwardSpeed`) (`self.DeltaSeconds`)) 0.0 (* (`self.UpSpeed`) (`self.DeltaSeconds`))) (`self.FlySpeedScaleFactor`)) true)
                (`self.FootPlacement`)
                (if (and (and (<= (`self.UpSpeed`) 0.0) (not (or (`self.ForwardAccelerationChange`) (`self.UpAccelerationChange`)))) (not (`self.IsTryLandPerch`)))
                  (set `self.IsSoaring` false)
                  ;;[1 1 1] Determining whether the Bald eagle is close to the ground or not.
                  (bind (_outhit _returnvalue_4) (`KismetSystemLibrary.LineTraceSingle` (`SceneComponent.K2_GetComponentLocation` (`self.CapsuleComponent`)) (`KismetMathLibrary.MakeVector` (.x (`SceneComponent.K2_GetComponentLocation` (`self.CapsuleComponent`))) (.y (`SceneComponent.K2_GetComponentLocation` (`self.CapsuleComponent`))) (- (.z (`SceneComponent.K2_GetComponentLocation` (`self.CapsuleComponent`))) (`self.IKTraceDistance`))) "TraceTypeQuery1"))
                  (if _returnvalue_4
                    ;;[1 1 1] Landing
                    (`CharacterMovementComponent.SetMovementMode` (`self.CharacterMovement`) "MOVE_Walking" 0)
                    (`PrimitiveComponent.SetEnableGravity` (`self.CapsuleComponent`) true)
                    (`PrimitiveComponent.SetSimulatePhysics` (`self.CapsuleComponent`) false)
                    (set `self.IKInterpSpeed` 10.0)
                    (`self.BehaviorOff`)
                    (set `self.AimForwardSpeed` 0.0)
                    (set `self.AimTurnSpeed` 0.0)
                    (set `self.ForwardSpeed` 0.0)
                    (set `self.TurnSpeed` 0.0)
                    (set `self.LandingStartTime` 0.0)))))
            (else
              ;[1 1 1] IsSwimming?
              (if (`NavMovementComponent.IsSwimming` (`self.CharacterMovement`))
                ;[1 1 1] Move the Character
                (`PawnMovementComponent.AddInputVector` (`self.CharacterMovement`) (* (* (`SceneComponent.GetForwardVector` (`self.CapsuleComponent`)) (`self.ForwardSpeed`)) (`self.InputScaleFactor`)) false)))))))))

(fn `BehaviorOff`
  ;[1 1 1] Turn off all actions.
  (set `self.IsAttacking` false)
  (set `self.IsAttacking2` false)
  (set `self.IsHitting` false)
  (set `self.IsGrooming` false)
  (set `self.IsCrying` false)
  (set `self.IsEating` false)
  (set `self.IsSleeping` false))

(fn `CanJumpInternal`
  (returns (ReturnValue :type Boolean))
  (return (and (and (and (and (and (and (and (and (or (`self.IsLandingPerch`) (`CharacterMovementComponent.IsWalking` (`self.CharacterMovement`))) (not (`self.IsAttacking`))) (not (`self.IsHitting`))) (not (`self.IsSneaking`))) (not (`self.IsGrooming`))) (not (`self.IsCrying`))) (not (`self.IsEating`))) (`self.IsLived`)) (not (`self.IsSleeping`)))))

(fn `FootPlacement`
  ;[1 1 1] Calculate the L_Tarsus_2EffectorLoc's Location and L_Tarsus_2's rotation.
  (bind (_legikeffectorloc _footrot) (`self.TraceIKEffector` (`self.L_Tarsus_2`) (`self.IKTraceDistance`) (`self.IKHeightOffset`)))
  ;[1 1 1] Set the left foot rotation.
  (set `self.L_Tarsus_2Rot` (`KismetMathLibrary.RInterpTo` (`self.L_Tarsus_2Rot`) _footrot (`GameplayStatics.GetWorldDeltaSeconds`) (`self.FootRotInterpSpeed`)))
  ;[1 1 1] Set the let foot IK effecter location.
  (set `self.L_Tarsus_2EffectorLoc` (`KismetMathLibrary.VInterpTo` (`self.L_Tarsus_2EffectorLoc`) _legikeffectorloc (`GameplayStatics.GetWorldDeltaSeconds`) (`self.IKInterpSpeed`)))
  ;[1 1 1] Calculate the R_Tarsus_2EffectorLoc's Location and R_Tarsus_2's rotation.
  (bind (_legikeffectorloc_2 _footrot_2) (`self.TraceIKEffector` (`self.R_Tarsus_2`) (`self.IKTraceDistance`) (`self.IKHeightOffset`)))
  ;[1 1 1] Set the right foot rotation.
  (set `self.R_Tarsus_2Rot` (`KismetMathLibrary.RInterpTo` (`self.R_Tarsus_2Rot`) _footrot_2 (`GameplayStatics.GetWorldDeltaSeconds`) (`self.FootRotInterpSpeed`)))
  ;[1 1 1] Set the right foot effector location.
  (set `self.R_Tarsus_2EffectorLoc` (`KismetMathLibrary.VInterpTo` (`self.R_Tarsus_2EffectorLoc`) _legikeffectorloc_2 (`GameplayStatics.GetWorldDeltaSeconds`) (`self.IKInterpSpeed`)))
  (return))

(fn `IsDoingSomething`
  (returns (IsSomething :type Boolean))
  (return (or (or (or (or (or (or (or (or (`self.IsCrying`) (`self.IsEating`)) (`self.IsSleeping`)) (`self.IsGrooming`)) (`self.IsHitting`)) (`self.IsAttacking`)) (`self.IsEating`)) (`self.IsSleeping`)) (`self.IsAttacking2`))))

(fn `PushedOutFromPerch`
  ;[1 1 1] When pushed out of a Perch by another eagle
  ;;[1 1 1] Set variable for soar.
  (set `self.IsSoaring` true)
  (set `self.FlyForwardSpeed` 10.0)
  (set `self.UpSpeed` 2.0)
  (set `self.FlyForwardAcceleration` 5.0)
  (set `self.FlyUpAcceleration` 2.0)
  (`self.Soar`)
  (set `self.IsObjectivePointLand` true)
  (set `self.IsLandingPerch` false))

(fn `Soar`
  ;[1 1 1] Initialize variables for flight
  (set `self.FlyForwardSpeed` 10.0)
  (set `self.UpSpeed` 2.0)
  (set `self.FlyForwardAcceleration` 5.0)
  (set `self.FlyUpAcceleration` 2.0)
  (set `self.AimFlyUpAcceleration` 0.0)
  (set `self.AimFlyForwardAcceleration` 0.0)
  (set `self.IKInterpSpeed` 50.0)
  (set `self.IsTryLandPerch` false)
  (set `self.IsLandingPerch` false)
  (`self.BehaviorOff`)
  ;[1 1 1] Change the settings for flight
  (`CharacterMovementComponent.SetMovementMode` (`self.CharacterMovement`) "MOVE_Flying" 0)
  (`PrimitiveComponent.SetEnableGravity` (`self.CapsuleComponent`) false)
  (`PrimitiveComponent.SetSimulatePhysics` (`self.CapsuleComponent`) true)
  (`ActorComponent.Activate` (`self.CharacterMovement`) false))

(fn `StartLandToPerch`
  (params (Arrow :type "ArrowComponent Object Reference") (LeftFootArrow :type "ArrowComponent Object Reference") (RightFootArrow :type "ArrowComponent Object Reference"))
  ;[1 1 1] Set variables to land on perch.
  (set `self.IsTryLandPerch` true)
  (`PrimitiveComponent.SetSimulatePhysics` (`self.CapsuleComponent`) false)
  (set `self.IsObjectivePointLand` false)
  ;[1 1 1] Set Arrows to determine the position of the torso and feet when landing on perch.
  (set `self.AimPerchArrow` Arrow)
  (set `self.PerchLeftFootArrow` LeftFootArrow)
  (set `self.PerchRightFootArrow` RightFootArrow))

(fn `TraceIKEffector`
  (params (FootName :type Name) (TraceDistance :type "Float (double-precision)" :default 50.0) (HeightOffset :type "Float (double-precision)" :default 10.0))
  (returns (LegIKEffectorLoc :type "Vector Structure") (FootRot :type "Rotator Structure"))
  (locals (GroundNormal :type "Vector Structure") (DoesReachThaGround :type Boolean) (InitialFootLocation :type "Vector Structure") (InitialFootRotation :type "Rotator Structure"))
  (bind _x (.x (`local.InitialFootLocation`)))
  (bind _y (.y (`local.InitialFootLocation`)))
  (bind _z (.z (`self.K2_GetActorLocation`)))
  (bind (_x_2 _y_2 _z_2) (`KismetMathLibrary.BreakRotIntoAxes` (`local.InitialFootRotation`)))
  (bind _returnvalue (`KismetMathLibrary.Cross_VectorVector` _y_2 (`local.GroundNormal`)))
  (bind _returnvalue_2 (`KismetMathLibrary.DegAsin` (`KismetMathLibrary.VSize` _returnvalue)))
  ;[1 1 1] Set the InitialFootLocation and InitialFootRotation  for use later.
  (set `local.InitialFootLocation` (`SceneComponent.GetSocketLocation` (`self.Mesh`) FootName))
  (set `local.InitialFootRotation` (`SceneComponent.GetSocketRotation` (`self.Mesh`) FootName))
  ;[1 1 1] Calculate the location of foot.
  ;;[1 1 1] Trace from foot location to the location lowered by the TraceDistance from the location of the foot
  (bind (_outhit _returnvalue_3) (`KismetSystemLibrary.LineTraceSingle` (`KismetMathLibrary.MakeVector` _x _y _z) (`KismetMathLibrary.MakeVector` _x _y (- _z TraceDistance)) "TraceTypeQuery1" true))
  ;;[1 1 1] Set the DoesReachTheGround and GroundNormal  for use later.
  (set `local.DoesReachThaGround` _returnvalue_3)
  (bind (_bblockinghit _binitialoverlap _time _distance _location _impactpoint _normal) (`GameplayStatics.BreakHitResult` _outhit))
  (set `local.GroundNormal` _normal)
  (return (`KismetMathLibrary.SelectVector` (`KismetMathLibrary.MakeVector` (.x _location) (.y _location) (+ (.z _location) HeightOffset)) (`local.InitialFootLocation`) (`local.DoesReachThaGround`)) (`KismetMathLibrary.SelectRotator` (`KismetMathLibrary.MakeRotationFromAxes` (`KismetMathLibrary.RotateAngleAxis` _x_2 _returnvalue_2 _returnvalue) (`local.GroundNormal`) (`KismetMathLibrary.RotateAngleAxis` _z_2 _returnvalue_2 _returnvalue)) (`local.InitialFootRotation`) (`local.DoesReachThaGround`))))

(fn `UserConstructionScript`
  (bind _scale (`self.Scale`))
  ;[1 1 1] Set the eagle's scale.
  (set `self.Scale` (.z (.scale (`self.GetTransform`))))
  ;[1 1 1] Set the scale dependent variables.
  (set `self.IKTraceDistance` (* (* (`CapsuleComponent.CapsuleHalfHeight` (`self.CapsuleComponent`)) 3.0) _scale))
  (set `self.IKHeightOffset` (* _scale (`self.IKHeightOffset`)))
  (set `self.InputScaleFactor` (* (`self.InputScaleFactor`) _scale))
  (set `self.FlySpeedScaleFactor` (* (`self.FlySpeedScaleFactor`) _scale)))
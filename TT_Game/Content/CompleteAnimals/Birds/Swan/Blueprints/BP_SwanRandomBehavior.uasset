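; Autonomous swan behavior Blueprint that wanders on ground or water and flies between BP_SwanLandingPoint actors.
; On a random timer, Tick picks behavior flags like grooming, eating or diving, blending speeds, or starts a takeoff run.
; Airborne, it climbs using height traces, steers toward a random landing point in local space, then decelerates to land.
; Collisions trigger attacks or jumps between walking swans, and landing attempts when flying.
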(event `self.ReceiveBeginPlay`
  ;[1 1 1] Set the LandingPoints
  (bind _outactors (`GameplayStatics.GetAllActorsOfClass` "/Game/CompleteAnimals/Birds/Swan/Blueprints/BP_SwanLandingPoint.BP_SwanLandingPoint_C"))
  (bind _output_get (set `self.LandingPoints` _outactors))
  (set `self.LandingPoint` (`|GetArrayItem` _output_get (`KismetMathLibrary.RandomIntegerInRange` 0 (- (`KismetArrayLibrary.Array_Length` _output_get) 1)))))

(event `self.ReceiveTick`
  (params (DeltaSeconds :type "Float (single-precision)"))
  (bind _returnvalue (`SceneComponent.K2_GetComponentLocation` (`self.CapsuleComponent`)))
  (bind _returnvalue_2 (`SceneComponent.K2_GetComponentLocation` (`self.CapsuleComponent`)))
  (bind _returnvalue_3 (< (`self.FlyForwardSpeed`) (`self.MeanForwardSpeed`)))
  (bind _returnvalue_4 (`KismetMathLibrary.InverseTransformLocation` (`SceneComponent.K2_GetComponentToWorld` (`self.CapsuleComponent`)) (`self.ObjectivePoint`)))
  (bind _returnvalue_5 (`KismetMathLibrary.Normal` _returnvalue_4))
  (bind _returnvalue_6 (> (`KismetMathLibrary.VSizeSquared` _returnvalue_4) 20000.0))
  (`parent.ReceiveTick` DeltaSeconds)
  ;[1 1 1] Walking or Swimming?
  (if (or (`CharacterMovementComponent.IsWalking` (`self.CharacterMovement`)) (`NavMovementComponent.IsSwimming` (`self.CharacterMovement`)))
    ;[1 1 1] Is RunningStart true?
    (if (`self.RunningStart`)
      ;[1 1 1] Increment the RunningStartTime
      (set `self.RunningStartTime` (+ (`self.RunningStartTime`) (`GameplayStatics.GetWorldDeltaSeconds`)))
      ;[1 1 1] If RunningStartTime>3 then soar.
      (if (> (`self.RunningStartTime`) 3.0)
        ;[1 1 1] Soar
        (`self.Soar`)
        (set `self.RunningStart` false)
        (set `self.Rising` true)
        (`self.SetObjectivePoint`)
        (set `self.IsTryLandingToLand` false)
        ;;[1 1 1] Set the variables so that rising and turning while Rising is true.
        (set `self.AimFlyUpAcceleration` 5.0)
        (set `self.IsUpAccelerating` true)
        (set `self.AimTurnSpeed` -1.0))
      (else
        ;[1 1 1] Random behabior at the ground or water.
        ;;[1 1 1] Turn the Swan
        (if (and (`self.IsLived`) (not (or (or (or (or (or (or (or (`self.IsCourtship`) (`self.IsSitdown`)) (`self.IsGrooming`)) (`self.IsStandFlap`)) (`self.IsEating`)) (`self.IsAttacking`)) (`self.IsHitting`)) (`self.IsDiving`))))
          (`SceneComponent.K2_AddLocalRotation` (`self.CapsuleComponent`) (`KismetMathLibrary.MakeRotator` 0.0 0.0 (* (* (`self.DeltaSeconds`) (`self.TurnSpeed`)) 45.0)) false false))
        ;;[1 1 1] If ChangeTime>NextChangeTime then change the behavior.
        (if (> (`self.ChangeTime`) (`self.NextChangeTime`))
          (set `self.ChangeTime` 0.0)
          ;;[1 1 1] Stop all behaviors.
          (set `self.IsGrooming` false)
          (set `self.IsAttacking` false)
          (set `self.IsHitting` false)
          (set `self.IsStandFlap` false)
          (set `self.IsSitdown` false)
          (set `self.RunningStart` false)
          (set `self.IsEating` false)
          (set `self.IsCourtship` false)
          (set `self.IsDiving` false)
          ;;[1 1 1] If RandomBehavior is false, set RunningStart true for take off.
          (if (`self.RandomBehavior`)
            ;;[1 1 1] Set the behavior rundomly.
            (switch `int` (`KismetMathLibrary.RandomIntegerInRange` 0 9)
              (:`Default`
                ;;[1 1 1] Set AimForwardSpeed and AimTurnSpeed to rundom value.
                (set `self.NextChangeTime` (`KismetMathLibrary.RandomFloatInRange` 0.5 1.5) :!label _label)
                (set `self.InitialForwardSpeed` (`self.ForwardSpeed`))
                (set `self.AimForwardSpeed` (`KismetMathLibrary.RandomFloatInRange` -0.5 2.0))
                (set `self.InitialTurnSpeed` (`self.TurnSpeed`))
                (set `self.AimTurnSpeed` (`KismetMathLibrary.RandomFloatInRange` -1.0 1.0)))
              (:`0`
                (set `self.IsAttacking` true)
                (goto _label))
              (:`1`
                (set `self.IsGrooming` true)
                ;;[1 1 1] Set AimForwardSpeed and AimTurnSpeed to 0.
                (set `self.NextChangeTime` (`KismetMathLibrary.RandomFloatInRange` 2.0 3.0) :!label _label_2)
                (set `self.InitialForwardSpeed` (`self.ForwardSpeed`))
                (set `self.AimForwardSpeed` 0.0)
                (set `self.InitialTurnSpeed` (`self.TurnSpeed`))
                (set `self.AimTurnSpeed` 0.0))
              (:`2`
                (set `self.IsStandFlap` true)
                (goto _label_2))
              (:`3`
                (set `self.IsSitdown` true)
                (goto _label_2))
              (:`4`
                (set `self.IsEating` true)
                (goto _label_2))
              (:`5`
                (set `self.IsCourtship` true)
                (goto _label_2))
              (:`6`
                (set `self.RunningStart` true :!label _label_3)
                ;;[1 1 1] Begin running for takeoff.
                (set `self.InitialForwardSpeed` (`self.ForwardSpeed`))
                (set `self.AimForwardSpeed` 2.0)
                (set `self.InitialTurnSpeed` (`self.TurnSpeed`))
                (set `self.AimTurnSpeed` 0.0)
                (set `self.IsRunning` true)
                (set `self.RunningStartTime` 0.0))
              (:`7`
                (set `self.IsDiving` true)
                (goto _label_2)))
            (else
              (goto _label_3)))
          (else
            ;;[1 1 1] Increment the ChangeTime.
            (bind _output_get (set `self.ChangeTime` (+ (`self.ChangeTime`) (`GameplayStatics.GetWorldDeltaSeconds`))))
            ;;[1 1 1] Change the Forward Speed.
            (set `self.ForwardSpeed` (`KismetMathLibrary.Lerp` (`self.InitialForwardSpeed`) (`self.AimForwardSpeed`) (`KismetMathLibrary.FClamp` _output_get)))
            ;;[1 1 1] Change the TurnSpeed.
            (set `self.TurnSpeed` (`KismetMathLibrary.Lerp` (`self.InitialTurnSpeed`) (`self.AimForwardSpeed`) (`KismetMathLibrary.FClamp` _output_get)))))))
    (else
      ;[1 1 1] IsFlying?
      (if (`NavMovementComponent.IsFlying` (`self.CharacterMovement`))
        ;[1 1 1] Turn the Swan.
        (`SceneComponent.K2_AddLocalRotation` (`self.CapsuleComponent`) (`KismetMathLibrary.MakeRotator` 0.0 0.0 (* (* (`self.DeltaSeconds`) (`self.TurnSpeed`)) 45.0)) false false)
        ;[1 1 1] Is Rising true?
        (if (`self.Rising`)
          ;[1 1 1] Movement mode is Flying and Rising is true.
          ;;[1 1 1] Determine whether the distance to the ground is greater than MaxFlyHeight.
          (bind _outhit (`KismetSystemLibrary.LineTraceSingle` _returnvalue_2 (+ _returnvalue_2 (* (* (`SceneComponent.GetUpVector` (`self.Mesh`)) -2.0) (`self.MaxFlyHeight`))) "TraceTypeQuery1"))
          (if (> (- (.z _returnvalue_2) (.z (`.Location` (`GameplayStatics.BreakHitResult` _outhit)))) (`self.MaxFlyHeight`))
            (set `self.Rising` false)
            (set `self.IsUpAccelerating` false))
          (else
            ;[1 1 1] Is TryLandingToLand True?
            (if (`self.IsTryLandingToLand`)
              ;[1 1 1] Decelerate when IsTryLandingToLand is true.
              (set `self.AimFlyUpAcceleration` -5.0)
              (set `self.AimFlyForwardAcceleration` -5.0)
              (set `self.AimTurnSpeed` 0.0)
              (set `self.RandomBehavior` true)
              (else
                ;[1 1 1] Movement mode is Flying and IsTryingToLand is false.
                ;;[1 1 1] Calculate AimFlyUpAcceleration
                (bind _outhit_2 (`KismetSystemLibrary.LineTraceSingle` _returnvalue (+ _returnvalue (* (* (`SceneComponent.GetUpVector` (`self.Mesh`)) -2.0) (`self.MaxFlyHeight`))) "TraceTypeQuery1"))
                (if (> (- (.z _returnvalue) (.z (`.Location` (`GameplayStatics.BreakHitResult` _outhit_2)))) (`self.MaxFlyHeight`))
                  (set `self.AimFlyUpAcceleration` -5.0)
                  (else
                    (set `self.AimFlyUpAcceleration` 5.0)))
                (set `self.AimTurnSpeed` (* (.y _returnvalue_5) 5.0))
                ;;[1 1 1] Calculate AimFlyForwardAcceleration
                ;;;[1 1 1] (Away from ObjectivePoint and FlyForwardSpeed is slow) or (Near the ObjectivePoint and FlyForwardSpeed is fast) then accelerate.
                (if (or (and (not _returnvalue_6) (not _returnvalue_3)) (and _returnvalue_6 _returnvalue_3))
                  (set `self.IsForwardAccelerating` true)
                  (set `self.AimFlyForwardAcceleration` (`KismetMathLibrary.FClamp` (.x _returnvalue_5) -5.0 5.0))
                  (else
                    (set `self.IsForwardAccelerating` false)
                    (set `self.AimFlyForwardAcceleration` 0.0)
                    (set `self.AimForwardSpeed` 0.0)))
                (if (< (+ (`KismetMathLibrary.Square` (- (.x (`SceneComponent.K2_GetComponentLocation` (`self.CapsuleComponent`))) (.x (`self.ObjectivePoint`)))) (`KismetMathLibrary.Square` (- (.y (`SceneComponent.K2_GetComponentLocation` (`self.CapsuleComponent`))) (.y (`self.ObjectivePoint`))))) 20000.0)
                  ;;[1 1 1] Change settings to try landing.
                  (set `self.IsTryLandingToLand` true)
                  (set `self.IsUpAccelerating` false)
                  (set `self.IsForwardAccelerating` false)
                  (set `self.ForwardSpeed` 0.5)
                  (set `self.AimForwardSpeed` 0.5)
                  (set `self.ChangeTime` 0.0)
                  (set `self.NextChangeTime` (`KismetMathLibrary.RandomFloatInRange` 8.0 11.0)))))))))))

(event `self.CapsuleComponent.OnComponentHit`
  (params (HitComponent :type "PrimitiveComponent Object Reference") (OtherActor :type "Actor Object Reference") (OtherComp :type "PrimitiveComponent Object Reference") (NormalImpulse :type "Vector Structure") (Hit :type "HitResult Structure (by ref)"))
  ;[1 1 1] Hit the other swan?
  (cast `/Game/CompleteAnimals/Birds/Swan/Blueprints/BP_SwanCharacter` OtherActor
    (:`then`
      ;[1 1 1] IsWalking?
      (if (`CharacterMovementComponent.IsWalking` (`self.CharacterMovement`))
        ;[1 1 1] When Hit other Swan at the ground.
        (switch `int` (`KismetMathLibrary.RandomIntegerInRange` 0 5)
          (:`0`
            (set `self.IsAttacking` true))
          (:`1`
            (set `self.IsHitting` true))
          (:`2`
            (`self.Jump`)))
        (else
          ;[1 1 1] IsFlying?
          (if (`NavMovementComponent.IsFlying` (`self.CharacterMovement`)) :!label _label_4
            ;[1 1 1] Changing to setting to try landing.
            (set `self.IsTryLandingToLand` true)
            (set `self.IsUpAccelerating` false)
            (set `self.IsForwardAccelerating` false)
            (set `self.ForwardSpeed` 0.5)
            (set `self.AimForwardSpeed` 0.5)
            (set `self.ChangeTime` 0.0)
            (set `self.NextChangeTime` (`KismetMathLibrary.RandomFloatInRange` 8.0 11.0))))))
    (:`CastFailed`
      (goto _label_4))))

(fn `SetObjectivePoint`
  (bind _landingpoints (`self.LandingPoints`))
  ;[1 1 1] Is there landing point?
  (if (!= (`KismetArrayLibrary.Array_Length` (`self.LandingPoints`)) 0)
    ;[1 1 1] Random select LandingPoint from LandingPoints.
    (bind _output_get (set `self.LandingPoint` (`|GetArrayItem` _landingpoints (`KismetMathLibrary.RandomIntegerInRange` 0 (- (`KismetArrayLibrary.Array_Length` _landingpoints) 1)))))
    (set `self.ObjectivePoint` (`SceneComponent.K2_GetComponentLocation` (`/Game/CompleteAnimals/Birds/Swan/Blueprints/BP_SwanLandingPoint.DefaultSceneRoot` _output_get)))))

(fn `UserConstructionScript`
  (`parent.UserConstructionScript`)
  ;[1 1 1] Set the NextChangeTime rundomly.
  (set `self.NextChangeTime` (`KismetMathLibrary.RandomFloatInRange` 3.0 5.0)))
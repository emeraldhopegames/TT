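; Swan character that walks, swims and flies, with construction-time scaling of trace, foot offset and speed factors.
; Tick eases speeds toward targets, then moves the swan per movement mode, using a hand-rolled acceleration model for flight.
; Soar requires running before takeoff; downward traces, hits, overlaps and water-volume changes switch it to walking or swimming.
; Line traces compute smoothed foot IK locations and ground-aligned rotations outside swimming.
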(event `self.ReceiveTick`
  (params (DeltaSeconds :type "Float (single-precision)"))
  (bind _returnvalue (* (`SceneComponent.GetUpVector` (`self.CapsuleComponent`)) (`self.InputScaleFactor`)))
  (bind _returnvalue_2 (* (* (`SceneComponent.GetForwardVector` (`self.CapsuleComponent`)) (`self.ForwardSpeed`)) (`self.InputScaleFactor`)))
  ;[1 1 1] Set the DeltaSeconds for use lator.
  (set `self.DeltaSeconds` DeltaSeconds)
  ;[1 1 1] Set Forward Speed
  (set `self.ForwardSpeed` (`KismetMathLibrary.FInterpTo` (`self.ForwardSpeed`) (`self.AimForwardSpeed`) (`self.DeltaSeconds`) 5.0))
  ;[1 1 1] Set TurnSpeed
  (set `self.TurnSpeed` (`KismetMathLibrary.FInterpTo` (`self.TurnSpeed`) (`self.AimTurnSpeed`) (`self.DeltaSeconds`) 5.0))
  ;[1 1 1] IsWalking?
  (if (`CharacterMovementComponent.IsWalking` (`self.CharacterMovement`))
    ;[1 1 1] Movement mode is Walking
    (`self.FootPlacement`)
    (if (and (`self.IsLived`) (not (or (or (or (or (`self.IsCourtship`) (`self.IsSitdown`)) (`self.IsGrooming`)) (`self.IsStandFlap`)) (`self.IsEating`))))
      ;;[1 1 1] Move the Swan forward.
      (`PawnMovementComponent.AddInputVector` (`self.CharacterMovement`) (* (* (`SceneComponent.GetForwardVector` (`self.CapsuleComponent`)) (`self.ForwardSpeed`)) (`self.InputScaleFactor`)) false))
    (else
      ;[1 1 1] IsFalling?
      (if (`NavMovementComponent.IsFalling` (`self.CharacterMovement`))
        (`self.FootPlacement`)
        (else
          ;[1 1 1] IsFlying?
          (if (`NavMovementComponent.IsFlying` (`self.CharacterMovement`))
            ;[1 1 1] Movement mode is Flying
            ;;[1 1 1] Change UpSpeed by FlyUpAccelaration.
            (set `self.UpSpeed` (`KismetMathLibrary.FClamp` (+ (`self.UpSpeed`) (* (`self.FlyUpAcceleration`) (`self.DeltaSeconds`))) (`self.MaxDownSpeed`) (`self.MaxUpSpeed`)))
            ;;[1 1 1] Change FlyForwardSpeed by FlyForwardAcceleration.
            (set `self.FlyForwardSpeed` (`KismetMathLibrary.FClamp` (+ (`self.FlyForwardSpeed`) (* (`self.FlyForwardAcceleration`) (`self.DeltaSeconds`))) 0.0 (`self.MaxFlySpeed`)))
            ;;[1 1 1] Change FlyUpAcceleration by AimFlyUpAcceleration.
            (set `self.FlyUpAcceleration` (`KismetMathLibrary.FInterpTo` (`self.FlyUpAcceleration`) (`self.AimFlyUpAcceleration`) (`self.DeltaSeconds`) 5.0))
            ;;[1 1 1] Change FlyForwardAcceleration by AimFlyForwardAcceleration.
            (set `self.FlyForwardAcceleration` (`KismetMathLibrary.FInterpTo` (`self.FlyForwardAcceleration`) (`self.AimFlyForwardAcceleration`) (`self.DeltaSeconds`) 5.0))
            ;;[1 1 1] Accelerating?
            (if (not (or (`self.IsForwardAccelerating`) (`self.IsUpAccelerating`)))
              ;;[1 1 1] Calculate AimFlyUpAccleration and AimFlyForwardAcceleration from FlyForwardSpeed.
              (set `self.AimFlyUpAcceleration` (* (- (`self.FlyForwardSpeed`) (`self.MeanForwardSpeed`)) 0.03))
              (set `self.AimFlyForwardAcceleration` (`KismetMathLibrary.FClamp` (* (- (`self.FlyForwardSpeed`) (`self.MeanForwardSpeed`)) -0.1) -10.0 0.0)))
            ;;[1 1 1] Move the Swan by FlyForwardSpeed and FlyUpSpeed.
            (`self.K2_AddActorLocalOffset` (* (`KismetMathLibrary.MakeVector` (* (`self.FlyForwardSpeed`) (`self.DeltaSeconds`)) 0.0 (* (`self.UpSpeed`) (`self.DeltaSeconds`))) (`self.FlySpeedScaleFactor`)) true)
            (`self.FootPlacement`)
            (if (and (<= (`self.UpSpeed`) 0.0) (not (or (`self.IsForwardAccelerating`) (`self.IsUpAccelerating`))))
              (set `self.IsSoaring` false)
              ;;[1 1 1] Determine whether Swan is on the ground.
              (bind (_outhit _returnvalue_3) (`KismetSystemLibrary.LineTraceSingle` (`SceneComponent.K2_GetComponentLocation` (`self.CapsuleComponent`)) (`KismetMathLibrary.MakeVector` (.x (`SceneComponent.K2_GetComponentLocation` (`self.CapsuleComponent`))) (.y (`SceneComponent.K2_GetComponentLocation` (`self.CapsuleComponent`))) (- (.z (`SceneComponent.K2_GetComponentLocation` (`self.CapsuleComponent`))) (`self.IKTraceDistance`))) "TraceTypeQuery1"))
              (if _returnvalue_3
                ;;[1 1 1] Landing on land or water
                (if (`PhysicsVolume.bWaterVolume` (`SceneComponent.GetPhysicsVolume` (`.HitComponent` (`GameplayStatics.BreakHitResult` _outhit))))
                  (`self.LandingOnWater`)
                  (else
                    (`self.LandingOnLand`)))))
            (else
              ;[1 1 1] IsSwimming?
              (if (`NavMovementComponent.IsSwimming` (`self.CharacterMovement`))
                ;[1 1 1] Movement mode is Swimming
                (if (`self.IsLived`)
                  ;;[1 1 1] If Running.
                  (if (`self.IsRunning`)
                    (`PawnMovementComponent.AddInputVector` (`self.CharacterMovement`) (+ (* _returnvalue_2 15.0) _returnvalue) false)
                    (else
                      ;;[1 1 1] If IsLived and not Running.
                      (`PawnMovementComponent.AddInputVector` (`self.CharacterMovement`) (+ _returnvalue_2 _returnvalue) false)))
                  (else
                    ;;[1 1 1] If not IsLived.
                    (`PawnMovementComponent.AddInputVector` (`self.CharacterMovement`) _returnvalue false)))))))))))

(event `self.CapsuleComponent.PhysicsVolumeChangedDelegate`
  (params (NewVolume :type "PhysicsVolume Object Reference"))
  ;[1 1 1] Enter Water Volume?
  (if (`PhysicsVolume.bWaterVolume` NewVolume)
    ;[1 1 1] Set Movement Mode Swimming
    (`CharacterMovementComponent.SetMovementMode` (`self.CharacterMovement`) "MOVE_Swimming" 0 :!label _label)
    (`PrimitiveComponent.SetEnableGravity` (`self.CapsuleComponent`) false)
    (`PrimitiveComponent.SetSimulatePhysics` (`self.CapsuleComponent`) false)
    (set `self.IsSoaring` false)
    (set `self.IsRunning` false)
    (set `self.AimForwardSpeed` 0.0)
    (set `self.ForwardSpeed` (* (`self.FlyForwardSpeed`) 0.1))
    (else
      (if (not (or (`self.IsForwardAccelerating`) (`self.IsUpAccelerating`))) :!label _label_2
        ;[1 1 1] Set Movement mode Walking
        (`CharacterMovementComponent.SetMovementMode` (`self.CharacterMovement`) "MOVE_Walking" 0)
        (`PrimitiveComponent.SetEnableGravity` (`self.CapsuleComponent`) true)
        (`PrimitiveComponent.SetSimulatePhysics` (`self.CapsuleComponent`) false)
        (set `self.IsSoaring` false)
        (set `self.IsRunning` false)
        (set `self.IKInterpSpeed` 30.0)
        (set `self.ForwardSpeed` 0.0)
        (set `self.AimForwardSpeed` 0.0)))))

(event `self.CapsuleComponent.OnComponentBeginOverlap`
  (params (OverlappedComponent :type "PrimitiveComponent Object Reference") (OtherActor :type "Actor Object Reference") (OtherComp :type "PrimitiveComponent Object Reference") (OtherBodyIndex :type Integer) (bFromSweep :type Boolean) (SweepResult :type "HitResult Structure (by ref)"))
  ;[1 1 1] Enter Water Volume?
  (if (`PhysicsVolume.bWaterVolume` (`SceneComponent.GetPhysicsVolume` OverlappedComponent))
    (goto _label)
    (else
      (goto _label_2))))

(event `self.CapsuleComponent.OnComponentHit`
  (params (HitComponent :type "PrimitiveComponent Object Reference") (OtherActor :type "Actor Object Reference") (OtherComp :type "PrimitiveComponent Object Reference") (NormalImpulse :type "Vector Structure") (Hit :type "HitResult Structure (by ref)"))
  ;[1 1 1] Enter Water Volume?
  (if (`PhysicsVolume.bWaterVolume` (`SceneComponent.GetPhysicsVolume` HitComponent))
    (goto _label)
    (else
      (goto _label_2))))

(fn `CanJumpInternal`
  (returns (ReturnValue :type Boolean))
  (return (and (and (and (and (and (and (and (and (`CharacterMovementComponent.IsWalking` (`self.CharacterMovement`)) (`self.IsLived`)) (not (`self.IsAttacking`))) (not (`self.IsHitting`))) (not (`self.IsGrooming`))) (not (`self.IsSitdown`))) (not (`self.IsStandFlap`))) (not (`self.IsEating`))) (not (`self.IsCourtship`)))))

(fn `FootPlacement`
  ;[1 1 1] Calculate the L_Tarsus_2EffectorLoc's Location and L_Tarsus_2's rotation.
  (bind (_legikeffectorloc _footrot) (`self.TraceIKEffector` (`self.L_Tarsus_2`) (`self.IKTraceDistance`) (`self.IKHeightOffset`)))
  ;[1 1 1] Set the left foot rotation.
  (set `self.L_Tarsus_2Rot` (`KismetMathLibrary.RInterpTo` (`self.L_Tarsus_2Rot`) _footrot (`GameplayStatics.GetWorldDeltaSeconds`) (`self.FootRotInterpSpeed`)))
  ;[1 1 1] Set the left foot IK effecter location.
  (set `self.L_Tarsus_2EffectorLoc` (`KismetMathLibrary.VInterpTo` (`self.L_Tarsus_2EffectorLoc`) _legikeffectorloc (`GameplayStatics.GetWorldDeltaSeconds`) (`self.IKInterpSpeed`)))
  ;[1 1 1] Calculate the R_Tarsus_2EffectorLoc's Location and R_Tarsus_2's rotation.
  (bind (_legikeffectorloc_2 _footrot_2) (`self.TraceIKEffector` (`self.R_Tarsus_2`) (`self.IKTraceDistance`) (`self.IKHeightOffset`)))
  ;[1 1 1] Set the right foot rotation.
  (set `self.R_Tarsus_2Rot` (`KismetMathLibrary.RInterpTo` (`self.R_Tarsus_2Rot`) _footrot_2 (`GameplayStatics.GetWorldDeltaSeconds`) (`self.FootRotInterpSpeed`)))
  ;[1 1 1] Set the right foot effector location.
  (set `self.R_Tarsus_2EffectorLoc` (`KismetMathLibrary.VInterpTo` (`self.R_Tarsus_2EffectorLoc`) _legikeffectorloc_2 (`GameplayStatics.GetWorldDeltaSeconds`) (`self.IKInterpSpeed`)))
  (return))

(fn `LandingOnLand`
  ;[1 1 1] Change the settings for landing
  (`CharacterMovementComponent.SetMovementMode` (`self.CharacterMovement`) "MOVE_Walking" 0)
  (`PrimitiveComponent.SetEnableGravity` (`self.CapsuleComponent`) true)
  (`PrimitiveComponent.SetSimulatePhysics` (`self.CapsuleComponent`) false)
  ;[1 1 1] Initialize variables for stop the walking
  (set `self.IsSoaring` false)
  (set `self.IsRunning` false)
  (set `self.IKInterpSpeed` 30.0)
  (set `self.ForwardSpeed` 0.0)
  (set `self.AimForwardSpeed` 0.0))

(fn `LandingOnWater`
  ;[1 1 1] Change the settings for Water movement
  (`CharacterMovementComponent.SetMovementMode` (`self.CharacterMovement`) "MOVE_Swimming" 0)
  (`PrimitiveComponent.SetEnableGravity` (`self.CapsuleComponent`) true)
  (`PrimitiveComponent.SetSimulatePhysics` (`self.CapsuleComponent`) false)
  ;[1 1 1] Initialize the variables for set the Swimming spped
  (set `self.IsSoaring` false)
  (set `self.IsRunning` false)
  (set `self.IKInterpSpeed` 30.0)
  (set `self.ForwardSpeed` (`KismetMathLibrary.FClamp` (* (`self.FlyForwardSpeed`) 0.04)))
  (set `self.AimForwardSpeed` 0.0))

(fn `Soar`
  ;[1 1 1] Can soar?
  (if (and (and (and (or (`CharacterMovementComponent.IsWalking` (`self.CharacterMovement`)) (`NavMovementComponent.IsSwimming` (`self.CharacterMovement`))) (and (`self.IsRunning`) (> (`self.ForwardSpeed`) 0.5))) (`self.IsLived`)) (not (or (or (or (or (or (or (or (`self.IsCourtship`) (`self.IsSitdown`)) (`self.IsGrooming`)) (`self.IsStandFlap`)) (`self.IsEating`)) (`self.IsAttacking`)) (`self.IsHitting`)) (`self.IsDiving`))))
    ;[1 1 1] Change the settings for flight
    (set `self.IsSoaring` true)
    (`CharacterMovementComponent.SetMovementMode` (`self.CharacterMovement`) "MOVE_Flying" 0)
    (`PrimitiveComponent.SetEnableGravity` (`self.CapsuleComponent`) false)
    (`PrimitiveComponent.SetSimulatePhysics` (`self.CapsuleComponent`) true)
    ;[1 1 1] Initialize variables for flight
    (set `self.FlyForwardSpeed` 8.0)
    (set `self.UpSpeed` 1.5)
    (set `self.FlyForwardAcceleration` 5.0)
    (set `self.FlyUpAcceleration` 1.0)
    (set `self.AimFlyUpAcceleration` 0.0)
    (set `self.AimFlyForwardAcceleration` 10.0)
    (set `self.IKInterpSpeed` 50.0)
    (set `self.IsAttacking` false)
    (set `self.IsHitting` false)))

(fn `TraceIKEffector`
  (params (FootName :type Name) (TraceDistance :type "Float (double-precision)" :default 50.0) (HeightOffset :type "Float (double-precision)" :default 10.0))
  (returns (LegIKEffectorLoc :type "Vector Structure") (FootRot :type "Rotator Structure"))
  (locals (GroundNormal :type "Vector Structure") (TraceFootName :type Name) (DoesReachThaGround :type Boolean) (InitialFootLocation :type "Vector Structure") (InitialFootRotation :type "Rotator Structure"))
  (bind _x (.x (`local.InitialFootLocation`)))
  (bind _y (.y (`local.InitialFootLocation`)))
  (bind _z (.z (`self.K2_GetActorLocation`)))
  (bind (_x_2 _y_2 _z_2) (`KismetMathLibrary.BreakRotIntoAxes` (`local.InitialFootRotation`)))
  (bind _returnvalue (`KismetMathLibrary.Cross_VectorVector` _y_2 (`local.GroundNormal`)))
  (bind _returnvalue_2 (`KismetMathLibrary.DegAsin` (`KismetMathLibrary.VSize` _returnvalue)))
  ;[1 1 1] Set the InitialFootLocation and InitialFootRotation  for use later.
  (set `local.InitialFootLocation` (`SceneComponent.GetSocketLocation` (`self.Mesh`) FootName))
  (set `local.InitialFootRotation` (`SceneComponent.GetSocketRotation` (`self.Mesh`) FootName))
  ;[1 1 1] Calculate the location of foot.
  ;;[1 1 1] Trace from foot location to the location lowered by the TraceDistance from the location of the foot
  (bind (_outhit _returnvalue_3) (`KismetSystemLibrary.LineTraceSingle` (`KismetMathLibrary.MakeVector` _x _y _z) (`KismetMathLibrary.MakeVector` _x _y (- _z TraceDistance)) "TraceTypeQuery1" true))
  ;;[1 1 1] Set the DoesReachTheGround and GroundNormal  for use later.
  (set `local.DoesReachThaGround` _returnvalue_3)
  (bind (_bblockinghit _binitialoverlap _time _distance _location _impactpoint _normal) (`GameplayStatics.BreakHitResult` _outhit))
  (set `local.GroundNormal` _normal)
  (return (`KismetMathLibrary.SelectVector` (`KismetMathLibrary.MakeVector` (.x _location) (.y _location) (+ (.z _location) HeightOffset)) (`local.InitialFootLocation`) (`local.DoesReachThaGround`)) (`KismetMathLibrary.SelectRotator` (`KismetMathLibrary.MakeRotationFromAxes` (`KismetMathLibrary.RotateAngleAxis` _x_2 _returnvalue_2 _returnvalue) (`local.GroundNormal`) (`KismetMathLibrary.RotateAngleAxis` _z_2 _returnvalue_2 _returnvalue)) (`local.InitialFootRotation`) (`local.DoesReachThaGround`))))

(fn `UserConstructionScript`
  (bind _scale (`self.Scale`))
  (set `self.Scale` (.z (.scale (`self.GetTransform`))))
  ;[1 1 1] Set the scale dependent variables.
  (set `self.IKTraceDistance` (* (* (`CapsuleComponent.CapsuleHalfHeight` (`self.CapsuleComponent`)) 3.0) _scale))
  (set `self.IKHeightOffset` (* _scale (`self.IKHeightOffset`)))
  (set `self.InputScaleFactor` (* (`self.InputScaleFactor`) _scale))
  (set `self.FlySpeedScaleFactor` (* (`self.FlySpeedScaleFactor`) _scale)))
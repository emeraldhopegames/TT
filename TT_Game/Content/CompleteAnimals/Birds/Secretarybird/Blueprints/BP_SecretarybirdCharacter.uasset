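; Secretarybird character that walks, soars into flight and lands automatically when a downward trace finds ground.
; Tick eases speeds toward aim values, feeding movement input on foot or integrating accelerations into swept local offsets in flight.
; Soar switches to Flying with capsule physics on and gravity off; landing reverses this and clears action flags, which also block walking.
; FootPlacement traces under each foot and interpolates its rotation toward the ground normal.
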(event `self.ReceiveTick`
  (params (DeltaSeconds :type "Float (single-precision)"))
  (bind _output_get (set `self.DeltaSeconds` DeltaSeconds))
  ;[1 1 1] Set the elapsed time since starting transition to idle animation.
  (set `self.IdleTransitionTime` (+ _output_get (`self.IdleTransitionTime`)))
  ;[1 1 1] Set the elapsed time since landing started.
  (set `self.LandingStartTime` (+ (`self.DeltaSeconds`) (`self.LandingStartTime`)))
  ;[1 1 1] Set Forward Speed
  (set `self.ForwardSpeed` (`KismetMathLibrary.FInterpTo` (`self.ForwardSpeed`) (`self.AimForwardSpeed`) (`self.DeltaSeconds`) 5.0))
  ;[1 1 1] Set TurnSpeed
  (set `self.TurnSpeed` (`KismetMathLibrary.FInterpTo` (`self.TurnSpeed`) (`self.AimTurnSpeed`) (`self.DeltaSeconds`) 5.0))
  ;[1 1 1] IsWalking?
  (if (`CharacterMovementComponent.IsWalking` (`self.CharacterMovement`))
    ;[1 1 1] Movement mode is Walking
    (`self.FootPlacement`)
    (bind _isdoing (`self.IsDoingSomething`))
    (if (and (and (not _isdoing) (`self.IsLived`)) (>= (`self.LandingStartTime`) 2.0))
      (`PawnMovementComponent.AddInputVector` (`self.CharacterMovement`) (* (* (`SceneComponent.GetForwardVector` (`self.CapsuleComponent`)) (`self.ForwardSpeed`)) (`self.InputScaleFactor`)) false))
    (else
      ;[1 1 1] IsFalling?
      (if (`NavMovementComponent.IsFalling` (`self.CharacterMovement`))
        (`self.FootPlacement`)
        (else
          ;[1 1 1] IsFlying?
          (if (`NavMovementComponent.IsFlying` (`self.CharacterMovement`))
            ;[1 1 1] Movement mode is Flying.
            ;;[1 1 1] Change UpSpeed by FlyUpAccelaration.
            (set `self.UpSpeed` (`KismetMathLibrary.FClamp` (+ (`self.UpSpeed`) (* (`self.FlyUpAcceleration`) (`self.DeltaSeconds`))) (`self.MaxDownSpeed`) (`self.MaxUpSpeed`)))
            ;;[1 1 1] Change FlyForwardSpeed by FlyForwardAcceleration.
            (set `self.FlyForwardSpeed` (`KismetMathLibrary.FClamp` (+ (`self.FlyForwardSpeed`) (* (`self.FlyForwardAcceleration`) (`self.DeltaSeconds`))) 0.0 (`self.MaxFlySpeed`)))
            ;;[1 1 1] Change FlyUpAcceleration by AimFlyUpAcceleration.
            (set `self.FlyUpAcceleration` (`KismetMathLibrary.FInterpTo` (`self.FlyUpAcceleration`) (`self.AimFlyUpAcceleration`) (`self.DeltaSeconds`) 5.0))
            ;;[1 1 1] Change FlyForwardAcceleration by AimFlyForwardAcceleration.
            (set `self.FlyForwardAcceleration` (`KismetMathLibrary.FInterpTo` (`self.FlyForwardAcceleration`) (`self.AimFlyForwardAcceleration`) (`self.DeltaSeconds`) 5.0))
            (if (not (or (`self.ForwardAccelerationChange`) (`self.UpAccelerationChange`)))
              ;;[1 1 1] Calculate AimFlyUpAccleration and AimFlyForwardAcceleration from FlyForwardSpeed.
              (set `self.AimFlyUpAcceleration` (* (- (`self.MeanForwardSpeed`) (`self.FlyForwardSpeed`)) -0.1))
              (set `self.AimFlyForwardAcceleration` (* (`self.FlyForwardSpeed`) -0.1)))
            ;;[1 1 1] Move the Secretarybird by FlyForwardSpeed and FlyUpSpeed.
            (`self.K2_AddActorLocalOffset` (* (`KismetMathLibrary.MakeVector` (* (`self.FlyForwardSpeed`) (`self.DeltaSeconds`)) 0.0 (* (`self.UpSpeed`) (`self.DeltaSeconds`))) (`self.FlySpeedScaleFactor`)) true)
            (`self.FootPlacement`)
            (bind _output_get_2 (set `self.SoaringStartTime` (+ (`self.SoaringStartTime`) (`self.DeltaSeconds`))))
            (if (> _output_get_2 1.0)
              (set `self.IsSoaring` false)
              ;;[1 1 1] Determining whether the Secretqarybird is close to the ground or not.
              (bind (_outhit _returnvalue) (`KismetSystemLibrary.LineTraceSingle` (`SceneComponent.K2_GetComponentLocation` (`self.CapsuleComponent`)) (`KismetMathLibrary.MakeVector` (.x (`SceneComponent.K2_GetComponentLocation` (`self.CapsuleComponent`))) (.y (`SceneComponent.K2_GetComponentLocation` (`self.CapsuleComponent`))) (- (.z (`SceneComponent.K2_GetComponentLocation` (`self.CapsuleComponent`))) (`self.IKTraceDistance`))) "TraceTypeQuery1"))
              (if _returnvalue
                ;;[1 1 1] Landing
                (`CharacterMovementComponent.SetMovementMode` (`self.CharacterMovement`) "MOVE_Walking" 0)
                (`PrimitiveComponent.SetEnableGravity` (`self.CapsuleComponent`) true)
                (`PrimitiveComponent.SetSimulatePhysics` (`self.CapsuleComponent`) false)
                (set `self.IKInterpSpeed` 10.0)
                (`self.BehaviorOff`)
                (set `self.AimForwardSpeed` 0.0)
                (set `self.AimTurnSpeed` 0.0)
                (set `self.ForwardSpeed` 0.0)
                (set `self.TurnSpeed` 0.0)
                (set `self.LandingStartTime` 0.0)))))))))

(fn `BehaviorOff`
  ;[1 1 1] Turn off all actions.
  (set `self.IsAttacking` false)
  (set `self.IsHitting` false)
  (set `self.IsEating` false)
  (set `self.IsSleeping` false))

(fn `CalculateFootAngle`
  (params (FootName :type Name) (TraceDistance :type "Float (double-precision)" :default 50.0))
  (returns (FootRot :type "Rotator Structure"))
  (locals (GroundNormal :type "Vector Structure") (InitialFootRotation :type "Rotator Structure"))
  (bind _z (.z (`self.K2_GetActorLocation`)))
  (bind (_x _y _z_2) (`KismetMathLibrary.BreakRotIntoAxes` (`local.InitialFootRotation`)))
  (bind _x_2 (.x (`SceneComponent.GetSocketLocation` (`self.Mesh`) FootName)))
  (bind _y_2 (.y (`SceneComponent.GetSocketLocation` (`self.Mesh`) FootName)))
  (bind _returnvalue (`KismetMathLibrary.Cross_VectorVector` _y (`local.GroundNormal`)))
  (bind _returnvalue_2 (`KismetMathLibrary.DegAsin` (`KismetMathLibrary.VSize` _returnvalue)))
  ;[1 1 1] Set the InitialFootRotation.
  (set `local.InitialFootRotation` (`SceneComponent.GetSocketRotation` (`self.Mesh`) FootName))
  ;[1 1 1] Calculate the location of foot.
  ;;[1 1 1] Trace from foot location to the location lowered by the TraceDistance from the location of the foot
  (bind (_outhit _returnvalue_3) (`KismetSystemLibrary.LineTraceSingle` (`KismetMathLibrary.MakeVector` _x_2 _y_2 _z) (`KismetMathLibrary.MakeVector` _x_2 _y_2 (- _z TraceDistance)) "TraceTypeQuery1" true))
  (set `local.GroundNormal` (`.Normal` (`GameplayStatics.BreakHitResult` _outhit)))
  (return (`KismetMathLibrary.SelectRotator` (`KismetMathLibrary.MakeRotationFromAxes` (`KismetMathLibrary.RotateAngleAxis` _x _returnvalue_2 _returnvalue) (`local.GroundNormal`) (`KismetMathLibrary.RotateAngleAxis` _z_2 _returnvalue_2 _returnvalue)) (`local.InitialFootRotation`) _returnvalue_3)))

(fn `CanJumpInternal`
  (returns (ReturnValue :type Boolean))
  (return (and (and (and (and (and (`CharacterMovementComponent.IsWalking` (`self.CharacterMovement`)) (not (`self.IsAttacking`))) (not (`self.IsHitting`))) (not (`self.IsEating`))) (`self.IsLived`)) (not (`self.IsSleeping`)))))

(fn `FootPlacement`
  ;[1 1 1] Calculate the L_Tarsus_2's rotation.
  (bind _footrot (`self.CalculateFootAngle` (`self.L_Tarsus_2`) (`self.IKTraceDistance`)))
  ;[1 1 1] Set the left foot rotation.
  (set `self.L_Tarsus_2Rot` (`KismetMathLibrary.RInterpTo` (`self.L_Tarsus_2Rot`) _footrot (`GameplayStatics.GetWorldDeltaSeconds`) (`self.FootRotInterpSpeed`)))
  ;[1 1 1] Calculate the R_Tarsus_2's rotation.
  (bind _footrot_2 (`self.CalculateFootAngle` (`self.R_Tarsus_2`) (`self.IKTraceDistance`)))
  ;[1 1 1] Set the right foot rotation.
  (set `self.R_Tarsus_2Rot` (`KismetMathLibrary.RInterpTo` (`self.R_Tarsus_2Rot`) _footrot_2 (`GameplayStatics.GetWorldDeltaSeconds`) (`self.FootRotInterpSpeed`)))
  (return))

(fn `IsDoingSomething`
  (returns (IsDoing :type Boolean))
  (return (or (or (or (or (`self.IsSleeping`) (`self.IsHitting`)) (`self.IsAttacking`)) (`self.IsEating`)) (`self.IsSleeping`))))

(fn `Soar`
  ;[1 1 1] Initialize variables for flight
  (set `self.SoaringStartTime` 0.0)
  (set `self.FlyForwardSpeed` 10.0)
  (set `self.UpSpeed` 2.0)
  (set `self.FlyForwardAcceleration` 5.0)
  (set `self.FlyUpAcceleration` 2.0)
  (set `self.AimFlyUpAcceleration` 0.0)
  (set `self.AimFlyForwardAcceleration` 0.0)
  (set `self.IKInterpSpeed` 50.0)
  (`self.BehaviorOff`)
  ;[1 1 1] Change the settings for flight
  (`CharacterMovementComponent.SetMovementMode` (`self.CharacterMovement`) "MOVE_Flying" 0)
  (`PrimitiveComponent.SetEnableGravity` (`self.CapsuleComponent`) false)
  (`PrimitiveComponent.SetSimulatePhysics` (`self.CapsuleComponent`) true)
  (`ActorComponent.Activate` (`self.CharacterMovement`) false))

(fn `UserConstructionScript`
  (bind _scale (`self.Scale`))
  ;[1 1 1] Set the Secretarybird's scale.
  (set `self.Scale` (.z (.scale (`self.GetTransform`))))
  ;[1 1 1] Set the scale dependent variables.
  (set `self.IKTraceDistance` (* (* (`CapsuleComponent.CapsuleHalfHeight` (`self.CapsuleComponent`)) 3.0) _scale))
  (set `self.InputScaleFactor` (* (`self.InputScaleFactor`) _scale))
  (set `self.FlySpeedScaleFactor` (* (`self.FlySpeedScaleFactor`) _scale)))
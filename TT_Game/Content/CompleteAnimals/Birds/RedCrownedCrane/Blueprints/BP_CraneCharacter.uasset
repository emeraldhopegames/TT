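; Red-crowned crane character that makes a running takeoff, flies to a goal location, lands and then idles with random behaviors.
; Tick runs a four-state machine on CraneMode, easing forward, turn and climb speeds toward periodically chosen targets.
; In flight it offsets the capsule directly, using downward traces to hold height and stage glide and flap landing.
; Once grounded, it randomly walks or sets behavior flags such as eating, grooming, dancing or sleeping.
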(event `self.ReceiveTick`
  (params (DeltaSeconds :type "Float (single-precision)"))
  (bind _returnvalue (`GameplayStatics.GetWorldDeltaSeconds`))
  (bind _capsulecomponent (`self.CapsuleComponent`))
  (bind _maxwalkforwardspeed (`self.MaxWalkForwardSpeed`))
  (bind _maxwalkturnspeed (`self.MaxWalkTurnSpeed`))
  (bind _returnvalue_2 (`SceneComponent.K2_GetComponentLocation` _capsulecomponent))
  (bind _returnvalue_3 (* (`self.SpeedChangeTime`) 2.0))
  (bind _returnvalue_4 (`KismetMathLibrary.Dot_VectorVector` (`KismetMathLibrary.Normal` (- (`self.GoalLoc`) (`SceneComponent.K2_GetComponentLocation` (`self.CapsuleComponent`)))) (`SceneComponent.GetRightVector` (`self.CapsuleComponent`))))
  (switch `int` (`self.CraneMode`) ; 0:
    (:`0`
      ;[1 1 1] Set the AimTurnSpeed for Running Start
      (set `self.CraneMode` 1)
      (set `self.NextSpeedChangeTime` (`KismetMathLibrary.RandomFloatInRange` 5.0 8.0))
      (set `self.InitialForwardSpeed` (`self.ForwardSpeed`))
      (set `self.InitialTurnSpeed` (`self.TurnSpeed`))
      (set `self.AimForwardSpeed` (`self.MaxWalkForwardSpeed`))
      (if (> _returnvalue_4 0.1)
        (set `self.AimTurnSpeed` (`self.MaxWalkTurnSpeed`))
        (elif (> _returnvalue_4 -0.1)
          (set `self.AimTurnSpeed` 0.0)
          (else
            (set `self.AimTurnSpeed` (* (`self.MaxWalkTurnSpeed`) -1.0))))))
    (:`1`
      ;[1 1 1] RunningStart
      (if (< (`self.NextSpeedChangeTime`) (`self.SpeedChangeTime`))
        (set `self.CraneMode` 2)
        (`PrimitiveComponent.SetEnableGravity` (`self.CapsuleComponent`) false)
        (set `self.IsFlyingToGoal` true)
        (set `self.IsLanding` false)
        (`CharacterMovementComponent.SetMovementMode` (`self.CharacterMovement`) "MOVE_Flying" 0)
        (`PrimitiveComponent.SetSimulatePhysics` (`self.CapsuleComponent`) true)
        (else
          (set `self.SpeedChangeTime` (+ (`self.SpeedChangeTime`) (`GameplayStatics.GetWorldDeltaSeconds`)))
          (set `self.ForwardSpeed` (`KismetMathLibrary.Lerp` (`self.InitialForwardSpeed`) (`self.AimForwardSpeed`) (`KismetMathLibrary.FClamp` (* (/ (`self.SpeedChangeTime`) (`self.NextSpeedChangeTime`)) 2.0))))
          (set `self.TurnSpeed` (`KismetMathLibrary.Lerp` (`self.InitialTurnSpeed`) (`self.AimTurnSpeed`) (/ (`self.SpeedChangeTime`) (`self.NextSpeedChangeTime`)))))))
    (:`2`
      ;[1 1 1] FlyToGoal
      ;;[1 1 1] Forward and Turn moving
      (`SceneComponent.K2_AddLocalOffset` (`self.CapsuleComponent`) (`KismetMathLibrary.MakeVector` (* (`self.ForwardSpeed`) _returnvalue) 0.0 (* (`self.UpSpeed`) _returnvalue)) false false)
      (`SceneComponent.K2_AddLocalRotation` (`self.CapsuleComponent`) (`KismetMathLibrary.MakeRotator` 0.0 0.0 (* _returnvalue (`self.TurnSpeed`))) false false)
      (if (< (+ (`KismetMathLibrary.Square` (- (.x (`SceneComponent.K2_GetComponentLocation` (`self.CapsuleComponent`))) (.x (`self.GoalLoc`)))) (`KismetMathLibrary.Square` (- (.y (`SceneComponent.K2_GetComponentLocation` (`self.CapsuleComponent`))) (.y (`self.GoalLoc`))))) 20000.0)
        (set `self.IsFlyingToGoal` false)
        (set `self.IsTryToLandingGlide` true))
      (if (> (`self.SpeedChangeTime`) (`self.NextSpeedChangeTime`))
        (set `self.NextSpeedChangeTime` 0.5)
        (set `self.SpeedChangeTime` 0.0)
        ;;[1 1 1] Set AimTurnSpeed
        (set `self.InitialForwardSpeed` (`self.ForwardSpeed`))
        (set `self.InitialUpSpeed` (`self.UpSpeed`))
        (set `self.InitialTurnSpeed` (`self.TurnSpeed`))
        (set `self.AimForwardSpeed` (`KismetMathLibrary.FClamp` (`KismetMathLibrary.VSizeSquared` (- (`self.GoalLoc`) (`SceneComponent.K2_GetComponentLocation` (`self.CapsuleComponent`)))) 0.0 (`self.MaxFlyForwardSpeed`)))
        (if (< (.x (`KismetMathLibrary.Normal` (`KismetMathLibrary.InverseTransformLocation` (`SceneComponent.K2_GetComponentToWorld` (`self.CapsuleComponent`)) (`self.GoalLoc`)))) 0.0)
          (set `self.AimTurnSpeed` (* (.y (`KismetMathLibrary.Normal` (`KismetMathLibrary.InverseTransformLocation` (`SceneComponent.K2_GetComponentToWorld` (`self.CapsuleComponent`)) (`self.GoalLoc`)))) (`self.MaxFlyTurnSpeed`))))
        ;;[1 1 1] Calculate flying height
        (bind _outhit (`KismetSystemLibrary.LineTraceSingleForObjects` _returnvalue_2 (+ _returnvalue_2 (* (`SceneComponent.GetUpVector` _capsulecomponent) (* (`self.MaxFlyHeight`) -1.0))) (`|MakeArray` "ObjectTypeQuery1" :!type "EObjectTypeQuery Enum")))
        ;[1 1 1] Mode change corresponding to the height
        (if (`self.IsTryToLandingGlide`)
          (bind _returnvalue_5 (- (.z _returnvalue_2) (.z (`.Location` (`GameplayStatics.BreakHitResult` _outhit)))))
          (if (not (> _returnvalue_5 (* (`self.MaxFlyHeight`) 0.25)))
            (set `self.IsTryToLandingFlap` true)
            (set `self.IsTryToLandingGlide` false))
          (set `self.AimUpSpeed` (* -1.0 (`self.MaxFlyUpSpeed`)) :!label _label)
          (elif (`self.IsTryToLandingFlap`)
            (if (> _returnvalue_5 80.0)
              (goto _label)
              (else
                (`CharacterMovementComponent.SetMovementMode` (`self.CharacterMovement`) "MOVE_Walking" 0)
                (`PrimitiveComponent.SetSimulatePhysics` (`self.CapsuleComponent`) false)
                (set `self.CraneMode` 3)
                (set `self.IsTryToLandingFlap` false)
                (set `self.IsLanding` true)))
            (else
              ;[1 1 1] Set AimUpSpeed
              (set `self.AimUpSpeed` (/ (* (- (`self.MaxFlyHeight`) (* _returnvalue_5 2.0)) (`self.MaxFlyUpSpeed`)) (`self.MaxFlyHeight`))))))
        (else
          ;;[1 1 1] Set ForwardSpeed and TurnSpeed
          (set `self.SpeedChangeTime` (+ (`self.SpeedChangeTime`) (`GameplayStatics.GetWorldDeltaSeconds`)))
          (set `self.ForwardSpeed` (`KismetMathLibrary.Lerp` (`self.InitialForwardSpeed`) (`self.AimForwardSpeed`) _returnvalue_3))
          (set `self.TurnSpeed` (`KismetMathLibrary.Lerp` (`self.InitialTurnSpeed`) (`self.AimTurnSpeed`) _returnvalue_3))
          (set `self.UpSpeed` (`KismetMathLibrary.Lerp` (`self.InitialUpSpeed`) (`self.AimUpSpeed`) _returnvalue_3)))))
    (:`3`
      ;[1 1 1] Random behavior
      (if (> (`self.SpeedChangeTime`) (`self.NextSpeedChangeTime`))
        (`self.BehaviorOff`)
        (set `self.IsLived` true)
        ;;[1 1 1] Select random behavior
        (switch `int` (`KismetMathLibrary.RandomIntegerInRange` 0 15)
          (:`Default`
            (set `self.IsWalking` true :!label _label_2)
            (set `self.InitialForwardSpeed` (`self.ForwardSpeed`))
            (set `self.InitialTurnSpeed` (`self.TurnSpeed`))
            (set `self.AimForwardSpeed` (`KismetMathLibrary.RandomFloatInRange` (* _maxwalkforwardspeed -0.5) _maxwalkforwardspeed))
            (set `self.AimTurnSpeed` (`KismetMathLibrary.RandomFloatInRange` (* _maxwalkturnspeed -1.0) _maxwalkturnspeed))
            (set `self.NextSpeedChangeTime` (`KismetMathLibrary.RandomFloatInRange` 1.0 6.0))
            (set `self.SpeedChangeTime` 0.0))
          (:`0`
            (goto _label_2))
          (:`1`
            (set `self.IsAttacking` true)
            (set `self.InitialForwardSpeed` (`self.ForwardSpeed`) :!label _label_3)
            (set `self.InitialTurnSpeed` (`self.TurnSpeed`))
            (set `self.AimForwardSpeed` 0.0)
            (set `self.AimTurnSpeed` 0.0)
            (set `self.SpeedChangeTime` 0.0)
            (set `self.NextSpeedChangeTime` (`KismetMathLibrary.RandomFloatInRange` 1.0 6.0)))
          (:`2`
            (set `self.IsLived` false)
            (goto _label_3))
          (:`3`
            (set `self.IsEating` true)
            (goto _label_3))
          (:`4`
            (set `self.IsCalling` true)
            (goto _label_3))
          (:`5`
            (set `self.IsCrouchNeck` true)
            (goto _label_3))
          (:`6`
            (set `self.IsGrooming` true)
            (goto _label_3))
          (:`7`
            (set `self.IsOneLegSleep` true)
            (goto _label_3))
          (:`8`
            (set `self.IsSleep2` true)
            (goto _label_3))
          (:`9`
            (set `self.IsUpDownDance` true)
            (goto _label_3))
          (:`10`
            (set `self.IsJumpDance` true)
            (goto _label_3))
          (:`11`
            (set `self.IsSitDown` true)
            (goto _label_3)))
        (else
          ;;[1 1 1] Forward And TurnMoving
          (set `self.SpeedChangeTime` (+ (`self.SpeedChangeTime`) (`GameplayStatics.GetWorldDeltaSeconds`)))
          (set `self.ForwardSpeed` (`KismetMathLibrary.Lerp` (`self.InitialForwardSpeed`) (`self.AimForwardSpeed`) (`KismetMathLibrary.FClamp` (* (/ (`self.SpeedChangeTime`) (`self.NextSpeedChangeTime`)) 2.0))))
          (set `self.TurnSpeed` (`KismetMathLibrary.Lerp` (`self.InitialTurnSpeed`) (`self.AimTurnSpeed`) (`KismetMathLibrary.FClamp` (* (/ (`self.SpeedChangeTime`) (`self.NextSpeedChangeTime`)) 2.0)))))))))

(fn `BehaviorOff`
  ;[1 1 1] Off the all behavior
  (set `self.IsWalking` false)
  (set `self.IsAttacking` false)
  (set `self.IsHitting` false)
  (set `self.IsEating` false)
  (set `self.IsCalling` false)
  (set `self.IsCrouchNeck` false)
  (set `self.IsGrooming` false)
  (set `self.IsOneLegSleep` false)
  (set `self.IsSleep2` false)
  (set `self.IsSitDown` false)
  (set `self.IsUpDownDance` false)
  (set `self.IsJumpDance` false)
  (set `self.IsLanding` false))

(fn `UserConstructionScript`)
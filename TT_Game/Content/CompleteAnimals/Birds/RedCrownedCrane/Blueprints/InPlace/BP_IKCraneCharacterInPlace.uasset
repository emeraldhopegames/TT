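; In-place red-crowned crane character that moves itself along the ground and computes foot IK to fit the terrain.
; Each tick, downward traces under both tarsus bones yield height-offset effector locations and normal-aligned foot rotations, smoothed by interpolation.
; While walking, forward and turn speeds drive movement input and capsule yaw; landing zeroes those speeds.
; The construction script scales trace distance, foot offset and input factor by actor scale.
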(event `self.ReceiveTick`
  (params (DeltaSeconds :type "Float (single-precision)"))
  (`parent.ReceiveTick` DeltaSeconds)
  (`self.FootPlacement`)
  (if (`self.IsLanding`)
    (set `self.AimTurnSpeed` 0.0)
    (set `self.InitialTurnSpeed` 0.0)
    (set `self.TurnSpeed` 0.0)
    (set `self.AimForwardSpeed` 0.0)
    (set `self.InitialForwardSpeed` 0.0)
    (set `self.ForwardSpeed` 0.0)
    (elif (`CharacterMovementComponent.IsWalking` (`self.CharacterMovement`))
      (`PawnMovementComponent.AddInputVector` (`self.CharacterMovement`) (* (* (`SceneComponent.GetForwardVector` (`self.CapsuleComponent`)) (`self.ForwardSpeed`)) (`self.InputScaleFactor`)) false)
      (`SceneComponent.K2_AddLocalRotation` (`self.CapsuleComponent`) (`KismetMathLibrary.MakeRotator` 0.0 0.0 (* (* (`GameplayStatics.GetWorldDeltaSeconds`) (`self.TurnSpeed`)) 90.0)) false false))))

(fn `FootPlacement`
  ;[1 1 1] Calculate the L_Tarsus_2EffectorLoc's Location and L_Tarsus_2's rotation.
  (bind (_legikeffectorloc _footrot) (`self.TraceIKEffector` (`self.L_Tarsus_2`) (`self.IKTraceDistance`) (`self.IKHeightOffset`)))
  ;[1 1 1] Set the left foot rotation.
  (set `self.L_Tarsus_2Rot` (`KismetMathLibrary.RInterpTo` (`self.L_Tarsus_2Rot`) _footrot (`GameplayStatics.GetWorldDeltaSeconds`) (`self.FootRotInterpSpeed`)))
  ;[1 1 1] Set the left foot IK effecter location.
  (set `self.L_Tarsus_2EffectorLoc` (`KismetMathLibrary.VInterpTo` (`self.L_Tarsus_2EffectorLoc`) _legikeffectorloc (`GameplayStatics.GetWorldDeltaSeconds`) (`self.IKInterpSpeed`)))
  ;[1 1 1] Calculate the R_Tarsus_2EffectorLoc's Location and R_Tarsus_2's rotation.
  (bind (_legikeffectorloc_2 _footrot_2) (`self.TraceIKEffector` (`self.R_Tarsus_2`) (`self.IKTraceDistance`) (`self.IKHeightOffset`)))
  ;[1 1 1] Set the right foot rotation.
  (set `self.R_Tarsus_2Rot` (`KismetMathLibrary.RInterpTo` (`self.R_Tarsus_2Rot`) _footrot_2 (`GameplayStatics.GetWorldDeltaSeconds`) (`self.FootRotInterpSpeed`)))
  ;[1 1 1] Set the right foot effector location.
  (set `self.R_Tarsus_2EffectorLoc` (`KismetMathLibrary.VInterpTo` (`self.R_Tarsus_2EffectorLoc`) _legikeffectorloc_2 (`GameplayStatics.GetWorldDeltaSeconds`) (`self.IKInterpSpeed`)))
  (return))

(fn `TraceIKEffector`
  (params (FootName :type Name) (TraceDistance :type "Float (double-precision)") (HeightOffset :type "Float (double-precision)"))
  (returns (LegIKEffectorLoc :type "Vector Structure") (FootRot :type "Rotator Structure"))
  (locals (GroundNormal :type "Vector Structure") (TraceFootName :type Name) (DoesReachThaGround :type Boolean) (InitialFootLocation :type "Vector Structure") (InitialFootRotation :type "Rotator Structure"))
  (bind _x (.x (`local.InitialFootLocation`)))
  (bind _y (.y (`local.InitialFootLocation`)))
  (bind _z (.z (`self.K2_GetActorLocation`)))
  (bind (_x_2 _y_2 _z_2) (`KismetMathLibrary.BreakRotIntoAxes` (`local.InitialFootRotation`)))
  (bind _returnvalue (`KismetMathLibrary.Cross_VectorVector` _y_2 (`local.GroundNormal`)))
  (bind _returnvalue_2 (`KismetMathLibrary.DegAsin` (`KismetMathLibrary.VSize` _returnvalue)))
  ;[1 1 1] Set the InitialFootLocation and InitialFootRotation  for use later.
  (set `local.InitialFootLocation` (`SceneComponent.GetSocketLocation` (`self.Mesh`) FootName))
  (set `local.InitialFootRotation` (`SceneComponent.GetSocketRotation` (`self.Mesh`) FootName))
  ;[1 1 1] Calculate the location of foot.
  ;;[1 1 1] Trace from foot location to the location lowered by the TraceDistance from the location of the foot
  (bind (_outhit _returnvalue_3) (`KismetSystemLibrary.LineTraceSingle` (`KismetMathLibrary.MakeVector` _x _y _z) (`KismetMathLibrary.MakeVector` _x _y (- _z TraceDistance)) "TraceTypeQuery1" true))
  ;;[1 1 1] Set the DoesReachTheGround and GroundNormal  for use later.
  (set `local.DoesReachThaGround` _returnvalue_3)
  (bind (_bblockinghit _binitialoverlap _time _distance _location _impactpoint _normal) (`GameplayStatics.BreakHitResult` _outhit))
  (set `local.GroundNormal` _normal)
  (return (`KismetMathLibrary.SelectVector` (`KismetMathLibrary.MakeVector` (.x _location) (.y _location) (+ (.z _location) HeightOffset)) (`local.InitialFootLocation`) (`local.DoesReachThaGround`)) (`KismetMathLibrary.SelectRotator` (`KismetMathLibrary.MakeRotationFromAxes` (`KismetMathLibrary.RotateAngleAxis` _x_2 _returnvalue_2 _returnvalue) (`local.GroundNormal`) (`KismetMathLibrary.RotateAngleAxis` _z_2 _returnvalue_2 _returnvalue)) (`local.InitialFootRotation`) (`local.DoesReachThaGround`))))

(fn `UserConstructionScript`
  (`parent.UserConstructionScript`)
  ;[1 1 1] Set the Scale
  (set `self.Scale` (.z (.scale (`self.GetTransform`))))
  ;[1 1 1] Set the scale dependent variables.
  (set `self.IKTraceDistance` (* (* (`CapsuleComponent.CapsuleHalfHeight` (`self.CapsuleComponent`)) 3.0) (`self.Scale`)))
  (set `self.IKHeightOffset` (* (`self.Scale`) (`self.IKHeightOffset`)))
  (set `self.InputScaleFactor` (* (`self.Scale`) (`self.InputScaleFactor`))))
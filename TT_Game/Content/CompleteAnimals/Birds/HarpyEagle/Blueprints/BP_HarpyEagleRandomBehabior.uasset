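; Harpy eagle Blueprint that drives random wandering, idle actions and flight between perches and landing points.
; Tick branches on movement mode: timed random choices with lerped speeds on the ground, steering and acceleration toward ObjectivePoint in flight.
; BeginPlay gathers perch and landing-point actors, from which SetObjectivePoint picks random targets.
; Timeouts, perch pushes and capsule hits trigger take-off, attacks, jumps or landing attempts.
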(event `self.ReceiveTick`
  (params (DeltaSeconds :type "Float (single-precision)"))
  (bind _returnvalue (`SceneComponent.K2_GetComponentToWorld` (`self.CapsuleComponent`)))
  (bind _returnvalue_2 (< (`self.FlyForwardSpeed`) (`self.MeanForwardSpeed`)))
  (bind _returnvalue_3 (`KismetMathLibrary.InverseTransformLocation` _returnvalue (`self.ObjectivePoint`)))
  (bind _returnvalue_4 (- (.z (`self.ObjectivePoint`)) (.z (.location _returnvalue))))
  (bind _returnvalue_5 (> (`KismetMathLibrary.VSizeSquared` _returnvalue_3) 20000.0))
  (`parent.ReceiveTick` DeltaSeconds)
  (if (`CharacterMovementComponent.IsWalking` (`self.CharacterMovement`))
    (if (`self.IsLandingPerch`)
      ;[1 1 1] When IsLandingPerch is true
      (set `self.ChangeTime` (+ (`self.ChangeTime`) (`GameplayStatics.GetWorldDeltaSeconds`)))
      (if (> (`self.ChangeTime`) 10.0)
        (set `self.IsSoaring` true)
        (set `self.FlyForwardSpeed` 10.0)
        (set `self.UpSpeed` 2.0)
        (set `self.FlyForwardAcceleration` 5.0)
        (set `self.FlyUpAcceleration` 2.0)
        (if (< (`KismetMathLibrary.Abs` (`self.ForwardSpeed`)) 0.1)
          (`KismetSystemLibrary.Delay` 0.5))
        (`self.Soar`)
        (`self.SetObjectivePoint` true)
        (set `self.IsObjectivePointLand` true)
        (set `self.IsTryLandingToLand` false)
        (set `self.IsLandingPerch` false))
      (else
        ;[1 1 1] Random behabior at the ground.
        ;;[1 1 1] Turn the Harpy eagle
        (if (and (not (or (or (or (`self.IsCrying`) (`self.IsEating`)) (`self.IsSitdown`)) (`self.IsGrooming`))) (`self.IsLived`))
          (`SceneComponent.K2_AddLocalRotation` (`self.CapsuleComponent`) (`KismetMathLibrary.MakeRotator` 0.0 0.0 (* (* DeltaSeconds (`self.TurnSpeed`)) 45.0)) false false))
        (if (> (`self.ChangeTime`) (`self.NextChangeTime`))
          (if (not (`self.IsSoaring`))
            (set `self.IsGrooming` false)
            (set `self.IsEating` false)
            (set `self.IsCrying` false)
            (set `self.IsAttacking` false)
            (set `self.IsAttacking2` false)
            (set `self.IsHitting` false)
            (switch `int` (`KismetMathLibrary.RandomIntegerInRange` 0 9)
              (:`Default`
                (set `self.ChangeTime` 0.0 :!label _label)
                (set `self.NextChangeTime` (`KismetMathLibrary.RandomFloatInRange` 1.0 3.0))
                (set `self.InitialForwardSpeed` (`self.ForwardSpeed`))
                (set `self.AimForwardSpeed` (`KismetMathLibrary.RandomFloatInRange` -0.5 1.0))
                (set `self.InitialTurnSpeed` (`self.TurnSpeed`))
                (set `self.AimTurnSpeed` (`KismetMathLibrary.RandomFloatInRange` -1.0 1.0)))
              (:`0`
                (set `self.IsGrooming` true)
                (set `self.ChangeTime` 0.0 :!label _label_2)
                (set `self.NextChangeTime` (`KismetMathLibrary.RandomFloatInRange` 1.0 3.0))
                (set `self.InitialForwardSpeed` (`self.ForwardSpeed`))
                (set `self.AimForwardSpeed` 0.0)
                (set `self.InitialTurnSpeed` (`self.TurnSpeed`))
                (set `self.AimTurnSpeed` 0.0))
              (:`1`
                (set `self.IsEating` false)
                (goto _label_2))
              (:`2`
                (set `self.IsCrying` true)
                (goto _label_2))
              (:`3`
                (set `self.IsAttacking` true)
                (goto _label))
              (:`4`
                (set `self.IsAttacking2` true)
                (goto _label))
              (:`5`
                ;;[1 1 1] Soar
                (if (and (!= (`KismetArrayLibrary.Array_Length` (`self.LandingPoints`)) 0) (!= (`KismetArrayLibrary.Array_Length` (`self.Perches`)) 0))
                  (set `self.IsSoaring` true)
                  (set `self.FlyForwardSpeed` 10.0)
                  (set `self.UpSpeed` 2.0)
                  (set `self.FlyForwardAcceleration` 5.0)
                  (set `self.FlyUpAcceleration` 2.0)
                  (if (< (`KismetMathLibrary.Abs` (`self.ForwardSpeed`)) 0.1)
                    (`KismetSystemLibrary.Delay` 0.5))
                  (`self.Soar`)
                  (`self.SetObjectivePoint` false)
                  (set `self.IsTryLandingToLand` false)
                  (set `self.IsObjectivePointLand` false)
                  (set `self.ChangeTime` 0.0)
                  (set `self.NextChangeTime` 0.0)
                  (else
                    (goto _label))))))
          (else
            (bind _output_get (set `self.ChangeTime` (+ (`self.ChangeTime`) (`GameplayStatics.GetWorldDeltaSeconds`))))
            ;;[1 1 1] Change the Forward Speed.
            (set `self.ForwardSpeed` (`KismetMathLibrary.Lerp` (`self.InitialForwardSpeed`) (`self.AimForwardSpeed`) (`KismetMathLibrary.FClamp` _output_get)))
            ;;[1 1 1] Change the TurnSpeed.
            (set `self.TurnSpeed` (`KismetMathLibrary.Lerp` (`self.InitialTurnSpeed`) (`self.AimForwardSpeed`) (`KismetMathLibrary.FClamp` _output_get)))))))
    (elif (`NavMovementComponent.IsFlying` (`self.CharacterMovement`))
      (`SceneComponent.K2_AddLocalRotation` (`self.CapsuleComponent`) (`KismetMathLibrary.MakeRotator` 0.0 0.0 (* (* DeltaSeconds (`self.TurnSpeed`)) 45.0)) false false)
      (if (`self.IsTryLandPerch`)
        ;[1 1 1] When IsTryLandPerch is true
        (set `self.ChangeTime` (+ (`self.ChangeTime`) (`GameplayStatics.GetWorldDeltaSeconds`)))
        (if (> (`self.ChangeTime`) 5.0)
          ;;[1 1 1] If Harpy eagle can not landing to perch, when 5 seconds after.
          (set `self.IsTryLandPerch` false)
          (`self.SetObjectivePoint` true)
          (set `self.IsObjectivePointLand` true))
        (elif (`self.IsTryLandingToLand`)
          ;[1 1 1] Decelerate when IsTryLAndingToLand is true.
          (set `self.AimFlyUpAcceleration` -5.0)
          (set `self.AimFlyForwardAcceleration` -5.0)
          (else
            ;[1 1 1] Movement mode is Flying and IsTryLandPerch is false and IsTryingToLand is false.
            (if (> (`KismetMathLibrary.Abs` _returnvalue_4) 1.0)
              (set `self.UpAccelerationChange` true)
              (set `self.AimFlyUpAcceleration` (`KismetMathLibrary.FClamp` _returnvalue_4 -5.0 5.0))
              (else
                (set `self.UpAccelerationChange` false)
                (set `self.AimFlyUpAcceleration` 0.0)))
            (set `self.AimTurnSpeed` (* (.y (`KismetMathLibrary.Normal` _returnvalue_3)) 2.5))
            (if (or (and (not _returnvalue_5) (not _returnvalue_2)) (and _returnvalue_5 _returnvalue_2))
              (set `self.ForwardAccelerationChange` true)
              (set `self.AimFlyForwardAcceleration` (`KismetMathLibrary.FClamp` (.x _returnvalue_3) -5.0 5.0))
              (else
                (set `self.ForwardAccelerationChange` false)
                (set `self.AimFlyForwardAcceleration` 0.0)
                (set `self.AimForwardSpeed` 0.0)))
            (if (`self.IsObjectivePointLand`)
              (if (< (`KismetMathLibrary.VSizeSquared` (- (`SceneComponent.K2_GetComponentLocation` (`self.CapsuleComponent`)) (`self.ObjectivePoint`))) 20000.0)
                (set `self.IsTryLandingToLand` true)
                (set `self.ChangeTime` 0.0)
                (set `self.NextChangeTime` 5.0)
                (set `self.ForwardAccelerationChange` false)
                (set `self.UpAccelerationChange` false)))))))))

(event `self.ReceiveBeginPlay`
  ;[1 1 1] Set the Perches
  (bind _outactors (`GameplayStatics.GetAllActorsOfClass` "/Game/CompleteAnimals/Birds/HarpyEagle/Blueprints/BP_HarpyEaglePerch.BP_HarpyEaglePerch_C"))
  (set `self.Perches` _outactors)
  (set `self.APerch` (`|GetArrayItem` _outactors (`KismetMathLibrary.RandomIntegerInRange` 0 (- (`KismetArrayLibrary.Array_Length` _outactors) 1))))
  ;[1 1 1] Set the LandingPoints
  (bind _outactors_2 (`GameplayStatics.GetAllActorsOfClass` "/Game/CompleteAnimals/Birds/HarpyEagle/Blueprints/BP_LandingPoint.BP_LandingPoint_C"))
  (bind _output_get (set `self.LandingPoints` _outactors_2))
  (set `self.LandingPoint` (`|GetArrayItem` _output_get (`KismetMathLibrary.RandomIntegerInRange` 0 (- (`KismetArrayLibrary.Array_Length` _output_get) 1)))))

(event `self.PushedOutFromPerch`
  ;[1 1 1] Soaring when pushed out from perch.
  (set `self.IsSoaring` true)
  (set `self.FlyForwardSpeed` 10.0)
  (set `self.UpSpeed` 2.0)
  (set `self.FlyForwardAcceleration` 5.0)
  (set `self.FlyUpAcceleration` 2.0)
  (`self.Soar`)
  (set `self.IsObjectivePointLand` true)
  (set `self.IsLandingPerch` false)
  (set `self.IsTryLandingToLand` false)
  (set `self.IsObjectivePointLand` true)
  (`self.SetObjectivePoint` true))

(event `self.CapsuleComponent.OnComponentHit`
  (params (HitComponent :type "PrimitiveComponent Object Reference") (OtherActor :type "Actor Object Reference") (OtherComp :type "PrimitiveComponent Object Reference") (NormalImpulse :type "Vector Structure") (Hit :type "HitResult Structure (by ref)"))
  (cast `/Game/CompleteAnimals/Birds/HarpyEagle/Blueprints/BP_HarpyEagleCharacter` OtherActor
    (:`then`
      (if (`self.IsLandingPerch`)
        ;[1 1 1] When Hit other Harpy eagle on the perch.
        (set `self.IsLandingPerch` false)
        (`self.SetObjectivePoint` true)
        (set `self.IsSoaring` true)
        (set `self.FlyForwardSpeed` 10.0)
        (set `self.UpSpeed` 2.0)
        (set `self.FlyForwardAcceleration` 5.0)
        (set `self.FlyUpAcceleration` 2.0)
        (if (< (`KismetMathLibrary.Abs` (`self.ForwardSpeed`)) 0.1)
          (`KismetSystemLibrary.Delay` 0.5))
        (`self.Soar`)
        (set `self.IsObjectivePointLand` true)
        (elif (`CharacterMovementComponent.IsWalking` (`self.CharacterMovement`))
          ;[1 1 1] When Hit other Harpy eagle at the ground.
          (switch `int` (`KismetMathLibrary.RandomIntegerInRange` 0 5)
            (:`Default`
              (set `self.JumpStart` true)
              (`KismetSystemLibrary.Delay` 0.3)
              (`self.Jump`)
              (set `self.JumpStart` false))
            (:`0`
              (set `self.IsAttacking` true))
            (:`1`
              (set `self.IsAttacking2` true))
            (:`2`
              (set `self.IsHitting` true)))
          (else
            (if (`NavMovementComponent.IsFlying` (`self.CharacterMovement`)) :!label _label_3
              (set `self.IsTryLandingToLand` true)
              (set `self.ChangeTime` 0.0)
              (set `self.NextChangeTime` 5.0)
              (set `self.ForwardAccelerationChange` false)
              (set `self.UpAccelerationChange` false)
              (`PrimitiveComponent.SetEnableGravity` (`self.CapsuleComponent`) true))))))
    (:`CastFailed`
      (goto _label_3))))

(fn `SetObjectivePoint`
  (params (IsLand :type Boolean))
  (bind _perches (`self.Perches`))
  (bind _landingpoints (`self.LandingPoints`))
  (if IsLand
    ;[1 1 1] Random select LandingPoint from LandingPoints.
    (bind _output_get (set `self.LandingPoint` (`|GetArrayItem` _landingpoints (`KismetMathLibrary.RandomIntegerInRange` 0 (- (`KismetArrayLibrary.Array_Length` _landingpoints) 1)))))
    (set `self.ObjectivePoint` (`SceneComponent.K2_GetComponentLocation` (`/Game/CompleteAnimals/Birds/HarpyEagle/Blueprints/BP_LandingPoint.DefaultSceneRoot` _output_get)))
    (else
      ;[1 1 1] Random Select APerch from Perches.
      (bind _output_get_2 (set `self.APerch` (`|GetArrayItem` _perches (`KismetMathLibrary.RandomIntegerInRange` 0 (- (`KismetArrayLibrary.Array_Length` _perches) 1)))))
      (set `self.ObjectivePoint` (`SceneComponent.K2_GetComponentLocation` (`/Game/CompleteAnimals/Birds/HarpyEagle/Blueprints/BP_HarpyEaglePerch.DefaultSceneRoot` _output_get_2))))))

(fn `UserConstructionScript`
  (`parent.UserConstructionScript`))
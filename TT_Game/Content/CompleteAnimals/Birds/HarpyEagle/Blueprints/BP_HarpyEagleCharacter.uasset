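; Character Blueprint for a harpy eagle that walks, soars, lands on the ground and settles on perches.
; Tick branches on movement mode, driving walk input, acceleration-based flight offsets, trace-detected ground landing, or interpolation onto perch arrows.
; Foot IK targets come from line traces aligned to surface normals or from perch foot arrows, with trace and speed factors scaled by actor size.
; An eagle pushed off its perch resumes soaring.
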(event `self.ReceiveTick`
  (params (DeltaSeconds :type "Float (single-precision)"))
  (bind _aimpercharrow (`self.AimPerchArrow`))
  (bind _capsulecomponent (`self.CapsuleComponent`))
  (bind _capsulecomponent_2 (`self.CapsuleComponent`))
  (bind _aimpercharrow_2 (`self.AimPerchArrow`))
  (bind _returnvalue (`SceneComponent.K2_GetComponentLocation` _capsulecomponent))
  (bind _returnvalue_2 (`SceneComponent.K2_GetComponentLocation` _aimpercharrow))
  (bind _returnvalue_3 (`SceneComponent.K2_GetComponentLocation` _capsulecomponent_2))
  (bind _y (.y (`KismetMathLibrary.InverseTransformLocation` (`SceneComponent.K2_GetComponentToWorld` _capsulecomponent) (+ _returnvalue (`SceneComponent.GetForwardVector` _aimpercharrow)))))
  (bind _y_2 (.y (`KismetMathLibrary.InverseTransformLocation` (`SceneComponent.K2_GetComponentToWorld` _capsulecomponent_2) (+ _returnvalue_3 (`SceneComponent.GetForwardVector` _aimpercharrow_2)))))
  ;[1 1 1] Set Forward Speed
  (set `self.ForwardSpeed` (`KismetMathLibrary.FInterpTo` (`self.ForwardSpeed`) (`self.AimForwardSpeed`) DeltaSeconds 5.0))
  ;[1 1 1] Set TurnSpeed
  (set `self.TurnSpeed` (`KismetMathLibrary.FInterpTo` (`self.TurnSpeed`) (`self.AimTurnSpeed`) DeltaSeconds 5.0))
  (if (`CharacterMovementComponent.IsWalking` (`self.CharacterMovement`))
    (if (`self.IsLandingPerch`)
      ;[1 1 1] IsLandingPerch is true.
      (if (> (`KismetMathLibrary.VSizeSquared` (- (`SceneComponent.K2_GetComponentLocation` (`self.CapsuleComponent`)) (`SceneComponent.K2_GetComponentLocation` (`self.AimPerchArrow`)))) (* (`self.Scale`) 625.0))
        (`self.PushedOutFromPerch`)
        (else
          (`SceneComponent.K2_SetWorldLocation` (`self.CapsuleComponent`) (`KismetMathLibrary.VInterpTo` _returnvalue_3 (`SceneComponent.K2_GetComponentLocation` _aimpercharrow_2) (`GameplayStatics.GetWorldDeltaSeconds`) 10.0) false false)
          (if (> _y_2 0.05)
            (set `self.AimTurnSpeed` 0.5)
            (elif (< _y_2 -0.05)
              (set `self.AimTurnSpeed` -0.5)
              (else
                (set `self.AimTurnSpeed` 0.0))))
          ;;[1 1 1] Foot IKEffecter locations and FootRotations are Set by FootArrows.
          (set `self.L_Tarsus_2EffectorLoc` (`SceneComponent.K2_GetComponentLocation` (`self.PerchLeftFootArrow`)) :!label _label)
          (set `self.R_Tarsus_2EffectorLoc` (`SceneComponent.K2_GetComponentLocation` (`self.PerchRightFootArrow`)))
          (set `self.R_Tarsus_2Rot` (`KismetMathLibrary.RInterpTo` (`self.R_Tarsus_2Rot`) (`SceneComponent.K2_GetComponentRotation` (`self.PerchRightFootArrow`)) (`GameplayStatics.GetWorldDeltaSeconds`) (`self.FootRotInterpSpeed`)))
          (set `self.L_Tarsus_2Rot` (`KismetMathLibrary.RInterpTo` (`self.L_Tarsus_2Rot`) (`SceneComponent.K2_GetComponentRotation` (`self.PerchLeftFootArrow`)) (`GameplayStatics.GetWorldDeltaSeconds`) (`self.FootRotInterpSpeed`)))))
      (else
        ;[1 1 1] Movement mode is Walking and IsLandingPerch is false.
        (`self.FootPlacement`)
        (if (and (not (or (or (or (`self.IsCrying`) (`self.IsEating`)) (`self.IsSitdown`)) (`self.IsGrooming`))) (`self.IsLived`))
          (`PawnMovementComponent.AddInputVector` (`self.CharacterMovement`) (* (* (`SceneComponent.GetForwardVector` (`self.CapsuleComponent`)) (`self.ForwardSpeed`)) (`self.InputScaleFactor`)) false))))
    (elif (`NavMovementComponent.IsFalling` (`self.CharacterMovement`))
      (`self.FootPlacement`)
      (elif (`NavMovementComponent.IsFlying` (`self.CharacterMovement`))
        (if (`self.IsTryLandPerch`)
          ;[1 1 1] Movement mode is Flying and IsTryLandPerch is true.
          (`SceneComponent.K2_SetWorldLocation` (`self.CapsuleComponent`) (`KismetMathLibrary.VInterpTo` _returnvalue _returnvalue_2 (`GameplayStatics.GetWorldDeltaSeconds`) (* (`self.Scale`) 3.0)) false false)
          (if (> _y 0.01)
            (set `self.AimTurnSpeed` 0.5)
            (elif (< _y -0.01)
              (set `self.AimTurnSpeed` -0.5)))
          (if (and (< (`KismetMathLibrary.VSize` (- _returnvalue _returnvalue_2)) (* (`self.Scale`) 15.0)) (< (`KismetMathLibrary.Abs` _y) 0.05))
            ;;[1 1 1] When Harpy Eagle's position and rotation is near the AimPerchArrow's  position and rotation.
            (set `self.IsLandingPerch` true)
            (set `self.IsTryLandPerch` false)
            (`CharacterMovementComponent.SetMovementMode` (`self.CharacterMovement`) "MOVE_Walking" 0)
            (set `self.IsSoaring` false)
            (`PrimitiveComponent.SetSimulatePhysics` (`self.CapsuleComponent`) false)
            (else
              (goto _label)))
          (else
            ;[1 1 1] Movement mode is Flying and IsTryLandPerch is false.
            ;;[1 1 1] Change UpSpeed by FlyUpAccelaration.
            (set `self.UpSpeed` (`KismetMathLibrary.FClamp` (+ (`self.UpSpeed`) (* (`self.FlyUpAcceleration`) DeltaSeconds)) (`self.MaxDownSpeed`) (`self.MaxUpSpeed`)))
            ;;[1 1 1] Change FlyForwardSpeed by FlyForwardAcceleration.
            (set `self.FlyForwardSpeed` (`KismetMathLibrary.FClamp` (+ (`self.FlyForwardSpeed`) (* (`self.FlyForwardAcceleration`) DeltaSeconds)) 0.0 (`self.MaxFlySpeed`)))
            ;;[1 1 1] Change FlyUpAcceleration by AimFlyUpAcceleration.
            (set `self.FlyUpAcceleration` (`KismetMathLibrary.FInterpTo` (`self.FlyUpAcceleration`) (`self.AimFlyUpAcceleration`) DeltaSeconds 5.0))
            ;;[1 1 1] Change FlyForwardAcceleration by AimFlyForwardAcceleration.
            (set `self.FlyForwardAcceleration` (`KismetMathLibrary.FInterpTo` (`self.FlyForwardAcceleration`) (`self.AimFlyForwardAcceleration`) DeltaSeconds 5.0))
            (if (not (or (`self.ForwardAccelerationChange`) (`self.UpAccelerationChange`)))
              ;;[1 1 1] Calculate AimFlyUpAccleration and AimFlyForwardAcceleration from FlyForwardSpeed.
              (set `self.AimFlyUpAcceleration` (* (- (`self.MeanForwardSpeed`) (`self.FlyForwardSpeed`)) -0.1))
              (set `self.AimFlyForwardAcceleration` (* (`self.FlyForwardSpeed`) -0.1)))
            ;;[1 1 1] Move the Harpy Eagle by FlyForwardSpeed and FlyUpSpeed.
            (`self.K2_AddActorLocalOffset` (* (`KismetMathLibrary.MakeVector` (* (`self.FlyForwardSpeed`) DeltaSeconds) 0.0 (* (`self.UpSpeed`) DeltaSeconds)) (`self.FlySpeedScaleFactor`)) true)
            (`self.FootPlacement`)
            (if (and (and (<= (`self.UpSpeed`) 0.0) (not (or (`self.ForwardAccelerationChange`) (`self.UpAccelerationChange`)))) (not (`self.IsTryLandPerch`)))
              (set `self.IsSoaring` false)
              (bind (_outhit _returnvalue_4) (`KismetSystemLibrary.LineTraceSingle` (`SceneComponent.K2_GetComponentLocation` (`self.CapsuleComponent`)) (`KismetMathLibrary.MakeVector` (.x (`SceneComponent.K2_GetComponentLocation` (`self.CapsuleComponent`))) (.y (`SceneComponent.K2_GetComponentLocation` (`self.CapsuleComponent`))) (- (.z (`SceneComponent.K2_GetComponentLocation` (`self.CapsuleComponent`))) (`self.IKTraceDistance`))) "TraceTypeQuery1"))
              (if _returnvalue_4
                ;;[1 1 1] Landing
                (`CharacterMovementComponent.SetMovementMode` (`self.CharacterMovement`) "MOVE_Walking" 0)
                (`PrimitiveComponent.SetEnableGravity` (`self.CapsuleComponent`) true)
                (`PrimitiveComponent.SetSimulatePhysics` (`self.CapsuleComponent`) false)
                (set `self.IKInterpSpeed` 10.0)))))))))

(fn `CanJumpInternal`
  (returns (ReturnValue :type Boolean))
  (return (and (and (and (and (and (and (and (and (or (`self.IsLandingPerch`) (`CharacterMovementComponent.IsWalking` (`self.CharacterMovement`))) (not (`self.IsAttacking`))) (not (`self.IsHitting`))) (not (`self.IsSneaking`))) (not (`self.IsGrooming`))) (not (`self.IsCrying`))) (not (`self.IsEating`))) (`self.IsLived`)) (not (`self.IsSitdown`)))))

(fn `FootPlacement`
  (bind _returnvalue (`GameplayStatics.GetWorldDeltaSeconds`))
  (bind (_legikeffectorloc _footrot) (`self.TraceIKEffector` (`self.L_Tarsus_2`) (`self.IKTraceDistance`) (`self.IKHeightOffset`)))
  ;[1 1 1] Set the left foot rotation.
  (set `self.L_Tarsus_2Rot` (`KismetMathLibrary.RInterpTo` (`self.L_Tarsus_2Rot`) _footrot _returnvalue (`self.FootRotInterpSpeed`)))
  ;[1 1 1] Set the let foot IK effecter location.
  (set `self.L_Tarsus_2EffectorLoc` (`KismetMathLibrary.VInterpTo` (`self.L_Tarsus_2EffectorLoc`) _legikeffectorloc _returnvalue (`self.IKInterpSpeed`)))
  (bind (_legikeffectorloc_2 _footrot_2) (`self.TraceIKEffector` (`self.R_Tarsus_2`) (`self.IKTraceDistance`) (`self.IKHeightOffset`)))
  ;[1 1 1] Set the right foot rotation.
  (set `self.R_Tarsus_2Rot` (`KismetMathLibrary.RInterpTo` (`self.R_Tarsus_2Rot`) _footrot_2 _returnvalue (`self.FootRotInterpSpeed`)))
  ;[1 1 1] Set the right foot effector location.
  (set `self.R_Tarsus_2EffectorLoc` (`KismetMathLibrary.VInterpTo` (`self.R_Tarsus_2EffectorLoc`) _legikeffectorloc_2 _returnvalue (`self.IKInterpSpeed`)))
  (return))

(fn `PushedOutFromPerch`
  (set `self.IsSoaring` true)
  (set `self.FlyForwardSpeed` 10.0)
  (set `self.UpSpeed` 2.0)
  (set `self.FlyForwardAcceleration` 5.0)
  (set `self.FlyUpAcceleration` 2.0)
  (`self.Soar`)
  (set `self.IsObjectivePointLand` true)
  (set `self.IsLandingPerch` false)
  (set `self.IsHitting` false))

(fn `Soar`
  (`CharacterMovementComponent.SetMovementMode` (`self.CharacterMovement`) "MOVE_Flying" 0)
  (`PrimitiveComponent.SetEnableGravity` (`self.CapsuleComponent`) false)
  (`PrimitiveComponent.SetSimulatePhysics` (`self.CapsuleComponent`) true)
  (set `self.FlyForwardSpeed` 10.0)
  (set `self.UpSpeed` 2.0)
  (set `self.FlyForwardAcceleration` 5.0)
  (set `self.FlyUpAcceleration` 2.0)
  (set `self.AimFlyUpAcceleration` 0.0)
  (set `self.AimFlyForwardAcceleration` 0.0)
  (set `self.IKInterpSpeed` 50.0)
  (set `self.IsTryLandPerch` false)
  (set `self.IsLandingPerch` false)
  (set `self.IsAttacking` false)
  (set `self.IsHitting` false)
  (`ActorComponent.Activate` (`self.CharacterMovement`) false))

(fn `StartLandToPerch`
  (params (Arrow :type "ArrowComponent Object Reference") (LeftFootArrow :type "ArrowComponent Object Reference") (RightFootArrow :type "ArrowComponent Object Reference"))
  (set `self.IsTryLandPerch` true)
  (set `self.AimPerchArrow` Arrow)
  (set `self.PerchLeftFootArrow` LeftFootArrow)
  (set `self.PerchRightFootArrow` RightFootArrow)
  (`PrimitiveComponent.SetSimulatePhysics` (`self.CapsuleComponent`) false)
  (set `self.IsObjectivePointLand` false))

(fn `TraceIKEffector`
  (params (FootName :type Name) (TraceDistance :type "Float (double-precision)" :default 50.0) (HeightOffset :type "Float (double-precision)" :default 10.0))
  (returns (LegIKEffectorLoc :type "Vector Structure") (FootRot :type "Rotator Structure"))
  (bind _returnvalue (`SceneComponent.GetSocketLocation` (`self.Mesh`) FootName))
  (bind _returnvalue_2 (`SceneComponent.GetSocketRotation` (`self.Mesh`) FootName))
  (bind _z (.z (`self.K2_GetActorLocation`)))
  (bind _x (.x _returnvalue))
  (bind _y (.y _returnvalue))
  (bind (_x_2 _y_2 _z_2) (`KismetMathLibrary.BreakRotIntoAxes` _returnvalue_2))
  ;[1 1 1] Calculate the location of foot.
  (bind (_outhit _returnvalue_3) (`KismetSystemLibrary.LineTraceSingle` (`KismetMathLibrary.MakeVector` _x _y _z) (`KismetMathLibrary.MakeVector` _x _y (- _z TraceDistance)) "TraceTypeQuery1" true))
  (bind (_bblockinghit _binitialoverlap _time _distance _location _impactpoint _normal) (`GameplayStatics.BreakHitResult` _outhit))
  (bind _returnvalue_4 (`KismetMathLibrary.Cross_VectorVector` _y_2 _normal))
  (bind _returnvalue_5 (`KismetMathLibrary.DegAsin` (`KismetMathLibrary.VSize` _returnvalue_4)))
  (return (`KismetMathLibrary.SelectVector` (`KismetMathLibrary.MakeVector` (.x _location) (.y _location) (+ (.z _location) HeightOffset)) _returnvalue _returnvalue_3) (`KismetMathLibrary.SelectRotator` (`KismetMathLibrary.MakeRotationFromAxes` (`KismetMathLibrary.RotateAngleAxis` _x_2 _returnvalue_5 _returnvalue_4) _normal (`KismetMathLibrary.RotateAngleAxis` _z_2 _returnvalue_5 _returnvalue_4)) _returnvalue_2 _returnvalue_3)))

(fn `UserConstructionScript`
  (bind _scale (`self.Scale`))
  (set `self.Scale` (.z (.scale (`self.GetTransform`))))
  ;[1 1 1] Set the scale dependent variables.
  (set `self.IKTraceDistance` (* (* (`CapsuleComponent.CapsuleHalfHeight` (`self.CapsuleComponent`)) 3.0) _scale))
  (set `self.IKHeightOffset` (* _scale (`self.IKHeightOffset`)))
  (set `self.InputScaleFactor` (* (`self.InputScaleFactor`) _scale))
  (set `self.FlySpeedScaleFactor` (* (`self.FlySpeedScaleFactor`) _scale)))
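; BP_ChasePenguin is a penguin Blueprint that chases the first player's pawn by driving movement and swim variables.
; Each Tick runs the parent's logic, then retargets the player's current location.
; Dot products against capsule axes yield turn, yaw, pitch and forward aims, with a fixed turn when the goal is behind.
; Swim acceleration scales with squared distance, turn and forward speeds are interpolated, and forward aims zero when close.
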(event `self.ReceiveBeginPlay`
  ;[1 1 1] Set the Player
  (set `self.Player` (`GameplayStatics.GetPlayerPawn` 0)))

(event `self.ReceiveTick`
  (params (DeltaSeconds :type "Float (single-precision)"))
  (bind _returnvalue (- (`self.GoalLoc`) (`SceneComponent.K2_GetComponentLocation` (`self.CapsuleComponent`))))
  (bind _returnvalue_2 (`KismetMathLibrary.Normal` _returnvalue))
  (bind _returnvalue_3 (`KismetMathLibrary.Dot_VectorVector` _returnvalue_2 (`SceneComponent.GetForwardVector` (`self.CapsuleComponent`))))
  (bind _returnvalue_4 (`KismetMathLibrary.Dot_VectorVector` _returnvalue_2 (`SceneComponent.GetRightVector` (`self.CapsuleComponent`))))
  (bind _returnvalue_5 (>= _returnvalue_3 0.0))
  (`parent.ReceiveTick` DeltaSeconds)
  ;[1 1 1] Set the GoalLoc.
  (set `self.GoalLoc` (`self.K2_GetActorLocation` (`self.Player`)))
  ;[1 1 1] Is the goal close?
  (if (<= (`KismetMathLibrary.VSizeSquared` (- (`self.GoalLoc`) (`self.K2_GetActorLocation`))) 10000.0)
    (set `self.AimForwardSpeed` 0.0)
    (set `self.AimSwimForwardAcceleration` 0.0)
    (else
      ;[1 1 1] Set AimTurnSpeed according to the positional relationship between the character and the next movement point.
      (if _returnvalue_5
        (set `self.AimTurnSpeed` _returnvalue_4)
        (set `self.AimYawSpeed` (* _returnvalue_4 90.0))
        (else
          (set `self.AimTurnSpeed` -1.0)
          (set `self.AimYawSpeed` -90.0)))
      (set `self.AimPitchSpeed` (* (`KismetMathLibrary.Dot_VectorVector` (`SceneComponent.GetUpVector` (`self.CapsuleComponent`)) _returnvalue_2) 30.0))
      (set `self.SwimForwardAcceleration` (`KismetMathLibrary.FClamp` (* (- (`KismetMathLibrary.VSizeSquared` _returnvalue) -100000.0) 0.0001) -1000.0 (`self.MaxSwimForwardAcceleration`)))
      (set `self.AimForwardSpeed` (`KismetMathLibrary.SelectFloat` (`KismetMathLibrary.Abs` _returnvalue_3) 0.0 _returnvalue_5))
      ;[1 1 1] Set the TurnSpeed.
      (set `self.TurnSpeed` (`KismetMathLibrary.FInterpTo` (`self.TurnSpeed`) (`self.AimTurnSpeed`) (`self.DeltaSeconds`) 1.0))
      ;[1 1 1] Set the ForwardSpeed
      (set `self.ForwardSpeed` (`KismetMathLibrary.FInterpTo` (`self.ForwardSpeed`) (`self.AimForwardSpeed`) (`self.DeltaSeconds`) 15.0)))))

(fn `UserConstructionScript`
  (`parent.UserConstructionScript`))
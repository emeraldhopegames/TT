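; BP_BeastBoy is a player-controlled shapeshifter that swaps itself for a penguin or wolf character when key 1 or 2 is pressed.
; The Winter graph spawns the chosen animal at the actor's transform, lowered slightly, has the player controller possess it, then destroys BeastBoy.
; The penguin's spring arm takes on the control rotation; the wolf's matching step is disconnected and never runs.
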(event `Key|One`
  (params (Key :type "Key Structure"))
  (bind _returnvalue (`GameplayStatics.GetPlayerController` 0))
  (bind _returnvalue_2 (`self.GetTransform`))
  (:`Pressed`
    (bind _returnvalue_3 (`|SpawnActorFromClass` "/Game/CompleteAnimals/Birds/Penguin/Blueprints/BP_PenguinThirdPersonCharacter.BP_PenguinThirdPersonCharacter_C" (`KismetMathLibrary.MakeTransform` (`KismetMathLibrary.MakeVector` (.x (.location _returnvalue_2)) (.y (.location _returnvalue_2)) (- (.z (.location _returnvalue_2)) 50.0)) (.rotation _returnvalue_2)) "Undefined" "MultiplyWithRoot" null null))
    (`Controller.Possess` _returnvalue _returnvalue_3)
    (`SceneComponent.K2_SetRelativeRotation` (`/Game/CompleteAnimals/Birds/Penguin/Blueprints/BP_PenguinThirdPersonCharacter.SpringArm` _returnvalue_3) (`Controller.GetControlRotation` _returnvalue) false false)
    (`self.K2_DestroyActor`)))

(event `Key|Two`
  (params (Key :type "Key Structure"))
  (bind _returnvalue (`self.GetTransform`))
  (:`Pressed`
    (bind _returnvalue_2 (`|SpawnActorFromClass` "/Game/CompleteAnimals/Mammals/Wolf/Blueprints/BP_WolfThirdPerssonCharacter.BP_WolfThirdPerssonCharacter_C" (`KismetMathLibrary.MakeTransform` (`KismetMathLibrary.MakeVector` (.x (.location _returnvalue)) (.y (.location _returnvalue)) (- (.z (.location _returnvalue)) 50.0)) (.rotation _returnvalue)) "Undefined" "MultiplyWithRoot" null null))
    (`Controller.Possess` (`GameplayStatics.GetPlayerController` 0) _returnvalue_2)
    (`self.K2_DestroyActor`)))

(fn `UserConstructionScript`
  (`parent.UserConstructionScript`))
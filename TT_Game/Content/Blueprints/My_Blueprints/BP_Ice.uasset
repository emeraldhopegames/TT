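; BP_Ice is a trigger volume that flags the player character as standing on ice.
; On BeginPlay it caches player 0's SandboxCharacter_CMC.
; Its Box overlap events set that character's Ice flag true on entry and false on exit, leaving any movement response to the character.
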(event `self.ReceiveBeginPlay`
  (bind _assandbox_character_cmc (cast `/Game/Blueprints/SandboxCharacter_CMC` (`GameplayStatics.GetPlayerCharacter` 0)))
  (set `self.MainChar` _assandbox_character_cmc))

(event `self.Box.OnComponentBeginOverlap`
  (params (OverlappedComponent :type "PrimitiveComponent Object Reference") (OtherActor :type "Actor Object Reference") (OtherComp :type "PrimitiveComponent Object Reference") (OtherBodyIndex :type Integer) (bFromSweep :type Boolean) (SweepResult :type "HitResult Structure (by ref)"))
  (if (== OtherActor (`self.MainChar`))
    (set `/Game/Blueprints/SandboxCharacter_CMC.Ice?` true (`self.MainChar`))))

(event `self.Box.OnComponentEndOverlap`
  (params (OverlappedComponent :type "PrimitiveComponent Object Reference") (OtherActor :type "Actor Object Reference") (OtherComp :type "PrimitiveComponent Object Reference") (OtherBodyIndex :type Integer))
  (if (== OtherActor (`self.MainChar`))
    (set `/Game/Blueprints/SandboxCharacter_CMC.Ice?` false (`self.MainChar`))))

(fn `UserConstructionScript`)